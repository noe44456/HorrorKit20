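; BP_BackPack is a backpack pickup that the player interacts with to apply its Slots value to their inventory.
; BeginPlay caches player 0's MyCharacter.
; The Interactive event passes Slots and the HUD inventory widget to the character's InventoryComponent through FBackPack, plays a pickup sound at the backpack's location, then destroys the actor.
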(event EventInteractive
  (params (Component :type Primitive%20Component%20Object%20Reference))
  (Default|FBackPack (Variables|/Game/HorrorKit/Blueprints/Player/MyCharacter.MyCharacter_C|GetInventory_Component (Variables|Default|GetCharacter)) (Variables|Default|Get+Slots) (Variables|/Game/HorrorKit/Blueprints/Inventory/Inventory.Inventory_C|GetInventory (Variables|/Game/HorrorKit/Blueprints/Player/Hud.Hud_C|GetInventory (Variables|/Game/HorrorKit/Blueprints/Player/MyCharacter.MyCharacter_C|GetHud (Variables|Default|GetCharacter)))))
  (Audio|PlaySoundatLocation "/Game/HorrorKit/Assets/Audio/Interactive/PickUp/S_PickUp_Cue.S_PickUp_Cue" (Transformation|GetWorldLocation (Variables|Default|GetBackpack)) "0, 0, 0" 1.0 1.0 0.0 "/Game/HorrorKit/Assets/Audio/Interactive/PickUp/Info_Sound_PickUp.Info_Sound_PickUp")
  (Actor|DestroyActor))

(fn ConstructionScript)

(event EventBeginPlay
  (bind _asmy_character (Utilities|Casting|CastToMyCharacter (Game|GetPlayerCharacter 0)))
  (Variables|Default|SetCharacter _asmy_character))