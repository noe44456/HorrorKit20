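; BP_PickUp is a world item pickup whose mesh and identity come from the defaults of its assigned item Class.
; It sets the mesh at construction and BeginPlay, caches the player character, and destroys itself if no Class is set.
; Interacting opens the inventory inspection menu.
; AddItem branches on type and name to unhide the flashlight, assign the pistol, or add to inventory, playing a sound and destroying itself on success.
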(event Custom|Event%20Add%20Item
  (switch Utilities|FlowControl|Switch|SwitchonE_B_BasicPickUp_Type (.Type (Utilities|Struct|BreakS_B_Basic_PickUp (Utilities|GetClassDefaults (Variables|Default|GetClass))))
    (:NewEnumerator0
      (switch string (Utilities|String|ToString(Text) (.Name (Utilities|Struct|BreakS_B_Basic_PickUp (Utilities|GetClassDefaults (Variables|Default|GetClass)))))
        (:Default
          (bind _return (Default|AddItem (Variables|/Game/HorrorKit/Blueprints/Player/MyCharacter.MyCharacter_C|GetInventory_Component (Variables|Default|GetCharacter)) (Variables|Default|GetClass) 1 :!label _label))
          (if _return
            (Audio|PlaySoundatLocation "/Game/HorrorKit/Assets/Audio/Interactive/PickUp/S_PickUp_Cue.S_PickUp_Cue" (Transformation|GetWorldLocation (Variables|Default|GetItem)) "0, 0, 0" 1.0 1.0 0.0 "/Game/HorrorKit/Assets/Audio/Interactive/PickUp/Info_Sound_PickUp.Info_Sound_PickUp" :!label _label_2)
            (Actor|DestroyActor)))
        (:FlashLight
          (Development|SetHiddeninGame (Variables|/Game/HorrorKit/Blueprints/Player/MyCharacter.MyCharacter_C|GetFlashLight (Variables|Default|GetCharacter)) false false)
          (goto _label_2))
        (:Battery
          (goto _label))))
    (:NewEnumerator1
      (goto _label))
    (:NewEnumerator4
      (goto _label))
    (:NewEnumerator5
      (switch string (Utilities|String|ToString(Text) (.Name (Utilities|Struct|BreakS_B_Basic_PickUp (Utilities|GetClassDefaults (Variables|Default|GetClass)))))
        (:Pistol
          (Variables|/Game/HorrorKit/Blueprints/Weapons/Guns_Component.Guns_Component_C|SetBP_Pistol (Variables|/Game/HorrorKit/Blueprints/Player/MyCharacter.MyCharacter_C|GetGuns_Component (Variables|Default|GetCharacter)) "/Game/HorrorKit/Blueprints/Weapons/Class/BP_Pistol.BP_Pistol_C")
          (goto _label_2))))
    (:NewEnumerator3
      (goto _label))))

(event EventInteractive
  (params (Component :type Primitive%20Component%20Object%20Reference))
  (Default|OpenInspectionMenu (Variables|/Game/HorrorKit/Blueprints/Player/MyCharacter.MyCharacter_C|GetInventory_Component (Variables|Default|GetCharacter)) (Variables|/Script/Engine.StaticMeshComponent|GetStaticMesh (Variables|Default|GetItem)) self (Variables|Default|GetSee?)))

(fn ConstructionScript
  (bind _class (Variables|Default|GetClass))
  (if (Utilities|IsValidClass _class)
    (Utilities|IsValid (.SM (Utilities|Struct|BreakS_B_Basic_PickUp (Utilities|GetClassDefaults _class)))
      (:Is%20Valid
        (Components|StaticMesh|SetStaticMesh (Variables|Default|GetItem) (.SM (Utilities|Struct|BreakS_B_Basic_PickUp (Utilities|GetClassDefaults (Variables|Default|GetClass)))))))))

(event EventBeginPlay
  (Utilities|FlowControl|Delay 0.01)
  (if (Utilities|IsValidClass (Variables|Default|GetClass))
    (bind _asmy_character (Utilities|Casting|CastToMyCharacter (Game|GetPlayerCharacter 0)))
    (Variables|Default|SetCharacter _asmy_character)
    (Utilities|IsValid (.SM (Utilities|Struct|BreakS_B_Basic_PickUp (Utilities|GetClassDefaults (Variables|Default|GetClass))))
      (:Is%20Valid
        (Components|StaticMesh|SetStaticMesh (Variables|Default|GetItem) (.SM (Utilities|Struct|BreakS_B_Basic_PickUp (Utilities|GetClassDefaults (Variables|Default|GetClass)))))))
    (else
      (Actor|DestroyActor))))