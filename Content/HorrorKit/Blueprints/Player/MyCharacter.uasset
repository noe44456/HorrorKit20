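; First-person player character for the horror kit, turning input into movement, camera shake, sprinting, gunplay, flashlight use, inventory and object inspection.
; A shared camera line trace drives interaction, door key use, physics-handle grabbing and per-tick outline highlighting.
; Stamina, guns, inventory, inspection and outlines are delegated to components, while delays time flashlight and pistol swaps.
; The Branch flag blocks action inputs while the inventory is open, and inspection suspends movement and look.
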(fn ConstructionScript)

(fn FLineTrace
  (params (Distance :type Integer) (Type :type Array%20of%20EObjectTypeQuery%20Enums :default "ObjectTypeQuery1"))
  (bind _camera (Variables|Default|GetCamera))
  (bind _returnvalue (Transformation|GetWorldLocation _camera))
  (bind (_outhit _returnvalue_2) (Collision|LineTraceForObjects _returnvalue (+ _returnvalue (* (Math|Vector|GetForwardVector _camera) Distance)) Type false 0 "None"))
  (return _returnvalue_2 _outhit))

(event EventBeginPlay
  (Utilities|FlowControl|Sequence
    (:then_0
      (Utilities|FlowControl|Sequence
        (:then_0
          (bind _returnvalue (UserInterface|CreateWidget "/Game/HorrorKit/Blueprints/Player/Hud.Hud_C"))
          (bind _output_get (Variables|Reference|SetHud _returnvalue))
          (UserInterface|Viewport|AddtoViewport _output_get 0))))
    (:then_1
      (Utilities|FlowControl|Sequence
        (:then_0
          (bind _asmy_player_controller (Utilities|Casting|CastToMyPlayerController (Game|GetPlayerController 0)))
          (Variables|Reference|SetPlayerController _asmy_player_controller))
        (:then_1
          (bind _asanim_my_character (Utilities|Casting|CastToAnim_MyCharacter (Components|SkeletalMesh|GetAnimInstance (Variables|Default|GetSkeletal_Mesh))))
          (Variables|Animation|SetAnim_Blueprint _asanim_my_character))))))

(event Input|AxisEvents|InputAxisMouseY
  (params (AxisValue :type Float%20%28single-precision%29))
  (bind _hud (Variables|Reference|GetHud))
  (bind _camera (Variables|Default|GetCamera))
  (bind _options_menu (Variables|/Game/HorrorKit/Blueprints/Player/Hud.Hud_C|GetOptions_Menu _hud))
  (bind _mouse_info (Variables|/Game/HorrorKit/Blueprints/Widgets/Main_Menu/Options_Menu.Options_Menu_C|GetMouse_Info _options_menu))
  (bind (_sensivity _vertical_look) (Utilities|Struct|BreakMouse_Settings_S _mouse_info))
  (bind _returnvalue (Math|Float|SelectFloat -1.0 1.0 _vertical_look))
  (bind _returnvalue_2 (/ _sensivity 10))
  (bind _returnvalue_3 (Math|Conversions|ToFloat(Integer) _returnvalue_2))
  (bind _returnvalue_4 (* _returnvalue_3 _returnvalue))
  (bind _returnvalue_5 (* AxisValue _returnvalue_4))
  (if (and (Game|Player|IsInputKeyDown (Game|GetPlayerController 0) "LeftMouseButton") (Utilities|IsValid (Variables|Default|GetInspection_Object)))
    (Default|FRotateY (Variables|Default|GetInspection_Component) (Variables|Default|GetInspection_Object) _returnvalue_5)
    (elif (not (Variables|Other|GetInspection%20Object))
      (Pawn|Input|AddControllerPitchInput _returnvalue_5)
      (Physics|Components|PhysicsHandle|SetTargetLocation (Variables|Default|GetPhysicsHandle) (+ (Transformation|GetWorldLocation _camera) (* (Math|Vector|GetForwardVector _camera) 120))))))

(event Input|AxisEvents|InputAxisMouseX
  (params (AxisValue :type Float%20%28single-precision%29))
  (bind _hud (Variables|Reference|GetHud))
  (bind _camera (Variables|Default|GetCamera))
  (bind _options_menu (Variables|/Game/HorrorKit/Blueprints/Player/Hud.Hud_C|GetOptions_Menu _hud))
  (bind _mouse_info (Variables|/Game/HorrorKit/Blueprints/Widgets/Main_Menu/Options_Menu.Options_Menu_C|GetMouse_Info _options_menu))
  (bind (_sensivity _vertical_look) (Utilities|Struct|BreakMouse_Settings_S _mouse_info))
  (bind _returnvalue (/ _sensivity 10))
  (bind _returnvalue_2 (Math|Conversions|ToFloat(Integer) _returnvalue))
  (bind _returnvalue_3 (* AxisValue _returnvalue_2))
  (if (and (Game|Player|IsInputKeyDown (Game|GetPlayerController 0) "LeftMouseButton") (Utilities|IsValid (Variables|Default|GetInspection_Object)))
    (Default|FRotateX (Variables|Default|GetInspection_Component) (Variables|Default|GetInspection_Object) _returnvalue_3)
    (elif (not (Variables|Other|GetInspection%20Object))
      (Pawn|Input|AddControllerYawInput _returnvalue_3)
      (Physics|Components|PhysicsHandle|SetTargetLocation (Variables|Default|GetPhysicsHandle) (+ (Transformation|GetWorldLocation _camera) (* (Math|Vector|GetForwardVector _camera) 120))))))

(event Input|AxisEvents|InputAxisForwardMove
  (params (AxisValue :type Float%20%28single-precision%29))
  (if (not (Variables|Other|GetInspection%20Object))
    (Pawn|Input|AddMovementInput (Transformation|GetActorForwardVector) AxisValue false)
    (if (and (not (AI|Components|NavMovement|IsFalling (Variables|Character|GetCharacterMovement))) (> (Math|Vector|VectorLength (Transformation|GetVelocity)) 1.5e+02))
      (Class|PlayerController|ClientPlayCameraShake (Variables|Reference|GetPlayerController) "/Game/HorrorKit/Blueprints/Player/Shake/Horror_CameraShake.Horror_CameraShake_C" (Math|Float|SelectFloat 2.0 AxisValue (> (Math|Vector|VectorLength (Transformation|GetVelocity)) 3e+02)) "CameraLocal" "0, 0, 0"))))

(event Input|AxisEvents|InputAxisBackMove
  (params (AxisValue :type Float%20%28single-precision%29))
  (if (not (Variables|Other|GetInspection%20Object))
    (Pawn|Input|AddMovementInput (Transformation|GetActorForwardVector) AxisValue false)
    (if (not (and (not (AI|Components|NavMovement|IsFalling (Variables|Character|GetCharacterMovement))) (> (Math|Vector|VectorLength (Transformation|GetVelocity)) 1.5e+02)))
      (Class|PlayerController|ClientPlayCameraShake (Variables|Reference|GetPlayerController) "/Game/HorrorKit/Blueprints/Player/Shake/Horror_CameraShake.Horror_CameraShake_C" (Math|Float|SelectFloat 2.0 AxisValue (> (Math|Vector|VectorLength (Transformation|GetVelocity)) 3e+02)) "CameraLocal" "0, 0, 0"))))

(event Input|AxisEvents|InputAxisRightMove
  (params (AxisValue :type Float%20%28single-precision%29))
  (if (not (Variables|Other|GetInspection%20Object))
    (Pawn|Input|AddMovementInput (Transformation|GetActorRightVector) AxisValue false)
    (if (and (not (AI|Components|NavMovement|IsFalling (Variables|Character|GetCharacterMovement))) (> (Math|Vector|VectorLength (Transformation|GetVelocity)) 1.5e+02))
      (Class|PlayerController|ClientPlayCameraShake (Variables|Reference|GetPlayerController) "/Game/HorrorKit/Blueprints/Player/Shake/Horror_CameraShake.Horror_CameraShake_C" (Math|Float|SelectFloat 2.0 AxisValue (> (Math|Vector|VectorLength (Transformation|GetVelocity)) 3e+02)) "CameraLocal" "0, 0, 0"))))

(event Input|AxisEvents|InputAxisLeftMove
  (params (AxisValue :type Float%20%28single-precision%29))
  (if (not (Variables|Other|GetInspection%20Object))
    (Pawn|Input|AddMovementInput (Transformation|GetActorRightVector) AxisValue false)
    (if (not (and (not (AI|Components|NavMovement|IsFalling (Variables|Character|GetCharacterMovement))) (> (Math|Vector|VectorLength (Transformation|GetVelocity)) 1.5e+02)))
      (Class|PlayerController|ClientPlayCameraShake (Variables|Reference|GetPlayerController) "/Game/HorrorKit/Blueprints/Player/Shake/Horror_CameraShake.Horror_CameraShake_C" (Math|Float|SelectFloat 2.0 AxisValue (> (Math|Vector|VectorLength (Transformation|GetVelocity)) 3e+02)) "CameraLocal" "0, 0, 0"))))

(event Input|ActionEvents|InputActionRunning
  (params (Key :type Key%20Structure))
  (bind _footsteps_component (Variables|Default|GetFootSteps_Component))
  (bind _character_component (Variables|Default|GetCharacter_Component))
  (bind _branch (Variables|Other|GetBranch))
  (bind _returnvalue (not _branch))
  (bind _type_material (Variables|/Game/HorrorKit/Blueprints/Player/Components/FootSteps_Component/FootSteps_Component.FootSteps_Component_C|GetType%20Material _footsteps_component))
  (bind _returnvalue_2 (Utilities|Enum|NotEqual(Enum) _type_material "SurfaceType4"))
  (:Pressed
    (if _returnvalue
      (if _returnvalue_2
        (Default|EventMinusStamina _character_component))))
  (:Released
    (if _returnvalue
      (if _returnvalue_2
        (Default|EventResetMinusStamina _character_component)))))

(event Input|ActionEvents|InputActionGrab
  (params (Key :type Key%20Structure))
  (:Pressed
    (if (not (Variables|Other|GetBranch))
      (bind (_return _hit) (CallFunction|FLineTrace 180 (Utilities|Array|MakeArray "ObjectTypeQuery2" "ObjectTypeQuery4")))
      (if _return
        (bind _asbp_door_key (Utilities|Casting|CastToBP_Door_Key (.HitActor (Collision|BreakHitResult _hit))))
        (Default|EventUseKey _asbp_door_key)))))

(event Input|ActionEvents|InputActionFire
  (params (Key :type Key%20Structure))
  (:Pressed
    (if (not (Variables|Other|GetBranch))
      (Default|EventFireWeapon (Variables|Default|GetGuns_Component)))))

(event Input|ActionEvents|InputActionReload
  (params (Key :type Key%20Structure))
  (:Pressed
    (if (not (Variables|Other|GetBranch))
      (Default|ReloadWeapon (Variables|Default|GetGuns_Component)))))

(event Input|ActionEvents|InputActionSelectPistol
  (params (Key :type Key%20Structure))
  (:Pressed
    (if (not (Variables|Other|GetBranch))
      (if (not (Variables|Other|GetUse%20Phone))
        (if (not (Variables|/Game/HorrorKit/Blueprints/Weapons/Guns_Component.Guns_Component_C|GetUse%20Animation (Variables|Default|GetGuns_Component)))
          (if (Utilities|IsValidClass (Variables|/Game/HorrorKit/Blueprints/Weapons/Guns_Component.Guns_Component_C|GetBP_Pistol (Variables|Default|GetGuns_Component)))
            (if (Rendering|IsVisible (Variables|Default|GetFlashLight))
              (CallFunction|EventNotTakeFlashLight)
              (Utilities|FlowControl|Delay 1.5)
              (Variables|/Game/HorrorKit/Blueprints/Weapons/Guns_Component.Guns_Component_C|SetUse%20Animation (Variables|Default|GetGuns_Component) false))
            (Default|EventSelectPistol (Variables|Default|GetGuns_Component))))))))

(event Custom|Event%20Enable/Disable%20FlashLight
  (bind _asbp_flash_light (Utilities|Casting|CastToBP_FlashLight (Variables|/Script/Engine.ChildActorComponent|GetChildActor (Variables|Default|GetFlashLight))))
  (Default|EventOn/OffFlashLight _asbp_flash_light))

(event Input|ActionEvents|InputActionActivateFlashLight
  (params (Key :type Key%20Structure))
  (:Pressed
    (if (not (Variables|Other|GetBranch))
      (if (Rendering|IsVisible (Variables|Default|GetFlashLight))
        (if (not (Variables|/Game/HorrorKit/Blueprints/Weapons/Guns_Component.Guns_Component_C|GetUse%20Animation (Variables|Default|GetGuns_Component)))
          (Variables|/Game/HorrorKit/Blueprints/Weapons/Guns_Component.Guns_Component_C|SetUse%20Animation (Variables|Default|GetGuns_Component) true)
          (Utilities|FlowControl|Sequence
            (:then_0
              (Variables|/Game/HorrorKit/Blueprints/Player/Character/Animations/Anim_MyCharacter.Anim_MyCharacter_C|SetEnable_FlashLight (Variables|Animation|GetAnim_Blueprint) true))
            (:then_1
              (Utilities|FlowControl|Delay 1.25)
              (Variables|/Game/HorrorKit/Blueprints/Player/Character/Animations/Anim_MyCharacter.Anim_MyCharacter_C|SetEnable_FlashLight (Variables|Animation|GetAnim_Blueprint) false)
              (Utilities|FlowControl|Delay 0.5)
              (Variables|/Game/HorrorKit/Blueprints/Weapons/Guns_Component.Guns_Component_C|SetUse%20Animation (Variables|Default|GetGuns_Component) false))))))))

(event Custom|Event%20Not%20Take%20FlashLight
  (bind _guns_component (Variables|Default|GetGuns_Component))
  (if (not (Variables|/Game/HorrorKit/Blueprints/Weapons/Guns_Component.Guns_Component_C|GetUse%20Animation (Variables|Default|GetGuns_Component)))
    (if (not (Class|KismetSystemLibrary|IsTimerActive (.AsBP%20Flash%20Light (Utilities|Casting|CastToBP_FlashLight (Variables|/Script/Engine.ChildActorComponent|GetChildActor (Variables|Default|GetFlashLight)))) "F_Minus_FlashLight"))
      _
      (else
        (Variables|/Game/HorrorKit/Blueprints/Player/Character/Animations/Anim_MyCharacter.Anim_MyCharacter_C|SetEnable_FlashLight (Variables|Animation|GetAnim_Blueprint) true)
        (Variables|/Game/HorrorKit/Blueprints/Weapons/Guns_Component.Guns_Component_C|SetUse%20Animation _guns_component true)
        (Utilities|FlowControl|Delay 0.8)
        (Variables|/Game/HorrorKit/Blueprints/Player/Character/Animations/Anim_MyCharacter.Anim_MyCharacter_C|SetEnable_FlashLight (Variables|Animation|GetAnim_Blueprint) false)
        (Variables|/Game/HorrorKit/Blueprints/Weapons/Guns_Component.Guns_Component_C|SetUse%20Animation _guns_component false)))
    (Utilities|IsValid (Variables|/Script/Engine.ChildActorComponent|GetChildActor (Variables|Default|GetGun))
      (:Is%20Valid
        (Variables|Other|SetUse%20Take%20FlashLight true)
        (Default|EventSelectPistol (Variables|Default|GetGuns_Component))
        (Variables|/Game/HorrorKit/Blueprints/Weapons/Guns_Component.Guns_Component_C|SetUse%20Animation (Variables|Default|GetGuns_Component) true)
        (Utilities|FlowControl|Delay 2.0)
        (Variables|/Game/HorrorKit/Blueprints/Player/Character/Animations/Anim_MyCharacter.Anim_MyCharacter_C|SetTake_FlashLight (Variables|Animation|GetAnim_Blueprint) true)
        (Variables|Other|SetUse%20Take%20FlashLight false))
      (:Is%20Not%20Valid
        (Variables|/Game/HorrorKit/Blueprints/Player/Character/Animations/Anim_MyCharacter.Anim_MyCharacter_C|SetTake_FlashLight (Variables|Animation|GetAnim_Blueprint) (select (Variables|/Game/HorrorKit/Blueprints/Player/Character/Animations/Anim_MyCharacter.Anim_MyCharacter_C|GetTake_FlashLight (Variables|Animation|GetAnim_Blueprint)) false true))
        (Variables|/Game/HorrorKit/Blueprints/Weapons/Guns_Component.Guns_Component_C|SetUse%20Animation (Variables|Default|GetGuns_Component) true)))
    (if (Rendering|IsVisible (Variables|Default|GetFlashLight))
      (Utilities|FlowControl|Delay 1.0)
      (Rendering|SetVisibility (Variables|Default|GetFlashLight) false false)
      (else
        (Rendering|SetVisibility (Variables|Default|GetFlashLight) true false)))))

(event Input|ActionEvents|InputActionTakeFlashLight
  (params (Key :type Key%20Structure))
  (bind _guns_component (Variables|Default|GetGuns_Component))
  (:Pressed
    (if (not (Variables|Other|GetBranch))
      (if (not (Variables|/Script/Engine.SceneComponent|GetbHiddenInGame (Variables|Default|GetFlashLight)))
        (if (not (Variables|/Game/HorrorKit/Blueprints/Weapons/Guns_Component.Guns_Component_C|GetUse%20Animation (Variables|Default|GetGuns_Component)))
          (if (not (Class|KismetSystemLibrary|IsTimerActive (.AsBP%20Flash%20Light (Utilities|Casting|CastToBP_FlashLight (Variables|/Script/Engine.ChildActorComponent|GetChildActor (Variables|Default|GetFlashLight)))) "F_Minus_FlashLight"))
            _
            (else
              (Variables|/Game/HorrorKit/Blueprints/Player/Character/Animations/Anim_MyCharacter.Anim_MyCharacter_C|SetEnable_FlashLight (Variables|Animation|GetAnim_Blueprint) true)
              (Variables|/Game/HorrorKit/Blueprints/Weapons/Guns_Component.Guns_Component_C|SetUse%20Animation _guns_component true)
              (Utilities|FlowControl|Delay 0.8)
              (Variables|/Game/HorrorKit/Blueprints/Player/Character/Animations/Anim_MyCharacter.Anim_MyCharacter_C|SetEnable_FlashLight (Variables|Animation|GetAnim_Blueprint) false)
              (Variables|/Game/HorrorKit/Blueprints/Weapons/Guns_Component.Guns_Component_C|SetUse%20Animation _guns_component false)))
          (Utilities|IsValid (Variables|/Script/Engine.ChildActorComponent|GetChildActor (Variables|Default|GetGun))
            (:Is%20Valid
              (Variables|Other|SetUse%20Take%20FlashLight true)
              (Default|EventSelectPistol (Variables|Default|GetGuns_Component))
              (Variables|/Game/HorrorKit/Blueprints/Weapons/Guns_Component.Guns_Component_C|SetUse%20Animation (Variables|Default|GetGuns_Component) true)
              (Utilities|FlowControl|Delay 2.0)
              (Variables|/Game/HorrorKit/Blueprints/Player/Character/Animations/Anim_MyCharacter.Anim_MyCharacter_C|SetTake_FlashLight (Variables|Animation|GetAnim_Blueprint) true)
              (Variables|Other|SetUse%20Take%20FlashLight false))
            (:Is%20Not%20Valid
              (Variables|/Game/HorrorKit/Blueprints/Player/Character/Animations/Anim_MyCharacter.Anim_MyCharacter_C|SetTake_FlashLight (Variables|Animation|GetAnim_Blueprint) (select (Variables|/Game/HorrorKit/Blueprints/Player/Character/Animations/Anim_MyCharacter.Anim_MyCharacter_C|GetTake_FlashLight (Variables|Animation|GetAnim_Blueprint)) false true))
              (Variables|/Game/HorrorKit/Blueprints/Weapons/Guns_Component.Guns_Component_C|SetUse%20Animation (Variables|Default|GetGuns_Component) true)))
          (if (Rendering|IsVisible (Variables|Default|GetFlashLight))
            (Utilities|FlowControl|Delay 1.0)
            (Rendering|SetVisibility (Variables|Default|GetFlashLight) false false)
            (else
              (Rendering|SetVisibility (Variables|Default|GetFlashLight) true false))))))))

(event Input|ActionEvents|InputActionReloadFlashLight
  (params (Key :type Key%20Structure))
  (:Pressed
    (if (not (Variables|Other|GetBranch))
      (if (Rendering|IsVisible (Variables|Default|GetFlashLight))
        (if (not (Variables|/Game/HorrorKit/Blueprints/Weapons/Guns_Component.Guns_Component_C|GetUse%20Animation (Variables|Default|GetGuns_Component)))
          (bind _asbp_flash_light (Utilities|Casting|CastToBP_FlashLight (Variables|/Script/Engine.ChildActorComponent|GetChildActor (Variables|Default|GetFlashLight))))
          (Default|EventReloadFlashLightFind _asbp_flash_light))))))

(event Input|ActionEvents|InputActionInteractive
  (params (Key :type Key%20Structure))
  (:Pressed
    (if (not (Variables|Other|GetBranch))
      (if (not (Variables|Other|GetInspection%20Object))
        (bind (_return _hit) (CallFunction|FLineTrace 220 (Utilities|Array|MakeArray "ObjectTypeQuery4" "ObjectTypeQuery2")))
        (if _return
          (Class|FInteractive|Interactive(Message) (.HitActor (Collision|BreakHitResult _hit)) (.HitComponent (Collision|BreakHitResult _hit))))))))

(event Custom|Event%20Close%20Move%20Item
  (if (Widget|IsVisible (Variables|/Game/HorrorKit/Blueprints/Player/Hud.Hud_C|GetMove_Item (Variables|Reference|GetHud)))
    (Widget|SetVisibility (Variables|/Game/HorrorKit/Blueprints/Player/Hud.Hud_C|GetMove_Item (Variables|Reference|GetHud)) "Hidden")))

(event Custom|Event%20Close%20Inventory
  (Default|FSetDefaultButtons (Variables|Reference|GetPlayerController))
  (Utilities|FlowControl|Delay 0.035)
  (Widget|SetVisibility (Variables|/Game/HorrorKit/Blueprints/Player/Hud.Hud_C|GetInventory (Variables|Reference|GetHud)) "Hidden")
  (Default|FResetBlur (Variables|Reference|GetHud))
  (Default|FCloseWidget (Variables|Reference|GetPlayerController))
  (Default|FResetIgnoreInput (Variables|Reference|GetPlayerController))
  (Default|FFlipFlopVisCrosshair (Variables|Reference|GetHud) true)
  (Variables|Other|SetBranch false)
  (Default|SetDefaultInventory (Variables|Default|GetInventory_Component))
  (if (Widget|IsVisible (Variables|/Game/HorrorKit/Blueprints/Player/Hud.Hud_C|GetMove_Item (Variables|Reference|GetHud)))
    (Widget|SetVisibility (Variables|/Game/HorrorKit/Blueprints/Player/Hud.Hud_C|GetMove_Item (Variables|Reference|GetHud)) "Hidden")))

(event Input|ActionEvents|InputActionInventory
  (params (Key :type Key%20Structure))
  (:Pressed
    (if (and (not (Class|WidgetBlueprintLibrary|IsDragDropping)) (not (Variables|Other|GetInspection%20Object)))
      (if (Widget|IsVisible (Variables|/Game/HorrorKit/Blueprints/Player/Hud.Hud_C|GetInventory (Variables|Reference|GetHud)))
        (Default|FSetDefaultButtons (Variables|Reference|GetPlayerController))
        (Utilities|FlowControl|Delay 0.035)
        (Widget|SetVisibility (Variables|/Game/HorrorKit/Blueprints/Player/Hud.Hud_C|GetInventory (Variables|Reference|GetHud)) "Hidden")
        (Default|FResetBlur (Variables|Reference|GetHud))
        (Default|FCloseWidget (Variables|Reference|GetPlayerController))
        (Default|FResetIgnoreInput (Variables|Reference|GetPlayerController))
        (Default|FFlipFlopVisCrosshair (Variables|Reference|GetHud) true)
        (Variables|Other|SetBranch false)
        (Default|SetDefaultInventory (Variables|Default|GetInventory_Component))
        (if (Widget|IsVisible (Variables|/Game/HorrorKit/Blueprints/Player/Hud.Hud_C|GetMove_Item (Variables|Reference|GetHud)))
          (Widget|SetVisibility (Variables|/Game/HorrorKit/Blueprints/Player/Hud.Hud_C|GetMove_Item (Variables|Reference|GetHud)) "Hidden"))
        (else
          (Widget|SetVisibility (Variables|/Game/HorrorKit/Blueprints/Player/Hud.Hud_C|GetInventory (Variables|Reference|GetHud)) "Visible")
          (Default|FBlur (Variables|Reference|GetHud))
          (Default|FOpenWidget (Variables|Reference|GetPlayerController) (Variables|Reference|GetHud))
          (Default|FIgnoreInput (Variables|Reference|GetPlayerController))
          (Default|FFlipFlopVisCrosshair (Variables|Reference|GetHud) false)
          (Default|FSetCursorCenter (Variables|Reference|GetPlayerController))
          (Variables|Other|SetBranch true))))))

(event Input|ActionEvents|InputActionGrab
  (params (Key :type Key%20Structure))
  (bind _branch (Variables|Other|GetBranch))
  (bind _returnvalue (not _branch))
  (:Pressed
    (if _returnvalue
      (bind (_return _hit) (CallFunction|FLineTrace 220 (Utilities|Array|MakeArray "ObjectTypeQuery4")))
      (if _return
        (bind _asbp_grab_item (Utilities|Casting|CastToBP_Grab_Item (.HitActor (Collision|BreakHitResult _hit)))
          (:then
            (Class|PhysicsHandleComponent|SetInterpolationSpeed (Variables|Default|GetPhysicsHandle) (Variables|/Game/HorrorKit/Blueprints/Grab_Item/BP_Grab_Item.BP_Grab_Item_C|GetMass _asbp_grab_item)))
          (:CastFailed
            (bind _asbp_pick_up (Utilities|Casting|CastToBP_PickUp (.HitActor (Collision|BreakHitResult _hit))))
            (Class|PhysicsHandleComponent|SetInterpolationSpeed (Variables|Default|GetPhysicsHandle) (Utilities|Struct|BreakS_B_Basic_PickUp (Utilities|GetClassDefaults (Variables|/Game/HorrorKit/Blueprints/Inventory/Items/BP_PickUp.BP_PickUp_C|GetClass _asbp_pick_up))))))
        (Class|PhysicsHandleComponent|GrabComponentatLocation (Variables|Default|GetPhysicsHandle) (.HitComponent (Collision|BreakHitResult _hit)) "None" (Transformation|GetWorldLocation (.HitComponent (Collision|BreakHitResult _hit)))))))
  (:Released
    (if _returnvalue
      (Physics|Components|PhysicsHandle|ReleaseComponent (Variables|Default|GetPhysicsHandle)))))

(event EventTick
  (params (DeltaSeconds :type Float%20%28single-precision%29))
  (bind _outline_component (Variables|Default|GetOutline_Component))
  (bind (_return _hit) (CallFunction|FLineTrace 220 (Utilities|Array|MakeArray "ObjectTypeQuery2" "ObjectTypeQuery4")))
  (if _return
    (Default|FSetOutline _outline_component (.HitActor (Collision|BreakHitResult _hit)) (.HitComponent (Collision|BreakHitResult _hit)))
    (else
      (Default|FReleaseOutline _outline_component))))