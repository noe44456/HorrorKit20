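; Player controller for the horror kit that handles the pause menu, key rebinding and shared input helpers for widgets.
; P toggles pause, switching HUD visibility, blur layering, crosshair and input mode, but keeps the UI state if another menu, such as the inventory, is open.
; Helper functions lock input, switch input modes and reposition the cursor.
; While binding is active, any key press is passed to KeyboardComponent as the new key.
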(fn ConstructionScript)

(fn FIgnoreInput
  (Input|SetIgnoreMoveInput true)
  (Input|SetIgnoreLookInput true)
  (return))

(fn FResetIgnoreInput
  (Input|ResetIgnoreLookInput)
  (Input|ResetIgnoreMoveInput)
  (return))

(fn FOpenWidget
  (params (Widget :type Widget%20Object%20Reference))
  (Variables|Default|SetbShowMouseCursor true)
  (Input|SetInputModeGameandUI self Widget "DoNotLock" true)
  (return))

(fn FCloseWidget
  (Variables|Default|SetbShowMouseCursor false)
  (Input|SetInputModeGameOnly self)
  (return))

(fn FSetCursorCenter
  (bind (_sizex _sizey) (HUD|GetViewportSize))
  (Class|PlayerController|SetMouseLocation (/ _sizex 2) (/ _sizey 2))
  (return))

(fn FSetDefaultButtons
  (Class|PlayerController|SetMouseLocation 1000000 1000000)
  (return))

(event EventBeginPlay
  (bind _asmy_character (Utilities|Casting|CastToMyCharacter (Game|GetPlayerCharacter 0)))
  (Variables|Default|SetMyCharacter _asmy_character))

(event Custom|Event%20Close%20Pause%20Game
  (bind _mycharacter (Variables|Default|GetMyCharacter))
  (bind _hud (Variables|/Game/HorrorKit/Blueprints/Player/MyCharacter.MyCharacter_C|GetHud _mycharacter))
  (CallFunction|FSetDefaultButtons)
  (Utilities|FlowControl|Delay 0.035)
  (CallFunction|FSetCursorCenter)
  (Game|SetGamePaused false)
  (Widget|SetVisibility (Variables|/Game/HorrorKit/Blueprints/Player/Hud.Hud_C|GetPause_Game (Variables|/Game/HorrorKit/Blueprints/Player/MyCharacter.MyCharacter_C|GetHud (Variables|Default|GetMyCharacter))) "Hidden")
  (bind _ascanvas_panel_slot (Utilities|Casting|CastToCanvasPanelSlot (Variables|/Script/UMG.Widget|GetSlot (Variables|/Game/HorrorKit/Blueprints/Player/Hud.Hud_C|GetBlur_BackGround (Variables|/Game/HorrorKit/Blueprints/Player/MyCharacter.MyCharacter_C|GetHud (Variables|Default|GetMyCharacter))))))
  (Class|CanvasPanelSlot|SetZOrder _ascanvas_panel_slot)
  (if (not (Math|Boolean|ORBoolean (Widget|IsVisible (Variables|/Game/HorrorKit/Blueprints/Player/Hud.Hud_C|GetInventory _hud)) (Widget|IsVisible (Variables|/Game/HorrorKit/Blueprints/Player/Hud.Hud_C|GetDoor_Key_Widget _hud)) (Widget|IsVisible (Variables|/Game/HorrorKit/Blueprints/Player/Hud.Hud_C|GetPickUp_Menu _hud)) (Widget|IsVisible (Variables|/Game/HorrorKit/Blueprints/Player/Hud.Hud_C|GetSink_Kitchen_Widget _hud))))
    (CallFunction|FCloseWidget)
    (Default|FResetBlur (Variables|/Game/HorrorKit/Blueprints/Player/MyCharacter.MyCharacter_C|GetHud (Variables|Default|GetMyCharacter)))
    (Default|FFlipFlopVisCrosshair (Variables|/Game/HorrorKit/Blueprints/Player/MyCharacter.MyCharacter_C|GetHud (Variables|Default|GetMyCharacter)) true)))

(event Input|KeyboardEvents|P
  (params (Key :type Key%20Structure))
  (bind _mycharacter (Variables|Default|GetMyCharacter))
  (bind _mycharacter_2 (Variables|Default|GetMyCharacter))
  (bind _mycharacter_3 (Variables|Default|GetMyCharacter))
  (bind _mycharacter_4 (Variables|Default|GetMyCharacter))
  (bind _hud (Variables|/Game/HorrorKit/Blueprints/Player/MyCharacter.MyCharacter_C|GetHud _mycharacter))
  (bind _hud_2 (Variables|/Game/HorrorKit/Blueprints/Player/MyCharacter.MyCharacter_C|GetHud _mycharacter_2))
  (bind _hud_3 (Variables|/Game/HorrorKit/Blueprints/Player/MyCharacter.MyCharacter_C|GetHud _mycharacter_3))
  (bind _hud_4 (Variables|/Game/HorrorKit/Blueprints/Player/MyCharacter.MyCharacter_C|GetHud _mycharacter_4))
  (bind _pause_game (Variables|/Game/HorrorKit/Blueprints/Player/Hud.Hud_C|GetPause_Game _hud_3))
  (bind _options_menu (Variables|/Game/HorrorKit/Blueprints/Player/Hud.Hud_C|GetOptions_Menu _hud_4))
  (:Pressed
    (if (and (not (Widget|IsVisible (Variables|/Game/HorrorKit/Blueprints/Player/Hud.Hud_C|GetPause_Game (Variables|/Game/HorrorKit/Blueprints/Player/MyCharacter.MyCharacter_C|GetHud (Variables|Default|GetMyCharacter))))) (not (Widget|IsVisible (Variables|/Game/HorrorKit/Blueprints/Player/Hud.Hud_C|GetOptions_Menu (Variables|/Game/HorrorKit/Blueprints/Player/MyCharacter.MyCharacter_C|GetHud (Variables|Default|GetMyCharacter))))))
      (Game|SetGamePaused true)
      (Widget|SetVisibility _pause_game "Visible")
      (CallFunction|FOpenWidget _pause_game)
      (Default|FFlipFlopVisCrosshair (Variables|/Game/HorrorKit/Blueprints/Player/MyCharacter.MyCharacter_C|GetHud (Variables|Default|GetMyCharacter)) false)
      (Default|EventCloseMoveItem (Variables|Default|GetMyCharacter))
      (bind _ascanvas_panel_slot (Utilities|Casting|CastToCanvasPanelSlot (Variables|/Script/UMG.Widget|GetSlot (Variables|/Game/HorrorKit/Blueprints/Player/Hud.Hud_C|GetBlur_BackGround (Variables|/Game/HorrorKit/Blueprints/Player/MyCharacter.MyCharacter_C|GetHud (Variables|Default|GetMyCharacter))))))
      (Class|CanvasPanelSlot|SetZOrder _ascanvas_panel_slot 1)
      (CallFunction|FSetCursorCenter)
      (if (not (Math|Boolean|ORBoolean (Widget|IsVisible (Variables|/Game/HorrorKit/Blueprints/Player/Hud.Hud_C|GetInventory _hud_2)) (Widget|IsVisible (Variables|/Game/HorrorKit/Blueprints/Player/Hud.Hud_C|GetDoor_Key_Widget _hud_2)) (Widget|IsVisible (Variables|/Game/HorrorKit/Blueprints/Player/Hud.Hud_C|GetPickUp_Menu _hud_2)) (Widget|IsVisible (Variables|/Game/HorrorKit/Blueprints/Player/Hud.Hud_C|GetSink_Kitchen_Widget _hud_2))))
        (Default|FBlur (Variables|/Game/HorrorKit/Blueprints/Player/MyCharacter.MyCharacter_C|GetHud (Variables|Default|GetMyCharacter))))
      (elif (Default|FBranchApply _options_menu)
        (Default|EventBack _options_menu)
        (else
          (CallFunction|FSetDefaultButtons)
          (Utilities|FlowControl|Delay 0.035)
          (CallFunction|FSetCursorCenter)
          (Game|SetGamePaused false)
          (Widget|SetVisibility (Variables|/Game/HorrorKit/Blueprints/Player/Hud.Hud_C|GetPause_Game (Variables|/Game/HorrorKit/Blueprints/Player/MyCharacter.MyCharacter_C|GetHud (Variables|Default|GetMyCharacter))) "Hidden")
          (bind _ascanvas_panel_slot_2 (Utilities|Casting|CastToCanvasPanelSlot (Variables|/Script/UMG.Widget|GetSlot (Variables|/Game/HorrorKit/Blueprints/Player/Hud.Hud_C|GetBlur_BackGround (Variables|/Game/HorrorKit/Blueprints/Player/MyCharacter.MyCharacter_C|GetHud (Variables|Default|GetMyCharacter))))))
          (Class|CanvasPanelSlot|SetZOrder _ascanvas_panel_slot_2)
          (if (not (Math|Boolean|ORBoolean (Widget|IsVisible (Variables|/Game/HorrorKit/Blueprints/Player/Hud.Hud_C|GetInventory _hud)) (Widget|IsVisible (Variables|/Game/HorrorKit/Blueprints/Player/Hud.Hud_C|GetDoor_Key_Widget _hud)) (Widget|IsVisible (Variables|/Game/HorrorKit/Blueprints/Player/Hud.Hud_C|GetPickUp_Menu _hud)) (Widget|IsVisible (Variables|/Game/HorrorKit/Blueprints/Player/Hud.Hud_C|GetSink_Kitchen_Widget _hud))))
            (CallFunction|FCloseWidget)
            (Default|FResetBlur (Variables|/Game/HorrorKit/Blueprints/Player/MyCharacter.MyCharacter_C|GetHud (Variables|Default|GetMyCharacter)))
            (Default|FFlipFlopVisCrosshair (Variables|/Game/HorrorKit/Blueprints/Player/MyCharacter.MyCharacter_C|GetHud (Variables|Default|GetMyCharacter)) true)))))))

(event Input|KeyboardEvents|AnyKey
  (params (Key :type Key%20Structure))
  (bind _keyboard_component (Variables|Default|GetKeyboard_Component))
  (bind _keyboard_component_2 (Variables|Default|GetKeyboard_Component))
  (:Pressed
    (if (Variables|/Game/HorrorKit/Blueprints/Widgets/Main_Menu/Keyboard/Keyboard_Component.Keyboard_Component_C|GetBinding _keyboard_component)
      (Variables|/Game/HorrorKit/Blueprints/Widgets/Main_Menu/Keyboard/Keyboard_Component.Keyboard_Component_C|SetBinding _keyboard_component_2 false)
      (Variables|/Game/HorrorKit/Blueprints/Widgets/Main_Menu/Keyboard/Key_Binding_Widget.Key_Binding_Widget_C|SetBinding (Variables|/Game/HorrorKit/Blueprints/Widgets/Main_Menu/Keyboard/Keyboard_Component.Keyboard_Component_C|GetWidget _keyboard_component) false)
      (bind _branch (Default|FSetKey _keyboard_component_2 (Variables|/Game/HorrorKit/Blueprints/Widgets/Main_Menu/Keyboard/Keyboard_Component.Keyboard_Component_C|GetBinding%20Map _keyboard_component) Key))
      (if _branch
        (Variables|/Game/HorrorKit/Blueprints/Widgets/Main_Menu/Keyboard/Keyboard_Component.Keyboard_Component_C|SetApply_Settings _keyboard_component_2 true)))))