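; Interactive horror-kit washing machine with a timeline-animated door, sliding box and power button, each toggled through Interactive by the component used.
; Interlocks keep the button inactive while the door is open and the door locked while the machine runs or spins down.
; When running, looping timers rotate the drum at a randomly varying speed as start audio hands off to a loop.
; Switching off eases the drum to rest and fades the sound.
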(event Custom|Event%20Start%20Audio
  (Audio|Components|Audio|SetSound (Variables|Default|GetSound) "/Game/HorrorKit/Assets/Audio/Interactive/Washing_Machine/S_Washing_Machine_Loop_Cue.S_Washing_Machine_Loop_Cue")
  (Audio|Components|Audio|Play (Variables|Default|GetSound) 0.0))

(event EventInteractive
  (params (Component :type Primitive%20Component%20Object%20Reference))
  (bind _button (Variables|Default|GetButton))
  (bind _door (Variables|Default|GetDoor))
  (bind _returnvalue (Transformation|GetWorldLocation _door))
  (bind _relativelocation (Variables|/Script/Engine.SceneComponent|GetRelativeLocation _button))
  (if (== Component (Variables|Default|GetDoor))
    (if (and (not (Utilities|Time|IsValidTimerHandle (Variables|Default|GetTimer%20Event))) (not (stale _isa_2)))
      (if (not (Audio|Components|Audio|IsPlaying (Variables|Default|GetAnimation%20Door)))
        (bind _isa (Utilities|FlowControl|FlipFlop)
          (:A
            (Audio|PlaySoundatLocation "/Game/HorrorKit/Assets/Audio/Interactive/Washing_Machine/S_Washing_Machine_Open_Door_Cue.S_Washing_Machine_Open_Door_Cue" _returnvalue "0, 0, 0" 1.0 1.0 0.0 "/Game/HorrorKit/Assets/Audio/Interactive/Washing_Machine/Info_Sound_Washing_Machine.Info_Sound_Washing_Machine")
            (bind _door_2 (Timeline|Animation%20Door Play)
              (:Update
                (Transformation|SetRelativeRotation (Variables|Default|GetScene_Door) (Math|Rotator|MakeRotator 0.0 0.0 _door_2) false false))))
          (:B
            (Utilities|FlowControl|Sequence
              (:then_0
                (Timeline|Animation%20Door Reverse))
              (:then_1
                (Utilities|FlowControl|Delay 0.5)
                (Audio|PlaySoundatLocation "/Game/HorrorKit/Assets/Audio/Interactive/Washing_Machine/S_Washing_Machine_Close_Door_Cue.S_Washing_Machine_Close_Door_Cue" _returnvalue "0, 0, 0" 1.0 1.0 0.0 "/Game/HorrorKit/Assets/Audio/Interactive/Washing_Machine/Info_Sound_Washing_Machine.Info_Sound_Washing_Machine")))))))
    (elif (== Component (Variables|Default|GetBox))
      (if (not (Audio|Components|Audio|IsPlaying (Variables|Default|GetAnimation%20Box)))
        (Utilities|FlowControl|FlipFlop
          (:A
            (Audio|PlaySoundatLocation "/Game/HorrorKit/Assets/Audio/Interactive/Washing_Machine/S_Washing_Machine_Open_Cue.S_Washing_Machine_Open_Cue" (Transformation|GetWorldLocation (Variables|Default|GetBox)) "0, 0, 0" 1.0 1.0 0.0 "/Game/HorrorKit/Assets/Audio/Interactive/Washing_Machine/Info_Sound_Washing_Machine.Info_Sound_Washing_Machine")
            (bind _box (Timeline|Animation%20Box Play)
              (:Update
                (Transformation|SetRelativeLocation (Variables|Default|GetBox) (Math|Vector|MakeVector _box 0.0 0.0) false false))))
          (:B
            (Audio|PlaySoundatLocation "/Game/HorrorKit/Assets/Audio/Interactive/Washing_Machine/S_Washing_Machine_Close_Cue.S_Washing_Machine_Close_Cue" (Transformation|GetWorldLocation (Variables|Default|GetBox)) "0, 0, 0" 1.0 1.0 0.0 "/Game/HorrorKit/Assets/Audio/Interactive/Washing_Machine/Info_Sound_Washing_Machine.Info_Sound_Washing_Machine")
            (Timeline|Animation%20Box Reverse))))
      (elif (== Component (Variables|Default|GetButton))
        (if (not _isa)
          (if (not (Audio|Components|Audio|IsPlaying (Variables|Default|GetAnimation%20Button)))
            (if (not (Audio|Components|Audio|IsPlaying (Variables|Default|GetAnimation%20Button%20Reverse)))
              (Utilities|FlowControl|Sequence
                (:then_0
                  (bind _isa_2 (Utilities|FlowControl|FlipFlop)
                    (:A
                      (bind _button_2 (Timeline|Animation%20Button PlayFromStart)
                        (:Update
                          (Transformation|SetRelativeLocation (Variables|Default|GetButton) (Math|Vector|MakeVector _button_2 (.y _relativelocation) (.z _relativelocation)) false false))
                        (:Finished
                          (if _isa_2 :!label _label
                            (Utilities|FlowControl|Sequence
                              (:then_0
                                (Audio|Components|Audio|Play))
                              (:then_1
                                (Audio|Components|Audio|SetVolumeMultiplier (Variables|Default|GetSound) 1.0 :!class /Script/Engine.AudioComponent)
                                (Audio|Components|Audio|SetSound (Variables|Default|GetSound) "/Game/HorrorKit/Assets/Audio/Interactive/Washing_Machine/S_Washing_Machine_Start_Cue.S_Washing_Machine_Start_Cue")
                                (Audio|Components|Audio|Play (Variables|Default|GetSound) 0.0)
                                (bind _returnvalue_2 (Utilities|Time|SetTimerbyEvent (delegate Custom|Event%20Start%20Audio) 5.21))
                                (Variables|Default|SetTimer%20Audio _returnvalue_2)))
                            (else
                              (Utilities|FlowControl|Sequence
                                (:then_0
                                  (|RemovePlay))
                                (:then_1
                                  (Timeline|Volume_Minus Play))))))))
                    (:B
                      (bind _button_3 (Timeline|Animation%20Button%20Reverse PlayFromStart)
                        (:Update
                          (Transformation|SetRelativeLocation (Variables|Default|GetButton) (Math|Vector|MakeVector _button_3 (.y _relativelocation) (.z _relativelocation)) false false))
                        (:Finished
                          (goto _label))))))
                (:then_1
                  (Utilities|FlowControl|Delay 0.2)
                  (Audio|PlaySoundatLocation "/Game/HorrorKit/Assets/Audio/Interactive/Washing_Machine/S_Washing_Machine_Button_Cue.S_Washing_Machine_Button_Cue" (Transformation|GetWorldLocation (Variables|Default|GetButton)) "0, 0, 0" 1.0 1.0 0.0 "/Game/HorrorKit/Assets/Audio/Interactive/Washing_Machine/Info_Sound_Washing_Machine.Info_Sound_Washing_Machine"))))))))))

(fn ConstructionScript)

(fn FRotateDrum
  (Transformation|AddLocalRotation (Variables|Default|GetDrum) (Math|Rotator|MakeRotator (Variables|Default|GetMinus) 0.0 0.0) false false))

(event Custom|Event%20+%20Minus
  (if (> (Math|Float|Absolute(Float) (Variables|Default|GetMinus)) (Variables|Default|GetRandom%20Minus))
    (Variables|Default|SetMinus (Math|Float|Min(Float) (+ (Variables|Default|GetMinus) 0.5) 4.0))
    (else
      (Variables|Default|SetMinus (Math|Float|Max(Float) (- (Variables|Default|GetMinus) 0.5) -4.0)))))

(event Custom|Event%20Random
  (bind _minus (Variables|Default|GetMinus))
  (bind _returnvalue (Math|Float|Absolute(Float) _minus))
  (Variables|Default|SetRandom%20Minus (Math|Random|RandomFloatinRange (+ _returnvalue 0.5) (+ _returnvalue 1e+01))))

(event Custom|Event%20Remove%20Play
  (bind _output_get (Variables|Default|SetMinus (Math|Float|SelectFloat (Math|Float|Min(Float) (+ (Variables|Default|GetMinus) 0.5) 0.0) (Math|Float|Max(Float) (- (Variables|Default|GetMinus) 0.5) 0.0) (< (Variables|Default|GetMinus) 0.0))))
  (if (== _output_get 0.0)
    (Variables|Default|SetMinus 1.0)
    (Utilities|Time|ClearTimerbyFunctionName 0 "F_Rotate_Drum")
    (Utilities|Time|ClearandInvalidateTimerbyHandle (Variables|Default|GetTimer%20Event))
    (Utilities|Time|ClearandInvalidateTimerbyHandle (Variables|Default|GetTimer%20Remove%20play))
    (Utilities|Time|ClearandInvalidateTimerbyHandle (Variables|Default|GetTimer%20Random))))

(event Custom|Event%20Minus%20Audio
  (bind _sound (Variables|Default|GetSound))
  (bind _volumemultiplier (Variables|/Script/Engine.AudioComponent|GetVolumeMultiplier _sound))
  (Audio|Components|Audio|SetVolumeMultiplier _sound (Math|Float|Max(Float) (- _volumemultiplier 0.1) 0.0) :!class /Script/Engine.AudioComponent)
  (if (== _volumemultiplier 0.0)
    (Audio|Components|Audio|Stop (Variables|Default|GetSound))
    (Audio|Components|Audio|SetVolumeMultiplier (Variables|Default|GetSound) 1.0 :!class /Script/Engine.AudioComponent)
    (Utilities|Time|ClearandInvalidateTimerbyHandle (Variables|Default|GetTimer%20Minus%20Audio))))

(event EventBeginPlay
  (bind _returnvalue (Audio|SpawnSoundatLocation "/Game/HorrorKit/Assets/Audio/Interactive/Washing_Machine/S_Washing_Machine_Loop_Cue.S_Washing_Machine_Loop_Cue" (Transformation|GetWorldLocation (Variables|Default|GetDrum)) "0, 0, 0" 1.0 1.0 0.0 "/Game/HorrorKit/Assets/Audio/Interactive/Washing_Machine/Info_Sound_Washing_Machine.Info_Sound_Washing_Machine" 0 false))
  (bind _output_get (Variables|Default|SetSound _returnvalue))
  (Audio|Components|Audio|Stop _output_get))