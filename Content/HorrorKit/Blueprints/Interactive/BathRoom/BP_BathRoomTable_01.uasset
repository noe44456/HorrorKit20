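; Interactive bathroom table with two sliding drawers and a hinged door that the player can open and close.
; The Interactive event compares the hit component to each part and calls Box_01, Box_02 or Door.
; Each function ignores input while its timeline plays, otherwise a FlipFlop alternates playing and reversing it with open and close sounds.
; Timelines drive drawer X location and door yaw.
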(event EventInteractive
  (params (Component :type Primitive%20Component%20Object%20Reference))
  (if (== Component (Variables|Default|GetBox_Table_01))
    (|Box_01)
    (elif (== Component (Variables|Default|GetBox_Table_02))
      (|Box_02)
      (elif (== Component (Variables|Default|GetDoor_Table))
        (|Door)))))

(fn ConstructionScript)