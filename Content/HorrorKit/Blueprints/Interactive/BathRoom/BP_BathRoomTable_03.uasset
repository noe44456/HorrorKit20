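; Interactive bathroom table with two cabinet doors that the player can open and close independently.
; The Interactive event compares the hit component to each door and calls that door's system function.
; Each system uses a FlipFlop to play or reverse its timeline, rotating the door's scene component in yaw with wardrobe open and close sounds.
; Input is ignored while that door's timeline is playing.
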(event EventInteractive
  (params (Component :type Primitive%20Component%20Object%20Reference))
  (if (== Component (Variables|Default|GetDoor_01))
    (|Door_01_System)
    (elif (== Component (Variables|Default|GetDoor_02))
      (|Door_02_System))))

(fn ConstructionScript)