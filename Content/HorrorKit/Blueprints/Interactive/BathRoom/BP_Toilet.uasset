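; BP_Toilet is an interactive bathroom toilet with a hinged cover and a working flush button.
; Interactive branches on the component used: the cover alternately opens and closes through a FlipFlop-driven timeline that sets its pitch.
; The button runs a movement timeline with press and release sounds, then briefly activates the water effect and plays the flush audio.
; A Use flag blocks another flush until shortly after that audio finishes.
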(event OnAudioFinished(S_Toilet)
  (Utilities|FlowControl|Delay 1.0)
  (Variables|Default|SetUse false))

(event EventInteractive
  (params (Component :type Primitive%20Component%20Object%20Reference))
  (if (== Component (Variables|Default|GetCover_Toilet))
    (if (not (Audio|Components|Audio|IsPlaying (Variables|Default|GetAnimation%20Cover%20Toilet)))
      (Utilities|FlowControl|FlipFlop
        (:A
          (bind _cover (Timeline|Animation%20Cover%20Toilet Play)
            (:Update
              (Transformation|SetRelativeRotation (Variables|Default|GetScene_Cover_Toilet) (Math|Rotator|MakeRotator 0.0 _cover 0.0) false false))))
        (:B
          (Timeline|Animation%20Cover%20Toilet Reverse))))
    (elif (not (Variables|Default|GetUse))
      (if (== Component (Variables|Default|GetButton_Toilet))
        (if (not (Audio|Components|Audio|IsPlaying (Variables|Default|GetAnimation%20Button)))
          (Audio|PlaySoundatLocation "/Game/HorrorKit/Assets/Audio/Interactive/Toilet/S_Button_Toilet_Off_Cue.S_Button_Toilet_Off_Cue" (Transformation|GetWorldLocation (Variables|Default|GetToilet)))
          (bind _button (Timeline|Animation%20Button Play)
            (:Update
              (Transformation|SetRelativeLocation (Variables|Default|GetButton_Toilet) (Math|Vector|MakeVector 0.0 0.0 _button) false false))
            (:Finished
              (if (< _button 0.0)
                (Utilities|FlowControl|Sequence
                  (:then_0
                    (Utilities|FlowControl|Sequence
                      (:then_0
                        (Utilities|FlowControl|Delay 0.5)
                        (Audio|PlaySoundatLocation "/Game/HorrorKit/Assets/Audio/Interactive/Toilet/S_Button_Toilet_On_Cue.S_Button_Toilet_On_Cue" (Transformation|GetWorldLocation (Variables|Default|GetToilet)))
                        (Timeline|Animation%20Button Reverse))
                      (:then_1
                        (Timeline|Animation%20Button Reverse))))
                  (:then_1
                    (Utilities|FlowControl|Delay 1.0)
                    (Components|Activation|SetActive (Variables|Default|GetWater_01) true false)
                    (Utilities|FlowControl|Sequence
                      (:then_0
                        (Utilities|FlowControl|Delay 5.5)
                        (Components|Activation|SetActive (Variables|Default|GetWater_01) false false))
                      (:then_1
                        (Audio|Components|Audio|Play (Variables|Default|GetS_Toilet) 0.0)
                        (Variables|Default|SetUse true)))))))))))))

(fn ConstructionScript)

(event EventBeginPlay)