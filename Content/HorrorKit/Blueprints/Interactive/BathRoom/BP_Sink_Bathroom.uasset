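; Interactive bathroom sink with hot and cold valves that toggle water particles, sound and steam.
; The Interactive event picks the valve by component, a FlipFlop plays or reverses its rotation timeline, and the finished animation updates water and audio.
; One sound spawned at BeginPlay swaps between loop and end cues, louder with both taps open.
; Closing cold starts a timer that shows steam if hot is still running.
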(event Custom|Event%20Smoke
  (if (and (stale EventInteractive _isa) (not (stale EventInteractive _isa_2)))
    (Components|Activation|SetActive (Variables|Default|GetSmoke) true false)))

(event Custom|Event%20Sound
  (if (Variables|Default|GetUse%20Water)
    (Audio|Components|Audio|SetVolumeMultiplier (Variables|Default|GetSound) (select (and (stale EventInteractive _isa) (stale EventInteractive _isa_2)) 2.0 1.0) :!class /Script/Engine.AudioComponent)
    (else
      (Utilities|FlowControl|Delay 0.3)
      (Audio|Components|Audio|SetSound (Variables|Default|GetSound) (select (or (stale EventInteractive _isa) (stale EventInteractive _isa_2)) "/Game/HorrorKit/Assets/Audio/Interactive/Sink/S_Sink_Water_Loop_Cue.S_Sink_Water_Loop_Cue" "/Game/HorrorKit/Assets/Audio/Interactive/Sink/S_Sink_Water_End_Cue.S_Sink_Water_End_Cue"))
      (Audio|Components|Audio|SetVolumeMultiplier (Variables|Default|GetSound) (select (and (stale EventInteractive _isa) (stale EventInteractive _isa_2)) 2.0 1.0) :!class /Script/Engine.AudioComponent)
      (Audio|Components|Audio|Play (Variables|Default|GetSound) 0.0))))

(event EventInteractive
  (params (Component :type Primitive%20Component%20Object%20Reference))
  (if (== Component (Variables|Default|GetValve_Hot))
    (if (not (Audio|Components|Audio|IsPlaying (Variables|Default|GetAnimation%20Valve%20Hot)))
      (bind _isa (Utilities|FlowControl|FlipFlop)
        (:A
          (bind _valve (Timeline|Animation%20Valve%20Hot Play)
            (:Update
              (Transformation|SetRelativeRotation (Variables|Default|GetValve_Hot) (Math|Rotator|MakeRotator 0.0 0.0 _valve) false false))
            (:Finished
              (Components|Activation|SetActive (Variables|Default|GetParticleSystem) _isa false)
              (if _isa
                (CallFunction|EventSound)
                (Variables|Default|SetUse%20Water true)
                (else
                  (Utilities|Time|ClearandInvalidateTimerbyHandle (Variables|Default|GetTimer%20Smoke))
                  (Components|Activation|SetActive (Variables|Default|GetSmoke) false false)
                  (CallFunction|EventSound)
                  (Variables|Default|SetUse%20Water false)
                  (CallFunction|EventSound))))))
        (:B
          (Timeline|Animation%20Valve%20Hot Reverse))))
    (elif (== Component (Variables|Default|GetValve_Cold))
      (if (not (Audio|Components|Audio|IsPlaying (Variables|Default|GetAnimation%20Valve_Cold)))
        (bind _isa_2 (Utilities|FlowControl|FlipFlop)
          (:A
            (bind _valve_2 (Timeline|Animation%20Valve_Cold Play)
              (:Update
                (Transformation|SetRelativeRotation (Variables|Default|GetValve_Cold) (Math|Rotator|MakeRotator 0.0 0.0 _valve_2) false false))
              (:Finished
                (Components|Activation|SetActive (Variables|Default|GetParticleSystem1) _isa_2 false)
                (Utilities|Time|ClearandInvalidateTimerbyHandle (Variables|Default|GetTimer%20Smoke))
                (Components|Activation|SetActive (Variables|Default|GetSmoke) false false)
                (if (not _isa_2)
                  (Variables|Default|SetUse%20Water false)
                  (CallFunction|EventSound)
                  (Utilities|FlowControl|Sequence
                    (:then_0
                      (bind _returnvalue (Utilities|Time|SetTimerbyEvent (delegate Custom|Event%20Smoke) 3.0))
                      (Variables|Default|SetTimer%20Smoke _returnvalue)))
                  (else
                    (CallFunction|EventSound)
                    (Variables|Default|SetUse%20Water true))))))
          (:B
            (Timeline|Animation%20Valve_Cold Reverse)))))))

(fn ConstructionScript)

(event EventBeginPlay
  (bind _returnvalue (Audio|SpawnSoundatLocation "/Game/HorrorKit/Assets/Audio/Interactive/Sink/S_Sink_Water_End_Cue.S_Sink_Water_End_Cue" (Transformation|GetWorldLocation (Variables|Default|GetSink)) "0, 0, 0" 1.0 1.0 0.0 "/Game/HorrorKit/Assets/Audio/Interactive/Sink/Info_Sound_Sink.Info_Sound_Sink" 0 false))
  (bind _output_get (Variables|Default|SetSound _returnvalue))
  (Audio|Components|Audio|Stop _output_get))