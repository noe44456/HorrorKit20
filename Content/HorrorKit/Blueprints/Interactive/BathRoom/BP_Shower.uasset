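; BP_Shower is an interactive bathroom shower with two valves and a hinged door.
; Interactive routes by component to FlipFlop-toggled timelines that rotate each part, ignoring input while that part animates.
; Valves play open/close sounds, then switch their water effect and update one shared audio component spawned at the crane on BeginPlay.
; That audio switches between water loop and end cues, doubling volume when both valves are open.
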(event Custom|Event%20Sound
  (if (Variables|Default|GetUse%20Water)
    (Audio|Components|Audio|SetVolumeMultiplier (Variables|Default|GetSound) (select (and (stale EventInteractive _isa) (stale EventInteractive _isa_2)) 2.0 1.0) :!class /Script/Engine.AudioComponent)
    (else
      (Audio|Components|Audio|SetSound (Variables|Default|GetSound) (select (or (stale EventInteractive _isa) (stale EventInteractive _isa_2)) "/Game/HorrorKit/Assets/Audio/Interactive/Sink/S_Sink_Water_Loop_Cue.S_Sink_Water_Loop_Cue" "/Game/HorrorKit/Assets/Audio/Interactive/Sink/S_Sink_Water_End_Cue.S_Sink_Water_End_Cue"))
      (Audio|Components|Audio|SetVolumeMultiplier (Variables|Default|GetSound) (select (and (stale EventInteractive _isa) (stale EventInteractive _isa_2)) 2.0 1.0) :!class /Script/Engine.AudioComponent)
      (Audio|Components|Audio|Play (Variables|Default|GetSound) 0.0))))

(event EventInteractive
  (params (Component :type Primitive%20Component%20Object%20Reference))
  (bind _valve_02 (Variables|Default|GetValve_02))
  (bind _valve_01 (Variables|Default|GetValve_01))
  (bind _returnvalue (Transformation|GetWorldLocation _valve_02))
  (bind _returnvalue_2 (Transformation|GetWorldLocation _valve_01))
  (if (== Component (Variables|Default|GetValve_01))
    (if (not (Audio|Components|Audio|IsPlaying (Variables|Default|GetAnimation%20Valve%2001)))
      (bind _isa (Utilities|FlowControl|FlipFlop)
        (:A
          (Audio|PlaySoundatLocation "/Game/HorrorKit/Assets/Audio/Interactive/Sink/S_Open_Valve_Cue.S_Open_Valve_Cue" _returnvalue_2 "0, 0, 0" 1.0 1.0 0.0 "/Game/HorrorKit/Assets/Audio/Interactive/Sink/Info_Sound_Sink.Info_Sound_Sink")
          (bind _valve (Timeline|Animation%20Valve%2001 Play)
            (:Update
              (Transformation|SetRelativeRotation (Variables|Default|GetScene_Valve_01) (Math|Rotator|MakeRotator _valve 0.0 0.0) false false))
            (:Finished
              (Components|Activation|SetActive (Variables|Default|GetWater_01) _isa false)
              (if _isa
                (CallFunction|EventSound)
                (Variables|Default|SetUse%20Water (or (stale _isa_2) _isa))
                (else
                  (Variables|Default|SetUse%20Water false)
                  (CallFunction|EventSound))))))
        (:B
          (Audio|PlaySoundatLocation "/Game/HorrorKit/Assets/Audio/Interactive/Sink/S_Close_Valve_Cue.S_Close_Valve_Cue" _returnvalue_2 "0, 0, 0" 1.0 1.0 0.0 "/Game/HorrorKit/Assets/Audio/Interactive/Sink/Info_Sound_Sink.Info_Sound_Sink")
          (Timeline|Animation%20Valve%2001 Reverse))))
    (elif (== Component (Variables|Default|GetValve_02))
      (if (not (Audio|Components|Audio|IsPlaying (Variables|Default|GetAnimation%20Valve%2002)))
        (bind _isa_2 (Utilities|FlowControl|FlipFlop)
          (:A
            (Audio|PlaySoundatLocation "/Game/HorrorKit/Assets/Audio/Interactive/Sink/S_Open_Valve_Cue.S_Open_Valve_Cue" _returnvalue "0, 0, 0" 1.0 1.0 0.0 "/Game/HorrorKit/Assets/Audio/Interactive/Sink/Info_Sound_Sink.Info_Sound_Sink")
            (bind _valve_2 (Timeline|Animation%20Valve%2002 Play)
              (:Update
                (Transformation|SetRelativeRotation (Variables|Default|GetScene_Valve_02) (Math|Rotator|MakeRotator _valve_2 0.0 -1.8e+02) false false))
              (:Finished
                (Components|Activation|SetActive (Variables|Default|GetWater_02) _isa_2 false)
                (if _isa_2
                  (CallFunction|EventSound)
                  (Variables|Default|SetUse%20Water (or _isa_2 _isa))
                  (else
                    (Variables|Default|SetUse%20Water false)
                    (CallFunction|EventSound))))))
          (:B
            (Audio|PlaySoundatLocation "/Game/HorrorKit/Assets/Audio/Interactive/Sink/S_Close_Valve_Cue.S_Close_Valve_Cue" _returnvalue "0, 0, 0" 1.0 1.0 0.0 "/Game/HorrorKit/Assets/Audio/Interactive/Sink/Info_Sound_Sink.Info_Sound_Sink")
            (Timeline|Animation%20Valve%2002 Reverse))))
      (elif (== Component (Variables|Default|GetDoor))
        (if (not (Audio|Components|Audio|IsPlaying (Variables|Default|GetAnimation%20Door)))
          (Utilities|FlowControl|FlipFlop
            (:A
              (bind _valve_3 (Timeline|Animation%20Door Play)
                (:Update
                  (Transformation|SetRelativeRotation (Variables|Default|GetScene_Door) (Math|Rotator|MakeRotator 0.0 0.0 _valve_3) false false))))
            (:B
              (Timeline|Animation%20Door Reverse))))))))

(fn ConstructionScript)

(event EventBeginPlay
  (bind _returnvalue (Audio|SpawnSoundatLocation "/Game/HorrorKit/Assets/Audio/Interactive/Sink/S_Sink_Water_End_Cue.S_Sink_Water_End_Cue" (Transformation|GetWorldLocation (Variables|Default|GetCrane)) "0, 0, 0" 1.0 1.0 0.0 "/Game/HorrorKit/Assets/Audio/Interactive/Sink/Info_Sound_Sink.Info_Sound_Sink" 0 false))
  (bind _output_get (Variables|Default|SetSound _returnvalue))
  (Audio|Components|Audio|Stop _output_get))