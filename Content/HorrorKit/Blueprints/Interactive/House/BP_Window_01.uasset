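; Interactive hinged house window that alternates between swinging open and closed when its Window mesh receives the Interactive event.
; The construction script uses Rotate to set up the right-hand mesh, hinge and swing direction, then applies a preset or random starting angle.
; Each use plays an open or close sound and turns the SceneWindow pivot with MoveComponentTo, shortening the first move's duration according to that starting angle.
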(event EventInteractive
  (params (Component :type Primitive%20Component%20Object%20Reference))
  (if (== Component (Variables|Default|GetWindow))
    (if (not (Variables|Default|GetIs%20Play%20Anim))
      (Variables|Default|SetIs%20Play%20Anim true)
      (bind _isa (Utilities|FlowControl|FlipFlop)
        (:A
          _)
        (:B
          _))
      (Utilities|FlowControl|Sequence
        (:then_0
          (if (== (select _isa "/Game/HorrorKit/Assets/Audio/Interactive/Window/S_Open_Window_Cue.S_Open_Window_Cue" "/Game/HorrorKit/Assets/Audio/Interactive/Window/S_Close_Window_Cue.S_Close_Window_Cue") "/Game/HorrorKit/Assets/Audio/Interactive/Window/S_Close_Window.S_Close_Window")
            (Utilities|FlowControl|Delay 0.4))
          (Audio|PlaySoundatLocation (select _isa "/Game/HorrorKit/Assets/Audio/Interactive/Window/S_Open_Window_Cue.S_Open_Window_Cue" "/Game/HorrorKit/Assets/Audio/Interactive/Window/S_Close_Window_Cue.S_Close_Window_Cue") (Transformation|GetWorldLocation (Variables|Default|GetWindow)) "0, 0, 0" 1.0 1.0 0.0 "/Game/HorrorKit/Assets/Audio/Interactive/Window/Info_Sound_Window.Info_Sound_Window")
          (Variables|Default|SetIs%20Play%20Anim false)
          (Variables|Window|SetRotate%20Window 0.0)
          (Variables|Window|SetRandom false))
        (:then_1
          (Components|MoveComponentTo (Variables|Default|GetScene_Window) (Variables|/Script/Engine.SceneComponent|GetRelativeLocation (Variables|Default|GetScene_Window)) (Math|Rotator|SelectRotator (Math|Rotator|SelectRotator "0,90.000000, 0" "0,-90.000000, 0" (Variables|Window|GetRotate)) "0, 0, 0" _isa) false false (Math|Float|SelectFloat (- (Variables|Window|GetTime%20Open/Close) (/ (* (Variables|Window|GetTime%20Open/Close) (Math|Float|Absolute(Float) (.yaw (Variables|/Script/Engine.SceneComponent|GetRelativeRotation (Variables|Default|GetScene_Window))))) 9e+01)) (Math|Float|SelectFloat (- (Variables|Window|GetTime%20Open/Close) (/ (* (Variables|Window|GetTime%20Open/Close) (Math|Float|Absolute(Float) (Math|Float|SelectFloat (Math|Float|Clamp(Float) (Variables|Window|GetRotate%20Window) 0.0 9e+01) (Math|Float|Clamp(Float) (Variables|Window|GetRotate%20Window) -9e+01 0.0) (Variables|Window|GetRotate)))) 9e+01)) (Math|Float|Max(Float) (Variables|Window|GetTime%20Open/Close) 0.0) (!= (Variables|Window|GetRotate%20Window) 0.0)) (Variables|Window|GetRandom)) false))))))

(fn ConstructionScript
  (bind _rotate (Variables|Window|GetRotate))
  (Utilities|FlowControl|Sequence
    (:then_0
      (if (Variables|Window|GetRotate)
        (Components|StaticMesh|SetStaticMesh (Variables|Default|GetWindow) "/Game/HorrorKit/Assets/Models/Interactive/House/Windows/SM_Window_Right.SM_Window_Right")
        (Transformation|DetachFromComponent (Variables|Default|GetWindow) "KeepWorld" "KeepWorld" "KeepWorld" false)
        (Transformation|SetRelativeLocation (Variables|Default|GetScene_Window) "0,37.000000, 0" false false)
        (Transformation|AttachComponentToComponent (Variables|Default|GetWindow) (Variables|Default|GetScene_Window) "None" "KeepWorld" "KeepWorld" "KeepWorld" true)))
    (:then_1
      (Transformation|SetRelativeRotation (Variables|Default|GetScene_Window) (Math|Rotator|MakeRotator 0.0 0.0 (Math|Float|SelectFloat (Math|Random|RandomFloatinRange (Math|Float|SelectFloat 0.0 -9e+01 _rotate) (Math|Float|SelectFloat 9e+01 0.0 _rotate)) (Math|Float|SelectFloat (Math|Float|Clamp(Float) (Variables|Window|GetRotate%20Window) 0.0 9e+01) (Math|Float|Clamp(Float) (* (Variables|Window|GetRotate%20Window) -1.0) -9e+01 0.0) (Variables|Window|GetRotate)) (Variables|Window|GetRandom))) false false))))