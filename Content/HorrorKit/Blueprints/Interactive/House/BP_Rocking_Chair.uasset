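; BP_Rocking_Chair is a horror house prop: a chair that rocks with sound until something enters its trigger box.
; From BeginPlay, a timeline drives the pitch of SceneChair, looping back and forth by choosing Play or Reverse from the pitch on finish.
; Overlap cuts the sound, sets a stop flag and destroys the box.
; The timeline then halts once the floored pitch reaches zero, so the chair settles level.
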(event OnComponentBeginOverlap(Box)
  (params (OverlappedComponent :type Primitive%20Component%20Object%20Reference) (OtherActor :type Actor%20Object%20Reference) (OtherComp :type Primitive%20Component%20Object%20Reference) (OtherBodyIndex :type Integer) (bFromSweep :type Boolean) (SweepResult :type Hit%20Result%20Structure%20%28by%20ref%29))
  (Variables|Default|SetStop true)
  (Audio|Components|Audio|Stop (Variables|Default|GetSound))
  (Components|DestroyComponent (Variables|Default|GetBox)))

(event Custom|Event%20Reverse
  (bind _scene_chair (Variables|Default|GetScene_Chair))
  (bind _anim (Timeline|Animation%20Chair Reverse)
    (:Update
      (Transformation|SetRelativeRotation _scene_chair (Math|Rotator|MakeRotator 0.0 _anim 0.0) false false)
      (if (Variables|Default|GetStop)
        (if (== (Math|Float|Floor (.pitch (Variables|/Script/Engine.SceneComponent|GetRelativeRotation _scene_chair))) 0)
          (CallFunction|EventStop))))
    (:Finished
      (if (> (.pitch (Variables|/Script/Engine.SceneComponent|GetRelativeRotation (Variables|Default|GetScene_Chair))) 0.0)
        (CallFunction|EventReverse)
        (else
          (CallFunction|EventPlayAnimation))))))

(event Custom|Event%20Play%20Animation
  (bind _scene_chair (Variables|Default|GetScene_Chair))
  (bind _anim (Timeline|Animation%20Chair Play)
    (:Update
      (Transformation|SetRelativeRotation _scene_chair (Math|Rotator|MakeRotator 0.0 _anim 0.0) false false)
      (if (Variables|Default|GetStop)
        (if (== (Math|Float|Floor (.pitch (Variables|/Script/Engine.SceneComponent|GetRelativeRotation _scene_chair))) 0)
          (CallFunction|EventStop))))
    (:Finished
      (if (> (.pitch (Variables|/Script/Engine.SceneComponent|GetRelativeRotation (Variables|Default|GetScene_Chair))) 0.0)
        (CallFunction|EventReverse)
        (else
          (CallFunction|EventPlayAnimation))))))

(event Custom|Event%20Stop
  (bind _scene_chair (Variables|Default|GetScene_Chair))
  (bind _anim (Timeline|Animation%20Chair Stop)
    (:Update
      (Transformation|SetRelativeRotation _scene_chair (Math|Rotator|MakeRotator 0.0 _anim 0.0) false false)
      (if (Variables|Default|GetStop)
        (if (== (Math|Float|Floor (.pitch (Variables|/Script/Engine.SceneComponent|GetRelativeRotation _scene_chair))) 0)
          (CallFunction|EventStop))))
    (:Finished
      (if (> (.pitch (Variables|/Script/Engine.SceneComponent|GetRelativeRotation (Variables|Default|GetScene_Chair))) 0.0)
        (CallFunction|EventReverse)
        (else
          (CallFunction|EventPlayAnimation))))))

(event EventBeginPlay
  (bind _scene_chair (Variables|Default|GetScene_Chair))
  (Utilities|FlowControl|Sequence
    (:then_0
      (bind _returnvalue (Audio|SpawnSoundatLocation "/Game/HorrorKit/Assets/Audio/Interactive/Rocking_Chair/S_Rocking_Chair_Cue.S_Rocking_Chair_Cue" (Transformation|GetWorldLocation (Variables|Default|GetChair)) "0, 0, 0" 1.0 1.0 0.0 "/Game/HorrorKit/Assets/Audio/Interactive/Rocking_Chair/Info_Sound_Rocking_Chair.Info_Sound_Rocking_Chair" 0 false))
      (bind _output_get (Variables|Default|SetSound _returnvalue))
      (Audio|Components|Audio|Stop _output_get))
    (:then_1
      (Audio|Components|Audio|Play (Variables|Default|GetSound) 0.0)
      (bind _anim (Timeline|Animation%20Chair Play)
        (:Update
          (Transformation|SetRelativeRotation _scene_chair (Math|Rotator|MakeRotator 0.0 _anim 0.0) false false)
          (if (Variables|Default|GetStop)
            (if (== (Math|Float|Floor (.pitch (Variables|/Script/Engine.SceneComponent|GetRelativeRotation _scene_chair))) 0)
              (CallFunction|EventStop))))
        (:Finished
          (if (> (.pitch (Variables|/Script/Engine.SceneComponent|GetRelativeRotation (Variables|Default|GetScene_Chair))) 0.0)
            (CallFunction|EventReverse)
            (else
              (CallFunction|EventPlayAnimation))))))))

(fn ConstructionScript)