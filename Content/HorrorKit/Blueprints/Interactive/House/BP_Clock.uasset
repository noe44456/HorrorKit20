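; Interactive house prop: an analog wall or table clock with hour, minute and second hands that tick audibly during play.
; The construction script clamps the starting Hours, Minute and Second values and poses the hands in the editor.
; On BeginPlay a looping timer, paced by Speed, calls F_Clock to play a clack, advance the counters with rollover and call F_Rotate.
; F_Rotate converts each counter to a relative roll in whole-unit steps.
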(event EventBeginPlay
  (Utilities|Time|SetTimerbyFunctionName 0 "F_Clock" (Variables|Default|GetSpeed) true))

(fn ConstructionScript
  (Variables|Default|SetHours (Math|Integer|Clamp(Integer) (Variables|Default|GetHours) 0 12))
  (Variables|Default|SetMinute (Math|Integer|Clamp(Integer) (Variables|Default|GetMinute) 0 60))
  (Variables|Default|SetSecond (Math|Integer|Clamp(Integer) (Variables|Default|GetSecond) 0 60))
  (CallFunction|FRotate))

(fn FClock
  (Audio|PlaySoundatLocation "/Game/HorrorKit/Assets/Audio/Interactive/Clock/SoundEffectClockClac_Cue.SoundEffectClockClac_Cue" (Transformation|GetWorldLocation (Variables|Default|GetClock)) "0, 0, 0" 1.0 1.0 0.0 "/Game/HorrorKit/Assets/Audio/Interactive/Clock/Info_Sound_Clock.Info_Sound_Clock")
  (Utilities|FlowControl|Sequence
    (:then_0
      (if (== (Variables|Default|GetSecond) 60)
        (Variables|Default|SetSecond 0 :!label _label)
        (if (== (Variables|Default|GetMinute) 60)
          _
          (else
            (bind _result (Math|Integer|IncrementInt (Variables|Default|GetMinute))
              (:%20%20
                _))))
        (if (== _result 60)
          (Variables|Default|SetMinute 0)
          (if (== (Variables|Default|GetHours) 12)
            (Variables|Default|SetHours 0 :!label _label_2)
            (else
              (bind _result_2 (Math|Integer|IncrementInt (Variables|Default|GetHours))
                (:%20%20
                  (if (== _result_2 12)
                    (goto _label_2)))))))
        (else
          (bind _result_3 (Math|Integer|IncrementInt (Variables|Default|GetSecond))
            (:%20%20
              (if (== _result_3 60)
                (goto _label)))))))
    (:then_1
      (CallFunction|FRotate))))

(fn FRotate
  (Transformation|SetRelativeRotation (Variables|Default|GetArrow_Hours) (Math|Rotator|MakeRotator (Math|Conversions|ToFloat(Integer) (* (/ 360 12) (* (Variables|Default|GetHours) -1))) 0.0 0.0) false false)
  (Transformation|SetRelativeRotation (Variables|Default|GetArrow_Minute) (Math|Rotator|MakeRotator (Math|Conversions|ToFloat(Integer) (* (/ 360 60) (* (Variables|Default|GetMinute) -1))) 0.0 0.0) false false)
  (Transformation|SetRelativeRotation (Variables|Default|GetArrow_Second) (Math|Rotator|MakeRotator (Math|Conversions|ToFloat(Integer) (* (/ 360 60) (* (Variables|Default|GetSecond) -1))) 0.0 0.0) false false))