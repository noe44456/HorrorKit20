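; BP_Stair is an interactive house staircase that slows the player while a trigger box is overlapped.
; Begin overlap calls EventResetMinusStamina on the player's CharacterComponent and lowers walk speed, while end overlap sets a higher fixed speed.
; Both handlers act on player 0 without checking the overlapping actor.
; The construction script swaps the Stair mesh to SM_Stair_02 when Switch is enabled.
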(event OnComponentBeginOverlap(Box)
  (params (OverlappedComponent :type Primitive%20Component%20Object%20Reference) (OtherActor :type Actor%20Object%20Reference) (OtherComp :type Primitive%20Component%20Object%20Reference) (OtherBodyIndex :type Integer) (bFromSweep :type Boolean) (SweepResult :type Hit%20Result%20Structure%20%28by%20ref%29))
  (Default|EventResetMinusStamina (Variables|/Game/HorrorKit/Blueprints/Player/MyCharacter.MyCharacter_C|GetCharacter_Component (.AsMy%20Character (Utilities|Casting|CastToMyCharacter (Game|GetPlayerCharacter 0)))))
  (Variables|/Script/Engine.CharacterMovementComponent|SetMaxWalkSpeed (Variables|/Script/Engine.Character|GetCharacterMovement (Game|GetPlayerCharacter 0)) 1.1e+02))

(event OnComponentEndOverlap(Box)
  (params (OverlappedComponent :type Primitive%20Component%20Object%20Reference) (OtherActor :type Actor%20Object%20Reference) (OtherComp :type Primitive%20Component%20Object%20Reference) (OtherBodyIndex :type Integer))
  (Variables|/Script/Engine.CharacterMovementComponent|SetMaxWalkSpeed (Variables|/Script/Engine.Character|GetCharacterMovement (Game|GetPlayerCharacter 0)) 2.5e+02))

(fn ConstructionScript
  (if (Variables|Default|GetSwitch?)
    (Components|StaticMesh|SetStaticMesh (Variables|Default|GetStair) "/Game/HorrorKit/Assets/Models/Interactive/House/Stairs/SM_Stair_02.SM_Stair_02")))