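; Interactive horror-house TV that toggles between off and a noisy static screen when its button is used.
; A FlipFlop plays or reverses a timeline that rotates the button, with a delayed click sound.
; When the timeline finishes, its direction sets the screen material, spotlight visibility and looping sound pre-spawned at BeginPlay.
; While on, a looping timer picks random spotlight intensities to fake screen flicker.
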(event EventInteractive
  (params (Component :type Primitive%20Component%20Object%20Reference))
  (if (== Component (Variables|Default|GetButton))
    (if (not (Audio|Components|Audio|IsPlaying (Variables|Default|GetAnimation%20Button)))
      (Utilities|FlowControl|Sequence
        (:then_0
          (Utilities|FlowControl|FlipFlop
            (:A
              (bind (_direction _button) (Timeline|Animation%20Button Play)
                (:Update
                  (Transformation|SetRelativeRotation (Variables|Default|GetButton) (Math|Rotator|MakeRotator _button 0.0 0.0) false false))
                (:Finished
                  (switch Utilities|FlowControl|Switch|SwitchonETimelineDirection _direction
                    (:Forward
                      (Rendering|Material|SetMaterial (Variables|Default|GetTV) 1 "/Game/HorrorKit/Blueprints/Interactive/House/TV/Mat/M_TVNoise_Inst.M_TVNoise_Inst")
                      (Audio|Components|Audio|Play (Variables|Default|GetSound) 0.0)
                      (Utilities|Time|SetTimerbyFunctionName 0 "Random_Light" 0.4 true))
                    (:Backward
                      (Rendering|Material|SetMaterial (Variables|Default|GetTV) 1 "/Game/HorrorKit/Assets/Models/Interactive/House/TV/M_TV_Default_Inst.M_TV_Default_Inst")
                      (Audio|Components|Audio|Stop (Variables|Default|GetSound))
                      (Utilities|Time|ClearTimerbyFunctionName 0 "Random_Light")))
                  (Rendering|SetVisibility (Variables|Default|GetSpotLight) (Utilities|Select :Index _direction :Forward true :Backward false) false))))
            (:B
              (Timeline|Animation%20Button Reverse))))
        (:then_1
          (Utilities|FlowControl|Delay 0.2)
          (Audio|PlaySoundatLocation "/Game/HorrorKit/Assets/Audio/Interactive/TV/S_TV_Button_Cue.S_TV_Button_Cue" (Transformation|GetWorldLocation (Variables|Default|GetButton)) "0, 0, 0" 1.0 1.0 0.0 "/Game/HorrorKit/Assets/Audio/Interactive/TV/Info_Sound_TV.Info_Sound_TV"))))))

(fn ConstructionScript)

(fn RandomLight
  (Rendering|Components|Light|SetIntensity (Variables|Default|GetSpotLight) (Utilities|Select :Index (Math|Random|RandomIntegerinRange 0 4) :Option%200 5e+03 :Option%201 4e+03 :Option%202 3e+03 :Option%203 2e+03 :Option%204 1e+03)))

(event EventBeginPlay
  (bind _returnvalue (Audio|SpawnSoundatLocation "/Game/HorrorKit/Assets/Audio/Interactive/TV/S_TV_Loop_Cue.S_TV_Loop_Cue" (Transformation|GetWorldLocation (Variables|Default|GetTV)) "0, 0, 0" 2e+01 1.0 0.0 "/Game/HorrorKit/Assets/Audio/Interactive/TV/Info_Sound_TV.Info_Sound_TV" 0 false))
  (bind _output_get (Variables|Default|SetSound _returnvalue))
  (Audio|Components|Audio|Stop _output_get))