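; BP_Radio is an interactive house radio that the player switches on and off through its ActivateButton component.
; Interacting plays a click and runs a timeline forward or in reverse to rotate the button, ignoring input while it animates.
; When the timeline finishes, a boolean toggles playback of the sound spawned and stopped at BeginPlay.
; While that boolean is set, the audio-finished event restarts the sound to loop it.
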(event OnAudioFinished(Sound)
  (if (Variables|Default|GetFlipFlop)
    (Audio|Components|Audio|Play (Variables|Default|GetSound) 0.0)))

(event EventInteractive
  (params (Component :type Primitive%20Component%20Object%20Reference))
  (bind _activate_button (Variables|Default|GetActivate_Button))
  (bind _activate_button_2 (Variables|Default|GetActivate_Button))
  (bind _returnvalue (Transformation|GetWorldLocation _activate_button_2))
  (bind _relativerotation (Variables|/Script/Engine.SceneComponent|GetRelativeRotation _activate_button))
  (if (== Component (Variables|Default|GetActivate_Button))
    (if (not (Audio|Components|Audio|IsPlaying (Variables|Default|GetAnimation%20Rotate)))
      (Utilities|FlowControl|FlipFlop
        (:A
          (Audio|PlaySoundatLocation "/Game/HorrorKit/Assets/Audio/Interactive/Radio/S_Radio_Button.S_Radio_Button" _returnvalue "0, 0, 0" 1.0 1.0 0.0 "/Game/HorrorKit/Assets/Audio/Interactive/Radio/Info_Sound_Radio.Info_Sound_Radio")
          (bind _button (Timeline|Animation%20Rotate Play)
            (:Update
              (Transformation|SetRelativeRotation (Variables|Default|GetActivate_Button) (Math|Rotator|MakeRotator _button (.pitch _relativerotation) (.yaw _relativerotation)) false false))
            (:Finished
              (if (Variables|Default|GetFlipFlop)
                (Variables|Default|SetFlipFlop false)
                (Audio|Components|Audio|Stop (Variables|Default|GetSound))
                (else
                  (Variables|Default|SetFlipFlop true)
                  (Audio|Components|Audio|Play (Variables|Default|GetSound) 0.0))))))
        (:B
          (Audio|PlaySoundatLocation "/Game/HorrorKit/Assets/Audio/Interactive/Radio/S_Radio_Button.S_Radio_Button" _returnvalue "0, 0, 0" 1.0 1.0 0.0 "/Game/HorrorKit/Assets/Audio/Interactive/Radio/Info_Sound_Radio.Info_Sound_Radio")
          (Timeline|Animation%20Rotate Reverse))))))

(fn ConstructionScript)

(event EventBeginPlay
  (bind _returnvalue (Audio|SpawnSoundatLocation "/Game/HorrorKit/Assets/Audio/Interactive/Radio/S_Null_Radio_Cue.S_Null_Radio_Cue" (Transformation|GetWorldLocation (Variables|Default|GetRadio)) "0, 0, 0" 1.0 1.0 0.0 "/Game/HorrorKit/Assets/Audio/Interactive/Phone/Info_Sound_Phone.Info_Sound_Phone" 0 false))
  (bind _output_get (Variables|Default|SetSound _returnvalue))
  (Audio|Components|Audio|Stop _output_get))