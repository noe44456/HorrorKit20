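; Interactive electronic clock prop for a house that shows zero-padded hours and minutes, with an optional alarm.
; A looping timer advances seconds, minutes and hours at a configurable interval and refreshes the text.
; Interacting toggles the alarm, which fires either at a set clock time or after a delay from activation, starting a repeating sound timer.
; With both alarm modes off, BeginPlay clears the Clock component's tags.
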(event EventInteractive
  (params (Component :type Primitive%20Component%20Object%20Reference))
  (if (Variables|Clock_Alarm_Timer|GetUse_Timer_Alarm%20Clock)
    (if (Variables|Logic|GetFlipFlop)
      (Variables|Logic|SetFlipFlop false)
      (Utilities|Time|ClearandInvalidateTimerbyHandle (Variables|Logic|GetTimer_Sound) :!label _label)
      (else
        (Variables|Logic|SetFlipFlop true)))
    (elif (Variables|ClockAlarmTime|GetUse%20Time%20Alarm_Clock)
      (if (Variables|Logic|GetFlipFlop)
        (Variables|Logic|SetFlipFlop false)
        (goto _label)
        (else
          (Variables|Logic|SetFlipFlop true)
          (Utilities|Time|SetTimerbyFunctionName 0 "F_Alarm Clock" (Variables|ClockAlarmTime|GetTime_Alarm_Clock)))))))

(fn ConstructionScript
  (Variables|Clock|SetHours (Math|Integer|Clamp(Integer) (Variables|Clock|GetHours) 0 23))
  (Variables|Clock|SetMinute (Math|Integer|Clamp(Integer) (Variables|Clock|GetMinute) 0 59))
  (Variables|Clock|SetSecond (Math|Integer|Clamp(Integer) (Variables|Clock|GetSecond) 0 59))
  (CallFunction|FTextTime))

(fn FAlarmClock
  (CallFunction|FPlaySound)
  (bind _returnvalue (Utilities|Time|SetTimerbyEvent (EventDispatchers|CreateEvent :!event FPlaySound) (select (Variables|Clock_Alarm_Timer|GetUse_Timer_Alarm%20Clock) (Variables|Clock_Alarm_Timer|GetTimer_Play_Delay) (Variables|ClockAlarmTime|GetTime_Play_Delay)) true))
  (Variables|Logic|SetTimer_Sound _returnvalue))

(fn FTimerClock
  (Utilities|FlowControl|Sequence
    (:then_0
      (if (Variables|Logic|GetFlipFlop)
        (if (Variables|Clock_Alarm_Timer|GetUse_Timer_Alarm%20Clock)
          (if (Math|Boolean|ANDBoolean (== (Variables|Clock_Alarm_Timer|GetHours_Alarm_Clock) (Variables|Clock|GetHours)) (== (Variables|Clock_Alarm_Timer|GetMinute_Alarm_Clock) (Variables|Clock|GetMinute)) (== (Variables|Clock_Alarm_Timer|GetSecond_Alarm_Clock) (Variables|Clock|GetSecond)))
            (CallFunction|FAlarmClock)))))
    (:then_1
      (if (== (Variables|Clock|GetSecond) 60)
        (Variables|Clock|SetSecond 0 :!label _label)
        (if (== (Variables|Clock|GetMinute) 60)
          _
          (else
            (bind _result (Math|Integer|IncrementInt (Variables|Clock|GetMinute))
              (:%20%20
                _))))
        (if (== _result 60)
          (Variables|Clock|SetMinute 0)
          (if (== (Variables|Clock|GetHours) 24)
            (Variables|Clock|SetHours 0 :!label _label_2)
            (else
              (bind _result_2 (Math|Integer|IncrementInt (Variables|Clock|GetHours))
                (:%20%20
                  (if (== _result_2 24)
                    (goto _label_2)))))))
        (else
          (bind _result_3 (Math|Integer|IncrementInt (Variables|Clock|GetSecond))
            (:%20%20
              (if (== _result_3 60)
                (goto _label)))))))
    (:then_2
      (CallFunction|FTextTime))))

(fn FTextTime
  (Rendering|Components|TextRender|SetText (Variables|Default|GetText_Minute) (Utilities|Text|FormatText "{Hoursh}:{Minute}" (Utilities|Text|ToText(String) (Utilities|String|SelectString (Utilities|String|Append "0" (Utilities|String|ToString(Integer) (Variables|Clock|GetHours))) (Utilities|String|ToString(Integer) (Variables|Clock|GetHours)) (== (Variables|Clock|GetHours) (Math|Integer|Clamp(Integer) (Variables|Clock|GetHours) 0 9)))) (Utilities|Text|ToText(String) (Utilities|String|SelectString (Utilities|String|Append "0" (Utilities|String|ToString(Integer) (Variables|Clock|GetMinute))) (Utilities|String|ToString(Integer) (Variables|Clock|GetMinute)) (== (Variables|Clock|GetMinute) (Math|Integer|Clamp(Integer) (Variables|Clock|GetMinute) 0 9)))))))

(fn FPlaySound
  (Audio|Components|Audio|Play (Variables|Default|GetSound) 0.0))

(event EventBeginPlay
  (Utilities|FlowControl|Sequence
    (:then_0
      (if (not (or (Variables|ClockAlarmTime|GetUse%20Time%20Alarm_Clock) (Variables|Clock_Alarm_Timer|GetUse_Timer_Alarm%20Clock)))
        (Variables|/Script/Engine.ActorComponent|SetComponentTags (Variables|Default|GetClock) (Utilities|Array|MakeArray))))
    (:then_1
      (Utilities|Time|SetTimerbyFunctionName 0 "F_Timer_Clock" (Variables|Clock|GetTime_Speed) true))))