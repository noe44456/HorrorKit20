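; BP_Switch is an interactive light switch in HorrorKit's house set that toggles a linked lamp.
; Interactive plays an on or off click sound and eases the button's rotation with MoveComponentTo, then flips OnLights and calls EventSwitchLamp on the Lamp.
; The FlipFlop boolean blocks re-triggering while the button moves.
; BeginPlay switches the lamp and pre-rotates the button when OnLights starts true.
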(event EventBeginPlay
  (if (Variables|Default|GetOn%20Lights)
    (Default|EventSwitchLamp (Variables|Lamp|GetLamp))
    (Transformation|SetRelativeRotation (Variables|Default|GetScene_Button) (Math|Rotator|MakeRotator 0.0 25.0 0.0) false false)))

(event EventInteractive
  (params (Component :type Primitive%20Component%20Object%20Reference))
  (if (not (Variables|Default|GetFlipFlop))
    (Variables|Default|SetFlipFlop true)
    (Audio|PlaySoundatLocation (select (Variables|Default|GetOn%20Lights) "/Game/HorrorKit/Assets/Audio/Interactive/Switch/S_On_Lamp_Cue.S_On_Lamp_Cue" "/Game/HorrorKit/Assets/Audio/Interactive/Switch/S_Off_Lamp_Cue.S_Off_Lamp_Cue") (Transformation|GetWorldLocation (Variables|Default|GetSwitch)) "0, 0, 0" 1.0 1.0 0.0 "/Game/HorrorKit/Assets/Audio/Interactive/Switch/Info_Sound_Switch.Info_Sound_Switch")
    (Components|MoveComponentTo (Variables|Default|GetScene_Button) "0, 0, 0" (select (Variables|Default|GetOn%20Lights) "-25.000000, 0, 0" "25.000000, 0, 0") true true 0.4 false)
    (Variables|Default|SetFlipFlop false)
    (Variables|Default|SetOn%20Lights (select (Variables|Default|GetOn%20Lights) false true))
    (Default|EventSwitchLamp (Variables|Lamp|GetLamp))))

(fn ConstructionScript)