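; BP_Swtich_Lamp is a switchable house lamp in HorrorKit, with a bulb mesh, a point light and a spot light.
; Each SwitchLamp call alternates through a FlipFlop between on and off, toggling both lights' visibility and swapping the bulb's second material slot to match.
; The first call always turns the lamp on, as the state lives only in the FlipFlop and is not read from the lights.
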(event Custom|Event%20Switch%20Lamp
  (Utilities|FlowControl|FlipFlop
    (:A
      (Rendering|Material|SetMaterial (Variables|Default|GetBulb) 1 "/Game/HorrorKit/Assets/Models/Interactive/House/Switch/M_Switch_Lamp_Outline_Inst.M_Switch_Lamp_Outline_Inst")
      (Rendering|SetVisibility (Variables|Default|GetPointLight) true false))
    (:B
      (Rendering|Material|SetMaterial (Variables|Default|GetBulb) 1 "/Game/HorrorKit/Assets/Models/Interactive/House/Switch/M_Grass_Switch_Inst.M_Grass_Switch_Inst")
      (Rendering|SetVisibility (Variables|Default|GetPointLight) false false))))

(fn ConstructionScript)