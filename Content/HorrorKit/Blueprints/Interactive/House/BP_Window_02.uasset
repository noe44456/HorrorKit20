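; Interactive double-casement house window for HorrorKit, with two sashes that open and close independently when interacted with.
; The Interactive event picks a sash by component, then a FlipFlop alternates its open/close sound and MoveComponentTo swing behind a busy flag.
; The construction script sets initial yaw from fixed or random angles, with each sash reading the other's random flag.
; The swing duration scales with that starting angle.
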(event EventInteractive
  (params (Component :type Primitive%20Component%20Object%20Reference))
  (if (== Component (Variables|Default|GetWindow_01))
    (if (not (Variables|Default|GetIs%20Play%20Anim%20Window_01))
      (Variables|Default|SetIs%20Play%20Anim%20Window_01 true)
      (bind _isa (Utilities|FlowControl|FlipFlop)
        (:A
          _)
        (:B
          _))
      (Utilities|FlowControl|Sequence
        (:then_0
          (if (== (select _isa "/Game/HorrorKit/Assets/Audio/Interactive/Window/S_Open_Window_Cue.S_Open_Window_Cue" "/Game/HorrorKit/Assets/Audio/Interactive/Window/S_Close_Window_Cue.S_Close_Window_Cue") "/Game/HorrorKit/Assets/Audio/Interactive/Window/S_Close_Window_Cue.S_Close_Window_Cue")
            (Utilities|FlowControl|Delay 0.4))
          (Audio|PlaySoundatLocation (select _isa "/Game/HorrorKit/Assets/Audio/Interactive/Window/S_Open_Window_Cue.S_Open_Window_Cue" "/Game/HorrorKit/Assets/Audio/Interactive/Window/S_Close_Window_Cue.S_Close_Window_Cue") (Transformation|GetWorldLocation (Variables|Default|GetWindow_01)) "0, 0, 0" 1.0 1.0 0.0 "/Game/HorrorKit/Assets/Audio/Interactive/Window/Info_Sound_Window.Info_Sound_Window")
          (Variables|Window|SetRotate%20Window_01 0.0)
          (Variables|Window|SetRandom_Window_01 false))
        (:then_1
          (Components|MoveComponentTo (Variables|Default|GetScene_Window_01) (Variables|/Script/Engine.SceneComponent|GetRelativeLocation (Variables|Default|GetScene_Window_01)) (Math|Rotator|SelectRotator "0,-90.000000, 0" "0, 0, 0" _isa) false false (Math|Float|SelectFloat (- (Variables|Time|GetTime%20Open/Close) (/ (* (Variables|Time|GetTime%20Open/Close) (Math|Float|Absolute(Float) (.yaw (Variables|/Script/Engine.SceneComponent|GetRelativeRotation (Variables|Default|GetScene_Window_01))))) 9e+01)) (Math|Float|SelectFloat (- (Variables|Time|GetTime%20Open/Close) (/ (* (Variables|Time|GetTime%20Open/Close) (Math|Float|Absolute(Float) (Math|Float|Clamp(Float) (Variables|Window|GetRotate%20Window_01) -9e+01 0.0))) 9e+01)) (Math|Float|Max(Float) (Variables|Time|GetTime%20Open/Close) 0.0) (!= (Variables|Window|GetRotate%20Window_01) 0.0)) (Variables|Window|GetRandom_Window_01)) false)
          (Utilities|FlowControl|Delay 0.2)
          (Variables|Default|SetIs%20Play%20Anim%20Window_01 false))))
    (elif (not (Variables|Default|GetIs%20Play%20Anim%20Window_02))
      (Variables|Default|SetIs%20Play%20Anim%20Window_02 true)
      (bind _isa_2 (Utilities|FlowControl|FlipFlop)
        (:A
          _)
        (:B
          _))
      (Utilities|FlowControl|Sequence
        (:then_0
          (if (== (select _isa_2 "/Game/HorrorKit/Assets/Audio/Interactive/Window/S_Open_Window_Cue.S_Open_Window_Cue" "/Game/HorrorKit/Assets/Audio/Interactive/Window/S_Close_Window_Cue.S_Close_Window_Cue") "/Game/HorrorKit/Assets/Audio/Interactive/Window/S_Close_Window.S_Close_Window")
            (Utilities|FlowControl|Delay 0.4))
          (Audio|PlaySoundatLocation (select _isa_2 "/Game/HorrorKit/Assets/Audio/Interactive/Window/S_Open_Window_Cue.S_Open_Window_Cue" "/Game/HorrorKit/Assets/Audio/Interactive/Window/S_Close_Window_Cue.S_Close_Window_Cue") (Transformation|GetWorldLocation (Variables|Default|GetWindow_02)) "0, 0, 0" 1.0 1.0 0.0 "/Game/HorrorKit/Assets/Audio/Interactive/Window/Info_Sound_Window.Info_Sound_Window")
          (Variables|Window|SetRotate%20Window_02 0.0)
          (Variables|Window|SetRandom_Window_02 false))
        (:then_1
          (Components|MoveComponentTo (Variables|Default|GetScene_Window_02) (Variables|/Script/Engine.SceneComponent|GetRelativeLocation (Variables|Default|GetScene_Window_02)) (Math|Rotator|SelectRotator "0,90.000000, 0" "0, 0, 0" _isa_2) false false (Math|Float|SelectFloat (- (Variables|Time|GetTime%20Open/Close) (/ (* (Variables|Time|GetTime%20Open/Close) (Math|Float|Absolute(Float) (.yaw (Variables|/Script/Engine.SceneComponent|GetRelativeRotation (Variables|Default|GetScene_Window_02))))) 9e+01)) (Math|Float|SelectFloat (- (Variables|Time|GetTime%20Open/Close) (/ (* (Variables|Time|GetTime%20Open/Close) (Math|Float|Absolute(Float) (Math|Float|Clamp(Float) (Variables|Window|GetRotate%20Window_02) 0.0 9e+01))) 9e+01)) (Math|Float|Max(Float) (Variables|Time|GetTime%20Open/Close) 0.0) (!= (Variables|Window|GetRotate%20Window_02) 0.0)) (Variables|Window|GetRandom_Window_02)) false)
          (Utilities|FlowControl|Delay 0.2)
          (Variables|Default|SetIs%20Play%20Anim%20Window_02 false))))))

(fn ConstructionScript
  (Transformation|SetRelativeRotation (Variables|Default|GetScene_Window_01) (Math|Rotator|MakeRotator 0.0 0.0 (Math|Float|SelectFloat (Math|Random|RandomFloatinRange -75.0 -15.0) (Math|Float|Clamp(Float) (* (Variables|Window|GetRotate%20Window_01) -1.0) -9e+01 0.0) (Variables|Window|GetRandom_Window_02))) false false)
  (Transformation|SetRelativeRotation (Variables|Default|GetScene_Window_02) (Math|Rotator|MakeRotator 0.0 0.0 (Math|Float|SelectFloat (Math|Random|RandomFloatinRange 15.0 75.0) (Math|Float|Clamp(Float) (Variables|Window|GetRotate%20Window_02) 0.0 9e+01) (Variables|Window|GetRandom_Window_01))) false false))