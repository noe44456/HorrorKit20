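; Interactive hinged door that swings open and closed on the Interactive event, ignoring triggers while it animates.
; A FlipFlop picks sound and duration, and MoveComponentTo rotates SceneDoor between closed and 90 degrees in the direction set by Rotate.
; The construction script previews a clamped RotateDoor starting angle, which scales the first move's duration before being reset to zero.
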(event EventInteractive
  (params (Component :type Primitive%20Component%20Object%20Reference))
  (if (not (Variables|Default|GetIs%20Play%20Anim))
    (Variables|Default|SetIs%20Play%20Anim true)
    (bind _isa (Utilities|FlowControl|FlipFlop)
      (:A
        (Audio|PlaySound2D "/Game/HorrorKit/Assets/Audio/Interactive/Door/S_Open_Door_Cue.S_Open_Door_Cue")
        (Variables|Door|SetTime%20Open/Close 0.55))
      (:B
        (Audio|PlaySound2D "/Game/HorrorKit/Assets/Audio/Interactive/Door/S_Close_Door_Cue.S_Close_Door_Cue")
        (Variables|Door|SetTime%20Open/Close 0.35)))
    (Components|MoveComponentTo (Variables|Default|GetScene_Door) (Variables|/Script/Engine.SceneComponent|GetRelativeLocation (Variables|Default|GetScene_Door)) (Math|Rotator|SelectRotator (Math|Rotator|SelectRotator "0,90.000000, 0" "0,-90.000000, 0" (Variables|Door|GetRotate)) "0,0.000000, 0" _isa) false false (select (!= (Variables|Door|GetRotate_Door) 0.0) (/ (* (Variables|Door|GetTime%20Open/Close) (Math|Float|Absolute(Float) (select (Variables|Door|GetRotate) (Math|Float|Clamp(Float) (Variables|Door|GetRotate_Door) 0.0 9e+01) (Math|Float|Clamp(Float) (* (Variables|Door|GetRotate_Door) -1.0) -9e+01 0.0)))) 9e+01) (Math|Float|Max(Float) (Variables|Door|GetTime%20Open/Close) 0.0)) false)
    (Variables|Default|SetIs%20Play%20Anim false)
    (Variables|Door|SetRotate_Door 0.0)))

(fn ConstructionScript
  (Transformation|SetRelativeRotation (Variables|Default|GetScene_Door) (Math|Rotator|MakeRotator 0.0 0.0 (select (Variables|Door|GetRotate) (Math|Float|Clamp(Float) (Variables|Door|GetRotate_Door) 0.0 9e+01) (Math|Float|Clamp(Float) (* (Variables|Door|GetRotate_Door) -1.0) -9e+01 0.0))) false false))