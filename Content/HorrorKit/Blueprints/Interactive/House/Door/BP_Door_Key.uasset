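; Lockable horror-game house door that the player opens and closes, with a key widget for when they carry a "Key" item.
; Interacting swings the door via FlipFlop and MoveComponentTo with sounds, or plays a locked sound.
; UseKey checks inventory and that the door is shut, then shows the paused, blurred key widget; NotUseKey dismisses it.
; Open_Door and Close_Door set the lock state.
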(event Custom|Event%20Open_Door
  (Variables|Door|SetOpen? true)
  (Utilities|FlowControl|Gate (not (Variables|Door|GetOpen?))) ; enters at Open
)

(event Custom|Event%20Use%20Key
  (bind _character (Variables|Default|GetCharacter))
  (bind _character_2 (Variables|Default|GetCharacter))
  (bind _hud (Variables|/Game/HorrorKit/Blueprints/Player/MyCharacter.MyCharacter_C|GetHud _character))
  (bind _hud_2 (Variables|/Game/HorrorKit/Blueprints/Player/MyCharacter.MyCharacter_C|GetHud _character_2))
  (bind _door_key_widget (Variables|/Game/HorrorKit/Blueprints/Player/Hud.Hud_C|GetDoor_Key_Widget _hud))
  (if (Variables|Door|GetUse%20Door?)
    (bind _branch (Default|SearchItemName (Variables|/Game/HorrorKit/Blueprints/Player/MyCharacter.MyCharacter_C|GetInventory_Component (Variables|Default|GetCharacter)) "Key"))
    (if _branch
      (if (== (.yaw (Variables|/Script/Engine.SceneComponent|GetRelativeRotation (Variables|Default|GetScene_Door))) 0.0)
        (Variables|/Game/HorrorKit/Blueprints/Interactive/House/Door/Door_Key_Widget.Door_Key_Widget_C|SetDoor _door_key_widget self)
        (Default|FBlur _hud_2)
        (Game|SetGamePaused true)
        (Widget|SetVisibility _door_key_widget "Visible")
        (Default|FOpenWidget (Variables|/Game/HorrorKit/Blueprints/Player/MyCharacter.MyCharacter_C|GetPlayerController (Variables|Default|GetCharacter)) _hud_2)
        (Default|EventCheckButtons _door_key_widget)))))

(event Custom|Event%20Not%20Use%20Key
  (Default|FResetBlur (Variables|/Game/HorrorKit/Blueprints/Player/MyCharacter.MyCharacter_C|GetHud (Variables|Default|GetCharacter)))
  (Game|SetGamePaused false)
  (Widget|SetVisibility (Variables|/Game/HorrorKit/Blueprints/Player/Hud.Hud_C|GetDoor_Key_Widget (Variables|/Game/HorrorKit/Blueprints/Player/MyCharacter.MyCharacter_C|GetHud (Variables|Default|GetCharacter))) "Hidden")
  (Default|FCloseWidget (Variables|/Game/HorrorKit/Blueprints/Player/MyCharacter.MyCharacter_C|GetPlayerController (Variables|Default|GetCharacter))))

(event Custom|Event%20Close_Door
  (Variables|Door|SetOpen? false)
  (Utilities|FlowControl|Gate (not (Variables|Door|GetOpen?))) ; enters at Close
)

(event EventBeginPlay
  (bind _asmy_character (Utilities|Casting|CastToMyCharacter (Game|GetPlayerCharacter 0)))
  (Variables|Default|SetCharacter _asmy_character))

(event EventInteractive
  (params (Component :type Primitive%20Component%20Object%20Reference))
  (if (Variables|Door|GetOpen?)
    (Utilities|FlowControl|Gate (not (Variables|Door|GetOpen?))
      (:Exit
        (if (not (Variables|Default|GetIs%20Play%20Anim))
          (Variables|Default|SetIs%20Play%20Anim true)
          (bind _isa (Utilities|FlowControl|FlipFlop)
            (:A
              (Variables|Door|SetTime%20Open/Close 0.55)
              (Audio|PlaySound2D "/Game/HorrorKit/Assets/Audio/Interactive/Door/S_Open_Door_Cue.S_Open_Door_Cue"))
            (:B
              (Variables|Door|SetTime%20Open/Close 0.35)
              (Audio|PlaySound2D "/Game/HorrorKit/Assets/Audio/Interactive/Door/S_Close_Door_Cue.S_Close_Door_Cue")))
          (Components|MoveComponentTo (Variables|Default|GetScene_Door) (Variables|/Script/Engine.SceneComponent|GetRelativeLocation (Variables|Default|GetScene_Door)) (Math|Rotator|SelectRotator (Math|Rotator|SelectRotator "0,90.000000, 0" "0,-90.000000, 0" (Variables|Door|GetRotate)) "0, 0, 0" _isa) false false (Math|Float|Max(Float) (Variables|Door|GetTime%20Open/Close) 0.0) false)
          (Variables|Default|SetIs%20Play%20Anim false))))
    (else
      (Audio|PlaySound2D "/Game/HorrorKit/Assets/Audio/Interactive/Door/S_Closed_Door_Cue.S_Closed_Door_Cue"))))

(fn ConstructionScript)