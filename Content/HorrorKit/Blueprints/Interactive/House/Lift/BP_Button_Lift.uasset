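; Lift floor button for the house lift that, on interaction, sends its Lift to the button's Level, clamped to 1–12.
; A press is ignored while in use, or when Lift.StartLevel matches Level unless the left door sits at zero Y.
; A timeline slides the button in and back with sounds, changes its material and registers it as Lift.Panel.
; SetOutline re-arms the button and restores its default material.
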(event EventInteractive
  (params (Component :type Primitive%20Component%20Object%20Reference))
  (if (== Component (Variables|Default|GetButton))
    (if (not (Variables|Default|GetUse%20Button))
      (if (!= (Variables|/Game/HorrorKit/Blueprints/Interactive/House/Lift/BP_Lift.BP_Lift_C|GetStart%20Level (Variables|Default|GetLift)) (Variables|Default|GetLevel))
        (Variables|Default|SetUse%20Button true :!label _label)
        (CallFunction|ResetOutline)
        (Audio|PlaySound2D "/Game/HorrorKit/Assets/Audio/Interactive/Elevator/S_Elevator_Button_On_Cue.S_Elevator_Button_On_Cue")
        (bind _button (Timeline|Animation Play)
          (:Update
            (Transformation|SetRelativeLocation (Variables|Default|GetButton) (Math|Vector|MakeVector _button 0.0 0.0) false false))
          (:Finished
            (if (not (Variables|Default|GetFlipFlop))
              (Variables|Default|SetFlipFlop true)
              (Rendering|Material|SetMaterial (Variables|Default|GetButton) 1 "/Game/HorrorKit/Assets/Models/Interactive/House/Elevator/M_Outline_Button_Lift_Inst.M_Outline_Button_Lift_Inst")
              (Utilities|FlowControl|Delay 0.5)
              (Utilities|String|Reverse (Variables|Default|GetAnimation))
              (Audio|PlaySound2D "/Game/HorrorKit/Assets/Audio/Interactive/Elevator/S_Elevator_Button_Off_Cue.S_Elevator_Button_Off_Cue")
              (Variables|/Game/HorrorKit/Blueprints/Interactive/House/Lift/BP_Lift.BP_Lift_C|SetPanel (Variables|Default|GetLift) self)
              (Default|EventUp/DownLift (Variables|Default|GetLift) (Variables|Default|GetLevel)))))
        (elif (== (.y (Variables|/Script/Engine.SceneComponent|GetRelativeLocation (Variables|/Game/HorrorKit/Blueprints/Interactive/House/Lift/BP_Lift.BP_Lift_C|GetDoor_Left (Variables|Default|GetLift)))) 0.0)
          (goto _label))))))

(fn ConstructionScript
  (Variables|Default|SetLevel (Math|Integer|Clamp(Integer) (Variables|Default|GetLevel) 1 12)))

(fn ResetOutline
  (Variables|/Script/Engine.ActorComponent|SetComponentTags (Variables|Default|GetButton) (Utilities|Array|MakeArray))
  (Rendering|SetRenderCustomDepth (Variables|Default|GetButton) false))

(fn SetOutline
  (Variables|/Script/Engine.ActorComponent|SetComponentTags (Variables|Default|GetButton) (Utilities|Array|MakeArray "Outline"))
  (Rendering|Material|SetMaterial (Variables|Default|GetButton) 1 "/Game/HorrorKit/Assets/Models/Interactive/House/Elevator/M_Default_Button_Lift_Inst.M_Default_Button_Lift_Inst")
  (Variables|Default|SetFlipFlop false)
  (Variables|Default|SetUse%20Button false))