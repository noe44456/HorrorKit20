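; BP_Lift is an interactive twelve-floor elevator with interior buttons, sliding doors, sounds and a configurable start floor and travel time.
; A button press clears outlines and starts a close, move, open cycle, with travel time scaled by floor distance.
; Timelines slide the cabin doors while the matching floor's child actor under Mine toggles its doors.
; On arrival, it resets either the referenced Panel or the pressed button, restoring the latter's outlines.
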(fn ConstructionScript
  (Variables|Lift|SetStart%20Level (Math|Integer|Clamp(Integer) (Variables|Lift|GetStart%20Level) 1 12))
  (Variables|Lift|SetTime%20Up/Down (Math|Float|Clamp(Float) (Variables|Lift|GetTime%20Up/Down) 1.0 1e+02)))

(fn FButton
  (params (Button :type Primitive%20Component%20Object%20Reference))
  (bind _array_element (Utilities|Array|ForEachLoopwithBreak (Utilities|Array|MakeArray (Variables|Default|GetButton_1) (Variables|Default|GetButton_2) (Variables|Default|GetButton_3) (Variables|Default|GetButton_4) (Variables|Default|GetButton_5) (Variables|Default|GetButton_6) (Variables|Default|GetButton_7) (Variables|Default|GetButton_8) (Variables|Default|GetButton_9) (Variables|Default|GetButton_10) (Variables|Default|GetButton_11) (Variables|Default|GetButton_12)) :!label _label)
    (:LoopBody
      (if (== (Rendering|Material|GetMaterial _array_element 1) "/Game/HorrorKit/Assets/Models/Interactive/House/Elevator/M_Outline_Button_Lift_Inst.M_Outline_Button_Lift_Inst")
        (LocalVariables|SetBranch true)
        (goto _label Break)))
    (:Completed
      (if (not (LocalVariables|GetBranch))
        (bind _array_element_2 (Utilities|Array|ForEachLoopwithBreak (Utilities|Array|MakeArray (Variables|Default|GetButton_1) (Variables|Default|GetButton_2) (Variables|Default|GetButton_3) (Variables|Default|GetButton_4) (Variables|Default|GetButton_5) (Variables|Default|GetButton_6) (Variables|Default|GetButton_7) (Variables|Default|GetButton_8) (Variables|Default|GetButton_9) (Variables|Default|GetButton_10) (Variables|Default|GetButton_11) (Variables|Default|GetButton_12)) :!label _label_2)
          (:LoopBody
            (if (== _array_element_2 Button)
              (LocalVariables|SetLocal%20Button _array_element_2)
              (goto _label_2 Break)))
          (:Completed
            (return (LocalVariables|GetLocal%20Button))))
        (else
          (return 0))))))

(fn FResetOutline
  (for _array_element (Utilities|Array|MakeArray (Variables|Default|GetButton_1) (Variables|Default|GetButton_2) (Variables|Default|GetButton_3) (Variables|Default|GetButton_4) (Variables|Default|GetButton_5) (Variables|Default|GetButton_6) (Variables|Default|GetButton_7) (Variables|Default|GetButton_8) (Variables|Default|GetButton_9) (Variables|Default|GetButton_10) (Variables|Default|GetButton_11) (Variables|Default|GetButton_12))
    (Variables|/Script/Engine.ActorComponent|SetComponentTags _array_element (Utilities|Array|MakeArray))
    (Rendering|SetRenderCustomDepth _array_element false)))

(fn FSetOutline
  (for _array_element (Utilities|Array|MakeArray (Variables|Default|GetButton_1) (Variables|Default|GetButton_2) (Variables|Default|GetButton_3) (Variables|Default|GetButton_4) (Variables|Default|GetButton_5) (Variables|Default|GetButton_6) (Variables|Default|GetButton_7) (Variables|Default|GetButton_8) (Variables|Default|GetButton_9) (Variables|Default|GetButton_10) (Variables|Default|GetButton_11) (Variables|Default|GetButton_12))
    (Variables|/Script/Engine.ActorComponent|SetComponentTags _array_element (Utilities|Array|MakeArray "Outline"))
    (Rendering|Material|SetMaterial _array_element 1 "/Game/HorrorKit/Assets/Models/Interactive/House/Elevator/M_Default_Button_Lift_Inst.M_Default_Button_Lift_Inst")))

(event EventBeginPlay
  (bind _asmy_character (Utilities|Casting|CastToMyCharacter (Game|GetPlayerCharacter 0)))
  (Variables|Reference|SetCharacter _asmy_character)
  (Transformation|SetRelativeLocation (Variables|Default|GetLift) (Utilities|Array|Get(acopy) (Variables|Lift|GetArray%20Level%20Lift) (- (Variables|Lift|GetStart%20Level) 1)) false false)
  (bind _returnvalue (Audio|SpawnSoundatLocation "/Game/HorrorKit/Assets/Audio/Interactive/Elevator/S_Elevator_Run_Cue.S_Elevator_Run_Cue" (Transformation|GetWorldLocation (Variables|Default|GetLift)) "0, 0, 0" 1.0 1.0 0.0 0 0 false))
  (bind _output_get (Variables|Default|SetSound _returnvalue))
  (Audio|Components|Audio|Stop _output_get))

(event Custom|Event%20Remove%20Button
  (if (not (== (.x (Variables|/Script/Engine.SceneComponent|GetRelativeLocation (stale EventInteractive _component))) 0.0))
    (Variables|Button_System|SetFlipFlop true)
    (Audio|PlaySound2D "/Game/HorrorKit/Assets/Audio/Interactive/Elevator/S_Elevator_Button_Off_Cue.S_Elevator_Button_Off_Cue")
    (Components|MoveComponentTo (stale EventInteractive _component) (Math|Vector|MakeVector (Math|Float|SelectFloat 1.5 0.0 (== (.x (Variables|/Script/Engine.SceneComponent|GetRelativeLocation (stale EventInteractive _component))) 0.0)) 0.0 0.0) "0, 0, 0" true true 0.5 false)
    (Rendering|Material|SetMaterial (stale EventInteractive _component) 1 (select (== (.x (Variables|/Script/Engine.SceneComponent|GetRelativeLocation (stale EventInteractive _component))) 0.0) "/Game/HorrorKit/Assets/Models/Interactive/House/Elevator/M_Default_Button_Lift_Inst.M_Default_Button_Lift_Inst" "/Game/HorrorKit/Assets/Models/Interactive/House/Elevator/M_Outline_Button_Lift_Inst.M_Outline_Button_Lift_Inst"))
    (if (not (Variables|Button_System|GetFlipFlop))
      (CallFunction|EventUp/DownLift (+ (Utilities|Array|FindItem (Utilities|Array|MakeArray (Variables|Default|GetButton_1) (Variables|Default|GetButton_2) (Variables|Default|GetButton_3) (Variables|Default|GetButton_4) (Variables|Default|GetButton_5) (Variables|Default|GetButton_6) (Variables|Default|GetButton_7) (Variables|Default|GetButton_8) (Variables|Default|GetButton_9) (Variables|Default|GetButton_10) (Variables|Default|GetButton_11) (Variables|Default|GetButton_12)) (stale EventInteractive _component)) 1))
      (else
        (Variables|Button_System|SetFlipFlop false)))))

(event EventInteractive
  (params (Component :type Primitive%20Component%20Object%20Reference))
  (for (_array_element _array_index) (Utilities|Array|MakeArray (Variables|Default|GetButton_1) (Variables|Default|GetButton_2) (Variables|Default|GetButton_3) (Variables|Default|GetButton_4) (Variables|Default|GetButton_5) (Variables|Default|GetButton_6) (Variables|Default|GetButton_7) (Variables|Default|GetButton_8) (Variables|Default|GetButton_9) (Variables|Default|GetButton_10) (Variables|Default|GetButton_11) (Variables|Default|GetButton_12))
    (if (== _array_element Component)
      (if (== (+ _array_index 1) (Variables|Lift|GetStart%20Level))
        (Variables|Button_System|SetUse%20Button false)
        (else
          (Variables|Button_System|SetUse%20Button true)))))
  (if (Variables|Button_System|GetUse%20Button)
    (Variables|Button_System|SetUse%20Button false)
    (if (not (Variables|Button_System|GetButton_FlipFlop))
      (Variables|Button_System|SetButton_FlipFlop true)
      (bind _component (CallFunction|FButton Component))
      (Utilities|IsValid _component
        (:Is%20Valid
          (CallFunction|FResetOutline)
          (Audio|PlaySound2D "/Game/HorrorKit/Assets/Audio/Interactive/Elevator/S_Elevator_Button_On_Cue.S_Elevator_Button_On_Cue")
          (Components|MoveComponentTo _component (Math|Vector|MakeVector (Math|Float|SelectFloat 1.5 0.0 (== (.x (Variables|/Script/Engine.SceneComponent|GetRelativeLocation _component)) 0.0)) 0.0 0.0) "0, 0, 0" true true 0.5 false)
          (Rendering|Material|SetMaterial _component 1 (select (== (.x (Variables|/Script/Engine.SceneComponent|GetRelativeLocation _component)) 0.0) "/Game/HorrorKit/Assets/Models/Interactive/House/Elevator/M_Default_Button_Lift_Inst.M_Default_Button_Lift_Inst" "/Game/HorrorKit/Assets/Models/Interactive/House/Elevator/M_Outline_Button_Lift_Inst.M_Outline_Button_Lift_Inst"))
          (if (not (Variables|Button_System|GetFlipFlop))
            (CallFunction|EventUp/DownLift (+ (Utilities|Array|FindItem (Utilities|Array|MakeArray (Variables|Default|GetButton_1) (Variables|Default|GetButton_2) (Variables|Default|GetButton_3) (Variables|Default|GetButton_4) (Variables|Default|GetButton_5) (Variables|Default|GetButton_6) (Variables|Default|GetButton_7) (Variables|Default|GetButton_8) (Variables|Default|GetButton_9) (Variables|Default|GetButton_10) (Variables|Default|GetButton_11) (Variables|Default|GetButton_12)) _component) 1))
            (else
              (Variables|Button_System|SetFlipFlop false))))))))

(event Custom|Event%20Close%20Doors
  (Collision|SetCollisionEnabled (Variables|Default|GetBox) "QueryAndPhysics")
  (Utilities|FlowControl|Delay 1.0)
  (Utilities|FlowControl|Sequence
    (:then_0
      (Utilities|FlowControl|Sequence
        (:then_0
          (bind _door (Timeline|Animation%20Close%20Doors SetNewTime)
            (:Update
              (Transformation|SetRelativeLocation (Variables|Default|GetDoor_Left) (Math|Vector|MakeVector 0.0 _door 0.0) false false)
              (Transformation|SetRelativeLocation (Variables|Default|GetDoor_Right) (Math|Vector|MakeVector 0.0 (* _door -1.0) 0.0) false false))
            (:Finished
              (CallFunction|EventUp/DownLift (Variables|Logic|GetLevel%20To)))))
        (:then_1
          (Audio|PlaySoundatLocation "/Game/HorrorKit/Assets/Audio/Interactive/Elevator/S_Elevator_Close_Door_Cue.S_Elevator_Close_Door_Cue" (Transformation|GetWorldLocation (Variables|Default|GetDoor_Left)) "0, 0, 0" 1.0 1.0 0.0 "/Game/HorrorKit/Assets/Audio/Interactive/Elevator/Info_Sound_Elevator.Info_Sound_Elevator")
          (Timeline|Animation%20Close%20Doors Play))))
    (:then_1
      (Default|EventOpen/CloseDoors (Utilities|Array|Get(acopy) (Variables|/Game/HorrorKit/Blueprints/Interactive/House/Lift/BP_Mine.BP_Mine_C|GetChilds (Variables|Reference|GetMine)) (- (Variables|Lift|GetStart%20Level) 1))))))

(event Custom|Event%20Up/Down%20Lift
  (params (Level%20To :type Integer))
  (bind _output_get (Variables|Logic|SetLevel%20To Level%20To))
  (if (!= _output_get (Variables|Lift|GetStart%20Level))
    (if (== (.Y (Math|Vector|BreakVector (Variables|/Script/Engine.SceneComponent|GetRelativeLocation (Variables|Default|GetDoor_Left)))) 0.0)
      (Utilities|FlowControl|Delay 1.5)
      (Audio|Components|Audio|Play (Variables|Default|GetSound) 0.0)
      (Components|MoveComponentTo (Variables|Default|GetLift) (Utilities|Array|Get(acopy) (Variables|Lift|GetArray%20Level%20Lift) (- (Variables|Logic|GetLevel%20To) 1)) "0, 0, 0" true true (Math|Float|Absolute(Float) (* (- (Variables|Lift|GetStart%20Level) (Variables|Logic|GetLevel%20To)) (Math|Float|MapRangeClamped (Variables|Lift|GetTime%20Up/Down) 1.0 1e+02 1.0 1e+01))) false)
      (Variables|Lift|SetStart%20Level (Variables|Logic|GetLevel%20To))
      (CallFunction|EventOpenDoors)
      (Audio|Components|Audio|Stop (Variables|Default|GetSound))
      (else
        (Rendering|SetVisibility (Variables|Default|GetBox) false false)
        (CallFunction|EventCloseDoors)))
    (else
      (CallFunction|EventOpenDoors))))

(event Custom|Event%20Open%20Doors
  (Collision|SetCollisionEnabled (Variables|Default|GetBox) "NoCollision")
  (Utilities|FlowControl|Delay 1.0)
  (Utilities|FlowControl|Sequence
    (:then_0
      (Utilities|FlowControl|Sequence
        (:then_0
          (bind _door (Timeline|Animation%20Open%20Doors SetNewTime)
            (:Update
              (Transformation|SetRelativeLocation (Variables|Default|GetDoor_Left) (Math|Vector|MakeVector 0.0 _door 0.0) false false)
              (Transformation|SetRelativeLocation (Variables|Default|GetDoor_Right) (Math|Vector|MakeVector 0.0 (* _door -1.0) 0.0) false false))
            (:Finished
              (Utilities|IsValid (Variables|Reference|GetPanel)
                (:Is%20Valid
                  (Rendering|Material|SetMaterial (Variables|/Game/HorrorKit/Blueprints/Interactive/House/Lift/BP_Button_Lift.BP_Button_Lift_C|GetButton (Variables|Reference|GetPanel)) 1 "/Game/HorrorKit/Assets/Models/Interactive/House/Elevator/M_Default_Button_Lift_Inst.M_Default_Button_Lift_Inst")
                  (Variables|/Game/HorrorKit/Blueprints/Interactive/House/Lift/BP_Button_Lift.BP_Button_Lift_C|SetUse%20Button (Variables|Reference|GetPanel) false)
                  (Default|SetOutline (Variables|Reference|GetPanel))
                  (Variables|Reference|SetPanel 0))
                (:Is%20Not%20Valid
                  (CallFunction|EventRemoveButton)
                  (Utilities|FlowControl|Delay 1.0)
                  (Variables|Button_System|SetButton_FlipFlop false)
                  (CallFunction|FSetOutline))))))
        (:then_1
          (Audio|PlaySoundatLocation "/Game/HorrorKit/Assets/Audio/Interactive/Elevator/S_Elevator_Open_Door_Cue.S_Elevator_Open_Door_Cue" (Transformation|GetWorldLocation (Variables|Default|GetDoor_Left)) "0, 0, 0" 1.0 1.0 0.0 "/Game/HorrorKit/Assets/Audio/Interactive/Elevator/Info_Sound_Elevator.Info_Sound_Elevator")
          (Timeline|Animation%20Open%20Doors Play))))
    (:then_1
      (Default|EventOpen/CloseDoors (Utilities|Array|Get(acopy) (Variables|/Game/HorrorKit/Blueprints/Interactive/House/Lift/BP_Mine.BP_Mine_C|GetChilds (Variables|Reference|GetMine)) (- (Variables|Logic|GetLevel%20To) 1))))))