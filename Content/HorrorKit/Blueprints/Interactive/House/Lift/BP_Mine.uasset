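; BP_Mine is a modular lift shaft that builds itself in the editor and pairs with a referenced Lift actor.
; Its Construction Script stacks static mesh segments by the base mesh's bounds height, with a clamped count and a separate top piece.
; It snaps the Lift to the shaft, adds a BP_Door_Mine child actor per floor and fills the Lift's level-position array.
; On BeginPlay it registers itself with the Lift.
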(event EventBeginPlay
  (bind _lift (Variables|Default|GetLift)
    (:then
      (Variables|/Game/HorrorKit/Blueprints/Interactive/House/Lift/BP_Lift.BP_Lift_C|SetMine _lift self))
    (:else)))

(fn ConstructionScript
  (bind _lift (Variables|Default|GetLift))
  (bind _array_level_lift (Variables|/Game/HorrorKit/Blueprints/Interactive/House/Lift/BP_Lift.BP_Lift_C|GetArray%20Level%20Lift _lift))
  (if (Variables|Default|GetUpdate)
    _
    (else
      _))
  (Variables|Default|SetUpdate false)
  (Variables|Default|GetLift
    (:then
      (Variables|Default|SetAmount (Math|Integer|Clamp(Integer) (Variables|Default|GetAmount) 1 12))
      (CallFunction|AddMesh)
      (CallFunction|FLift)
      (Utilities|IsValid (Variables|Default|GetLift)
        (:Is%20Valid
          (Utilities|Array|Clear (Variables|Default|GetChilds))
          (Utilities|Array|Clear _array_level_lift)
          (bind _returnvalue (AddComponent|AddChildActorComponent false (Math|Transform|MakeTransform (Math|Vector|MakeVector 226.0 0.0 -75.0) "0,90.000000, 0")))
          (bind _asbp_door_mine (Utilities|Casting|CastToBP_Door_Mine (Variables|/Script/Engine.ChildActorComponent|GetChildActor _returnvalue)))
          (Utilities|Array|Add (Variables|Default|GetChilds) _asbp_door_mine)
          (Utilities|Array|Add :TargetArray _array_level_lift)
          (for _array_element (Variables|Default|GetMeshes)
            (Utilities|Array|Add _array_level_lift (Math|Vector|MakeVector (.x (Variables|/Script/Engine.SceneComponent|GetRelativeLocation _array_element)) (.y (Variables|/Script/Engine.SceneComponent|GetRelativeLocation _array_element)) (+ (.z (Variables|/Script/Engine.SceneComponent|GetRelativeLocation _array_element)) 75.0)))
            (bind _returnvalue_2 (AddComponent|AddChildActorComponent false (Math|Transform|MakeTransform (Math|Vector|MakeVector (+ (.x (Variables|/Script/Engine.SceneComponent|GetRelativeLocation _array_element)) 226.0) (.y (Variables|/Script/Engine.SceneComponent|GetRelativeLocation _array_element)) (.z (Variables|/Script/Engine.SceneComponent|GetRelativeLocation _array_element))) "0,90.000000, 0")))
            (bind _asbp_door_mine_2 (Utilities|Casting|CastToBP_Door_Mine (Variables|/Script/Engine.ChildActorComponent|GetChildActor _returnvalue_2)))
            (Utilities|Array|Add (Variables|Default|GetChilds) _asbp_door_mine_2)))))
    (:else)))

(fn AddMesh
  (Utilities|Array|Clear (Variables|Default|GetMeshes))
  (LocalVariables|SetSpace (* (.Z (Math|Vector|BreakVector (Math|BoxSphereBounds|BreakBoxSphereBounds (StaticMesh|GetBounds (Variables|Default|Get1_Mesh))))) 2.0))
  (for _index (range 1 (- (Variables|Default|GetAmount) 1))
    (LocalVariables|SetDistance (* _index (LocalVariables|GetSpace)))
    (bind _returnvalue (AddComponent|AddStaticMeshComponent false (Math|Transform|MakeTransform (Math|Vector|MakeVector 0.0 0.0 (LocalVariables|GetDistance)))))
    (Utilities|Array|Add (Variables|Default|GetMeshes) _returnvalue)
    (Components|StaticMesh|SetStaticMesh _returnvalue (select (== _index (- (Variables|Default|GetAmount) 1)) (Variables|Default|Get12_Mesh) (Variables|Default|Get2-11_Mesh)))))

(fn FLift
  (bind _returnvalue (Transformation|GetActorTransform))
  (bind (_location _rotation) (Math|Transform|BreakTransform _returnvalue))
  (bind (_x _y _z) (Math|Vector|BreakVector _location))
  (Utilities|IsValid (Variables|Default|GetLift)
    (:Is%20Valid
      (Transformation|SetActorTransform (Variables|Default|GetLift) (Math|Transform|MakeTransform (Math|Vector|MakeVector (+ _x -2e+01) _y (- _z 57.0)) _rotation "1,1,1")))))