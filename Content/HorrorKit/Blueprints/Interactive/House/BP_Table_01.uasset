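; BP_Table_01 is an interactive house table with a box component, likely a drawer, that the player can open and close.
; The Interactive event reacts only to the BoxTable component and ignores input while its animation plays.
; A FlipFlop alternates between playing and reversing a timeline that slides BoxTable along its relative X axis, with a positioned open or close sound.
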(event EventInteractive
  (params (Component :type Primitive%20Component%20Object%20Reference))
  (if (== Component (Variables|Default|GetBox_Table))
    (if (not (Audio|Components|Audio|IsPlaying (Variables|Default|GetAnimation_Box_Table)))
      (Utilities|FlowControl|FlipFlop
        (:A
          (Audio|PlaySoundatLocation "/Game/HorrorKit/Assets/Audio/Interactive/Box_Table/Open_Box_Cue.Open_Box_Cue" (Transformation|GetWorldLocation (Variables|Default|GetBox_Table)) "0, 0, 0" 1.0 1.0 0.0 "/Game/HorrorKit/Assets/Audio/Interactive/Wardrobe/Info_Sound_Box_WardRobe_Table.Info_Sound_Box_WardRobe_Table")
          (bind _open_close (Timeline|Animation_Box_Table Play)
            (:Update
              (Transformation|SetRelativeLocation (Variables|Default|GetBox_Table) (Math|Vector|MakeVector _open_close 0.0 0.0) false false))))
        (:B
          (Audio|PlaySoundatLocation "/Game/HorrorKit/Assets/Audio/Interactive/Box_Table/Close_Box_Cue.Close_Box_Cue" (Transformation|GetWorldLocation (Variables|Default|GetTable)) "0, 0, 0" 1.0 1.0 0.0 "/Game/HorrorKit/Assets/Audio/Interactive/Wardrobe/Info_Sound_Box_WardRobe_Table.Info_Sound_Box_WardRobe_Table")
          (Timeline|Animation_Box_Table Reverse))))))

(fn ConstructionScript)