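; Interactive wardrobe prop for the HorrorKit house, with four swinging doors (two big, two small) and two sliding boxes.
; The Interactive event matches the passed component to a part, and a per-part FlipFlop alternates between opening and closing with sounds played at the wardrobe.
; Timelines drive door yaw and box X position, reverse to close, and IsPlaying checks gate retriggering.
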(event EventInteractive
  (params (Component :type Primitive%20Component%20Object%20Reference))
  (bind _wardrobe (Variables|Default|GetWardrobe))
  (bind _wardrobe_2 (Variables|Default|GetWardrobe))
  (bind _wardrobe_3 (Variables|Default|GetWardrobe))
  (bind _wardrobe_4 (Variables|Default|GetWardrobe))
  (bind _wardrobe_5 (Variables|Default|GetWardrobe))
  (bind _wardrobe_6 (Variables|Default|GetWardrobe))
  (bind _returnvalue (Transformation|GetWorldLocation _wardrobe))
  (bind _returnvalue_2 (Transformation|GetWorldLocation _wardrobe_2))
  (bind _returnvalue_3 (Transformation|GetWorldLocation _wardrobe_3))
  (bind _returnvalue_4 (Transformation|GetWorldLocation _wardrobe_4))
  (bind _returnvalue_5 (Transformation|GetWorldLocation _wardrobe_6))
  (bind _returnvalue_6 (Transformation|GetWorldLocation _wardrobe_5))
  (if (== Component (Variables|Default|GetDoor_Left_Big))
    (if (not (Audio|Components|Audio|IsPlaying (Variables|Default|GetAnimation%20Door%20Left%20Big)))
      (Utilities|FlowControl|FlipFlop
        (:A
          (Audio|PlaySoundatLocation "/Game/HorrorKit/Assets/Audio/Interactive/Wardrobe/S_Open_Wardrobe_Cue.S_Open_Wardrobe_Cue" _returnvalue "0, 0, 0" 1.0 1.0 0.0 "/Game/HorrorKit/Assets/Audio/Interactive/Wardrobe/Info_Sound_Box_WardRobe_Table.Info_Sound_Box_WardRobe_Table")
          (bind _door (Timeline|Animation%20Door%20Left%20Big Play)
            (:Update
              (Transformation|SetRelativeRotation (Variables|Default|GetScene_Door_Left_Big) (Math|Rotator|MakeRotator 0.0 0.0 _door) false false))))
        (:B
          (Audio|PlaySoundatLocation "/Game/HorrorKit/Assets/Audio/Interactive/Wardrobe/S_Close_Wardrobe_Cue.S_Close_Wardrobe_Cue" _returnvalue "0, 0, 0" 1.0 1.0 0.0 "/Game/HorrorKit/Assets/Audio/Interactive/Wardrobe/Info_Sound_Box_WardRobe_Table.Info_Sound_Box_WardRobe_Table")
          (Timeline|Animation%20Door%20Left%20Big Reverse))))
    (elif (== Component (Variables|Default|GetDoor_Right_Big))
      (if (not (Audio|Components|Audio|IsPlaying (Variables|Default|GetAnimation%20Door%20Right%20Big)))
        (Utilities|FlowControl|FlipFlop
          (:A
            (Audio|PlaySoundatLocation "/Game/HorrorKit/Assets/Audio/Interactive/Wardrobe/S_Open_Wardrobe_Cue.S_Open_Wardrobe_Cue" _returnvalue_2 "0, 0, 0" 1.0 1.0 0.0 "/Game/HorrorKit/Assets/Audio/Interactive/Wardrobe/Info_Sound_Box_WardRobe_Table.Info_Sound_Box_WardRobe_Table")
            (bind _door_2 (Timeline|Animation%20Door%20Right%20Big Play)
              (:Update
                (Transformation|SetRelativeRotation (Variables|Default|GetScene_Door_Right_Big) (Math|Rotator|MakeRotator 0.0 0.0 _door_2) false false))))
          (:B
            (Audio|PlaySoundatLocation "/Game/HorrorKit/Assets/Audio/Interactive/Wardrobe/S_Close_Wardrobe_Cue.S_Close_Wardrobe_Cue" _returnvalue_2 "0, 0, 0" 1.0 1.0 0.0 "/Game/HorrorKit/Assets/Audio/Interactive/Wardrobe/Info_Sound_Box_WardRobe_Table.Info_Sound_Box_WardRobe_Table")
            (Timeline|Animation%20Door%20Right%20Big Reverse))))
      (elif (== Component (Variables|Default|GetDoor_Left_Small))
        (if (not (Audio|Components|Audio|IsPlaying (Variables|Default|GetAnimation%20Door%20Left%20Small)))
          (Utilities|FlowControl|FlipFlop
            (:A
              (Audio|PlaySoundatLocation "/Game/HorrorKit/Assets/Audio/Interactive/Wardrobe/S_Open_Wardrobe_Cue.S_Open_Wardrobe_Cue" _returnvalue_3 "0, 0, 0" 1.0 1.0 0.0 "/Game/HorrorKit/Assets/Audio/Interactive/Wardrobe/Info_Sound_Box_WardRobe_Table.Info_Sound_Box_WardRobe_Table")
              (bind _door_3 (Timeline|Animation%20Door%20Left%20Small Play)
                (:Update
                  (Transformation|SetRelativeRotation (Variables|Default|GetScene_Door_Left_Small) (Math|Rotator|MakeRotator 0.0 0.0 _door_3) false false))))
            (:B
              (Audio|PlaySoundatLocation "/Game/HorrorKit/Assets/Audio/Interactive/Wardrobe/S_Close_Wardrobe_Cue.S_Close_Wardrobe_Cue" _returnvalue_3 "0, 0, 0" 1.0 1.0 0.0 "/Game/HorrorKit/Assets/Audio/Interactive/Wardrobe/Info_Sound_Box_WardRobe_Table.Info_Sound_Box_WardRobe_Table")
              (Timeline|Animation%20Door%20Left%20Small Reverse))))
        (elif (== Component (Variables|Default|GetDoor_Right_Small))
          (if (not (Audio|Components|Audio|IsPlaying (Variables|Default|GetAnimation%20Door%20Right%20Small)))
            (Utilities|FlowControl|FlipFlop
              (:A
                (Audio|PlaySoundatLocation "/Game/HorrorKit/Assets/Audio/Interactive/Wardrobe/S_Open_Wardrobe_Cue.S_Open_Wardrobe_Cue" _returnvalue_4 "0, 0, 0" 1.0 1.0 0.0 "/Game/HorrorKit/Assets/Audio/Interactive/Wardrobe/Info_Sound_Box_WardRobe_Table.Info_Sound_Box_WardRobe_Table")
                (bind _door_4 (Timeline|Animation%20Door%20Right%20Small Play)
                  (:Update
                    (Transformation|SetRelativeRotation (Variables|Default|GetScene_Door_Right_Small) (Math|Rotator|MakeRotator 0.0 0.0 _door_4) false false))))
              (:B
                (Audio|PlaySoundatLocation "/Game/HorrorKit/Assets/Audio/Interactive/Wardrobe/S_Close_Wardrobe_Cue.S_Close_Wardrobe_Cue" _returnvalue_4 "0, 0, 0" 1.0 1.0 0.0 "/Game/HorrorKit/Assets/Audio/Interactive/Wardrobe/Info_Sound_Box_WardRobe_Table.Info_Sound_Box_WardRobe_Table")
                (Timeline|Animation%20Door%20Right%20Small Reverse))))
          (elif (== Component (Variables|Default|GetBox_02))
            (if (not (Audio|Components|Audio|IsPlaying (Variables|Default|GetAnimation_Box_02)))
              (Utilities|FlowControl|FlipFlop
                (:A
                  (Audio|PlaySoundatLocation "/Game/HorrorKit/Assets/Audio/Interactive/Box_Table/Open_Box_Cue.Open_Box_Cue" _returnvalue_5 "0, 0, 0" 1.0 1.0 0.0 "/Game/HorrorKit/Assets/Audio/Interactive/Wardrobe/Info_Sound_Box_WardRobe_Table.Info_Sound_Box_WardRobe_Table")
                  (bind _door_5 (Timeline|Animation_Box_02 Play)
                    (:Update
                      (Transformation|SetRelativeLocation (Variables|Default|GetBox_02) (Math|Vector|MakeVector _door_5 0.0 0.0) false false))))
                (:B
                  (Audio|PlaySoundatLocation "/Game/HorrorKit/Assets/Audio/Interactive/Box_Table/Close_Box_Cue.Close_Box_Cue" _returnvalue_5 "0, 0, 0" 1.0 1.0 0.0 "/Game/HorrorKit/Assets/Audio/Interactive/Wardrobe/Info_Sound_Box_WardRobe_Table.Info_Sound_Box_WardRobe_Table")
                  (Timeline|Animation_Box_02 Reverse))))
            (elif (== Component (Variables|Default|GetBox_01))
              (if (not (Audio|Components|Audio|IsPlaying (Variables|Default|GetAnimation%20Box_01)))
                (Utilities|FlowControl|FlipFlop
                  (:A
                    (Audio|PlaySoundatLocation "/Game/HorrorKit/Assets/Audio/Interactive/Box_Table/Open_Box_Cue.Open_Box_Cue" _returnvalue_6 "0, 0, 0" 1.0 1.0 0.0 "/Game/HorrorKit/Assets/Audio/Interactive/Wardrobe/Info_Sound_Box_WardRobe_Table.Info_Sound_Box_WardRobe_Table")
                    (bind _door_6 (Timeline|Animation%20Box_01 Play)
                      (:Update
                        (Transformation|SetRelativeLocation (Variables|Default|GetBox_01) (Math|Vector|MakeVector _door_6 0.0 0.0) false false))))
                  (:B
                    (Audio|PlaySoundatLocation "/Game/HorrorKit/Assets/Audio/Interactive/Box_Table/Close_Box_Cue.Close_Box_Cue" _returnvalue_6 "0, 0, 0" 1.0 1.0 0.0 "/Game/HorrorKit/Assets/Audio/Interactive/Wardrobe/Info_Sound_Box_WardRobe_Table.Info_Sound_Box_WardRobe_Table")
                    (Timeline|Animation%20Box_01 Reverse)))))))))))

(fn ConstructionScript)