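; BP_Lamp_01 is an interactive house lamp that switches its point light on and off.
; The Interactive event alternates through a FlipFlop between two timelines that move the button along Z, ignoring input while either plays.
; When either timeline finishes, the FlipFlop state sets the light's visibility and picks the on or off sound played at the lamp's location.
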(event EventInteractive
  (params (Component :type Primitive%20Component%20Object%20Reference))
  (if (not (or (Audio|Components|Audio|IsPlaying (Variables|Default|GetAnimation%20Button)) (Audio|Components|Audio|IsPlaying (Variables|Default|GetAnimation%20Reverse))))
    (bind _isa (Utilities|FlowControl|FlipFlop)
      (:A
        (bind _button (Timeline|Animation%20Button PlayFromStart)
          (:Update
            (Transformation|SetRelativeLocation (Variables|Default|GetButton) (Math|Vector|MakeVector 0.0 0.0 _button) false false))
          (:Finished
            (Rendering|SetVisibility (Variables|Default|GetPointLight) _isa false :!label _label)
            (Audio|PlaySoundatLocation (select _isa "/Game/HorrorKit/Assets/Audio/Interactive/Switch/S_On_Lamp_Cue.S_On_Lamp_Cue" "/Game/HorrorKit/Assets/Audio/Interactive/Switch/S_Off_Lamp_Cue.S_Off_Lamp_Cue") (Transformation|GetWorldLocation (Variables|Default|GetLamp)) "0, 0, 0" 1.0 1.0 0.0 "/Game/HorrorKit/Assets/Audio/Interactive/Switch/Info_Sound_Switch.Info_Sound_Switch"))))
      (:B
        (bind _button_2 (Timeline|Animation%20Reverse PlayFromStart)
          (:Update
            (Transformation|SetRelativeLocation (Variables|Default|GetButton) (Math|Vector|MakeVector 0.0 0.0 _button_2) false false))
          (:Finished
            (goto _label)))))))

(fn ConstructionScript)