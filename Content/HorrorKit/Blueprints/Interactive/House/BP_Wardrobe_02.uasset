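; BP_Wardrobe_02 is an interactive house wardrobe with left and right big doors that open and close independently.
; The Interactive event checks which door component was used and ignores it while that door's timeline is still playing.
; A FlipFlop per door alternates open and close, playing a sound at the wardrobe and running the timeline forward or in reverse to set the door scene component's yaw.
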(event EventInteractive
  (params (Component :type Primitive%20Component%20Object%20Reference))
  (bind _wardrobe (Variables|Default|GetWardrobe))
  (bind _wardrobe_2 (Variables|Default|GetWardrobe))
  (bind _returnvalue (Transformation|GetWorldLocation _wardrobe))
  (bind _returnvalue_2 (Transformation|GetWorldLocation _wardrobe_2))
  (if (== Component (Variables|Default|GetDoor_Left_Big))
    (if (not (Audio|Components|Audio|IsPlaying (Variables|Default|GetAnimation%20Door%20Left%20Big)))
      (Utilities|FlowControl|FlipFlop
        (:A
          (Audio|PlaySoundatLocation "/Game/HorrorKit/Assets/Audio/Interactive/Wardrobe/S_Open_Wardrobe_Cue.S_Open_Wardrobe_Cue" _returnvalue_2 "0, 0, 0" 1.0 1.0 0.0 "/Game/HorrorKit/Assets/Audio/Interactive/Wardrobe/Info_Sound_Box_WardRobe_Table.Info_Sound_Box_WardRobe_Table")
          (bind _door (Timeline|Animation%20Door%20Left%20Big Play)
            (:Update
              (Transformation|SetRelativeRotation (Variables|Default|GetScene_Door_Left_Big) (Math|Rotator|MakeRotator 0.0 0.0 _door) false false))))
        (:B
          (Audio|PlaySoundatLocation "/Game/HorrorKit/Assets/Audio/Interactive/Wardrobe/S_Close_Wardrobe_Cue.S_Close_Wardrobe_Cue" _returnvalue_2 "0, 0, 0" 1.0 1.0 0.0 "/Game/HorrorKit/Assets/Audio/Interactive/Wardrobe/Info_Sound_Box_WardRobe_Table.Info_Sound_Box_WardRobe_Table")
          (Timeline|Animation%20Door%20Left%20Big Reverse))))
    (elif (== Component (Variables|Default|GetDoor_Right_Big))
      (if (not (Audio|Components|Audio|IsPlaying (Variables|Default|GetAnimation%20Door%20Right%20Big)))
        (Utilities|FlowControl|FlipFlop
          (:A
            (Audio|PlaySoundatLocation "/Game/HorrorKit/Assets/Audio/Interactive/Wardrobe/S_Open_Wardrobe_Cue.S_Open_Wardrobe_Cue" _returnvalue "0, 0, 0" 1.0 1.0 0.0 "/Game/HorrorKit/Assets/Audio/Interactive/Wardrobe/Info_Sound_Box_WardRobe_Table.Info_Sound_Box_WardRobe_Table")
            (bind _door_2 (Timeline|Animation%20Door%20Right%20Big Play)
              (:Update
                (Transformation|SetRelativeRotation (Variables|Default|GetScene_Door_Right_Big) (Math|Rotator|MakeRotator 0.0 0.0 _door_2) false false))))
          (:B
            (Audio|PlaySoundatLocation "/Game/HorrorKit/Assets/Audio/Interactive/Wardrobe/S_Close_Wardrobe_Cue.S_Close_Wardrobe_Cue" _returnvalue "0, 0, 0" 1.0 1.0 0.0 "/Game/HorrorKit/Assets/Audio/Interactive/Wardrobe/Info_Sound_Box_WardRobe_Table.Info_Sound_Box_WardRobe_Table")
            (Timeline|Animation%20Door%20Right%20Big Reverse)))))))

(fn ConstructionScript)