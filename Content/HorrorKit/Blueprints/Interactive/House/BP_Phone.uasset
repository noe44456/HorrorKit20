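; Interactive house phone for the horror kit that can ring until the player picks up its handset.
; A delayed event loop replays a spawned ring sound while Call is set.
; Interacting waits for any pistol or flashlight to be put away, attaches the handset to the character, shows the cord and stops the ringing.
; Interacting again or leaving the box snaps the handset back onto its base.
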(event Custom|Event%20Call%20Phone
  (if (Variables|Phone|GetCall)
    (Audio|Components|Audio|Play (Variables|Default|GetSound) 0.0)
    (Utilities|FlowControl|Delay (Variables|Phone|GetTime_Drop_Call))
    (if (Variables|Phone|GetCall)
      (CallFunction|EventCallPhone))))

(fn ConstructionScript)

(event EventBeginPlay
  (bind _asmy_character (Utilities|Casting|CastToMyCharacter (Game|GetPlayerCharacter 0)))
  (Variables|Default|SetCharacter _asmy_character)
  (bind _returnvalue (Audio|SpawnSoundatLocation "/Game/HorrorKit/Assets/Audio/Interactive/Phone/S_Call_Phone_Cue.S_Call_Phone_Cue" (Transformation|GetWorldLocation (Variables|Default|GetPhone)) "0, 0, 0" 1.0 1.0 0.0 "/Game/HorrorKit/Assets/Audio/Interactive/Phone/Info_Sound_Phone.Info_Sound_Phone" 0 false))
  (bind _output_get (Variables|Default|SetSound _returnvalue))
  (Audio|Components|Audio|Stop _output_get)
  (CallFunction|EventCallPhone))

(event OnComponentEndOverlap(Box)
  (params (OverlappedComponent :type Primitive%20Component%20Object%20Reference) (OtherActor :type Actor%20Object%20Reference) (OtherComp :type Primitive%20Component%20Object%20Reference) (OtherBodyIndex :type Integer))
  (Utilities|IsValid (Variables|Default|GetCharacter)
    (:Is%20Valid
      (if (== (Transformation|GetAttachParent (Variables|Default|GetTube)) (Variables|/Game/HorrorKit/Blueprints/Player/MyCharacter.MyCharacter_C|GetScene_Phone (Variables|Default|GetCharacter)))
        (CallFunction|EventDetach)))))

(event Custom|Event_Detach
  (Audio|PlaySoundatLocation "/Game/HorrorKit/Assets/Audio/Interactive/Phone/S_Drop_Phone_Cue.S_Drop_Phone_Cue" (Transformation|GetWorldLocation (Variables|Default|GetPhone)) "0, 0, 0" 1.0 1.0 0.0 "/Game/HorrorKit/Assets/Audio/Interactive/Phone/Info_Sound_Phone.Info_Sound_Phone")
  ;[0 0 0] Lay Phone
  (Transformation|DetachFromComponent (Variables|Default|GetTube) "KeepRelative" "KeepRelative" "KeepRelative" true)
  (Transformation|AttachComponentToComponent (Variables|Default|GetTube) (Variables|Default|GetScene_Tube) "None" "SnapToTarget" "SnapToTarget" "KeepRelative" true)
  (Collision|SetCollisionEnabled (Variables|Default|GetTube) "QueryAndPhysics")
  (Development|SetHiddeninGame (Variables|Default|GetCable_Phone) true false)
  (Variables|/Game/HorrorKit/Blueprints/Player/MyCharacter.MyCharacter_C|SetUse%20Phone (Variables|Default|GetCharacter) false))

(event EventInteractive
  (params (Component :type Primitive%20Component%20Object%20Reference))
  (bind _phone (Variables|Default|GetPhone))
  (bind _returnvalue (Transformation|GetWorldLocation _phone))
  (if (not (Variables|/Game/HorrorKit/Blueprints/Weapons/Guns_Component.Guns_Component_C|GetUse%20Animation (Variables|/Game/HorrorKit/Blueprints/Player/MyCharacter.MyCharacter_C|GetGuns_Component (Variables|Default|GetCharacter))))
    (if (== (Transformation|GetAttachParent (Variables|Default|GetTube)) (Variables|/Game/HorrorKit/Blueprints/Player/MyCharacter.MyCharacter_C|GetScene_Phone (Variables|Default|GetCharacter)))
      (Audio|PlaySoundatLocation "/Game/HorrorKit/Assets/Audio/Interactive/Phone/S_Drop_Phone_Cue.S_Drop_Phone_Cue" _returnvalue "0, 0, 0" 1.0 1.0 0.0 "/Game/HorrorKit/Assets/Audio/Interactive/Phone/Info_Sound_Phone.Info_Sound_Phone")
      ;[0 0 0] Lay Phone
      (Transformation|DetachFromComponent (Variables|Default|GetTube) "KeepRelative" "KeepRelative" "KeepRelative" true)
      (Transformation|AttachComponentToComponent (Variables|Default|GetTube) (Variables|Default|GetScene_Tube) "None" "SnapToTarget" "SnapToTarget" "KeepRelative" true)
      (Collision|SetCollisionEnabled (Variables|Default|GetTube) "QueryAndPhysics")
      (Development|SetHiddeninGame (Variables|Default|GetCable_Phone) true false)
      (Variables|/Game/HorrorKit/Blueprints/Player/MyCharacter.MyCharacter_C|SetUse%20Phone (Variables|Default|GetCharacter) false)
      (else
        (if (Utilities|IsValidClass (Variables|/Script/Engine.ChildActorComponent|GetChildActorClass (Variables|/Game/HorrorKit/Blueprints/Player/MyCharacter.MyCharacter_C|GetGun (Variables|Default|GetCharacter))))
          (Variables|/Game/HorrorKit/Blueprints/Player/Character/Animations/Anim_MyCharacter.Anim_MyCharacter_C|SetTake_Pistol (Variables|/Game/HorrorKit/Blueprints/Player/MyCharacter.MyCharacter_C|GetAnim_Blueprint (Variables|Default|GetCharacter)) false)
          (Utilities|FlowControl|Delay 2.0)
          (elif (Rendering|IsVisible (Variables|/Game/HorrorKit/Blueprints/Player/MyCharacter.MyCharacter_C|GetFlashLight (Variables|Default|GetCharacter)))
            (Default|EventNotTakeFlashLight (Variables|Default|GetCharacter))
            (Utilities|FlowControl|Delay 1.2)))
        (Audio|PlaySoundatLocation "/Game/HorrorKit/Assets/Audio/Interactive/Phone/S_PickUp_Phone_Cue.S_PickUp_Phone_Cue" _returnvalue "0, 0, 0" 1.0 1.0 0.0 "/Game/HorrorKit/Assets/Audio/Interactive/Phone/Info_Sound_Phone.Info_Sound_Phone")
        ;[0 0 0] Take Phone
        (Transformation|DetachFromComponent (Variables|Default|GetTube) "KeepRelative" "KeepRelative" "KeepRelative" true)
        (Transformation|AttachComponentToComponent (Variables|Default|GetTube) (Variables|/Game/HorrorKit/Blueprints/Player/MyCharacter.MyCharacter_C|GetScene_Phone (Variables|Default|GetCharacter)) "None" "SnapToTarget" "SnapToTarget" "KeepRelative" true)
        (Collision|SetCollisionEnabled (Variables|Default|GetTube) "NoCollision")
        (Development|SetHiddeninGame (Variables|Default|GetCable_Phone) false false)
        (Variables|Phone|SetCall false)
        (Audio|Components|Audio|Stop (Variables|Default|GetSound))
        (Variables|/Game/HorrorKit/Blueprints/Player/MyCharacter.MyCharacter_C|SetUse%20Phone (Variables|Default|GetCharacter) true)))))