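; Interactive kitchen stove for HorrorKit with an animated oven door, sliding box and five rotating knobs.
; The Interactive event branches on the touched component, using FlipFlops to play or reverse timelines with sound cues.
; Knobs control loop sounds spawned at BeginPlay, with Button01 and Button02 sharing the first.
; Knobs 02–05 also toggle their fire effect and point light, flickered by looping timers that randomize intensity.
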(event Custom|Event%20Light_05
  (CallFunction|RandomLight (Variables|Default|GetPointLight_05)))

(event Custom|Event%20Light_02
  (CallFunction|RandomLight (Variables|Default|GetPointLight_02)))

(event Custom|Event%20Light_03
  (CallFunction|RandomLight (Variables|Default|GetPointLight_03)))

(event Custom|Event%20Light_04
  (CallFunction|RandomLight (Variables|Default|GetPointLight_04)))

(event EventInteractive
  (params (Component :type Primitive%20Component%20Object%20Reference))
  (bind _sounds (Variables|Default|GetSounds))
  (bind _sounds_2 (Variables|Default|GetSounds))
  (bind _sounds_3 (Variables|Default|GetSounds))
  (bind _sounds_4 (Variables|Default|GetSounds))
  (bind _sounds_5 (Variables|Default|GetSounds))
  (bind _output (Utilities|Array|Get(acopy) _sounds_5))
  (bind _output_2 (Utilities|Array|Get(acopy) _sounds))
  (bind _output_3 (Utilities|Array|Get(acopy) _sounds_2 1))
  (bind _output_4 (Utilities|Array|Get(acopy) _sounds_3 2))
  (bind _output_5 (Utilities|Array|Get(acopy) _sounds_4 3))
  (if (== Component (Variables|Default|GetDoor))
    (if (not (Audio|Components|Audio|IsPlaying (Variables|Default|GetAnimation%20Door)))
      (Utilities|FlowControl|FlipFlop
        (:A
          (Audio|PlaySoundatLocation "/Game/HorrorKit/Assets/Audio/Interactive/Plate/S_Open_Door_Plate_Cue.S_Open_Door_Plate_Cue" (Transformation|GetWorldLocation (Variables|Default|GetPlate)) "0, 0, 0" 1.0 1.0 0.0 "/Game/HorrorKit/Assets/Audio/Interactive/Plate/Info_Sound_Plate.Info_Sound_Plate")
          (bind _door (Timeline|Animation%20Door Play)
            (:Update
              (Transformation|SetRelativeRotation (Variables|Default|GetScene_Door) (Math|Rotator|MakeRotator 0.0 _door 0.0) false false))))
        (:B
          (Utilities|FlowControl|Sequence
            (:then_0
              (Timeline|Animation%20Door Reverse))
            (:then_1
              (Utilities|FlowControl|Delay 0.4)
              (Audio|PlaySoundatLocation "/Game/HorrorKit/Assets/Audio/Interactive/Plate/S_Close_Door_Plate_Cue.S_Close_Door_Plate_Cue" (Transformation|GetWorldLocation (Variables|Default|GetPlate)) "0, 0, 0" 1.0 1.0 0.0 "/Game/HorrorKit/Assets/Audio/Interactive/Plate/Info_Sound_Plate.Info_Sound_Plate")
              (Timeline|Animation%20Door Reverse))))))
    (elif (== Component (Variables|Default|GetBox))
      (if (not (Audio|Components|Audio|IsPlaying (Variables|Default|GetAnimation%20Box)))
        (Utilities|FlowControl|FlipFlop
          (:A
            (Audio|PlaySoundatLocation "/Game/HorrorKit/Assets/Audio/Interactive/Plate/S_Open_Box_Plate_Cue.S_Open_Box_Plate_Cue" (Transformation|GetWorldLocation (Variables|Default|GetPlate)) "0, 0, 0" 1.0 1.0 0.0 "/Game/HorrorKit/Assets/Audio/Interactive/Plate/Info_Sound_Plate.Info_Sound_Plate")
            (bind _door_2 (Timeline|Animation%20Box Play)
              (:Update
                (Transformation|SetRelativeLocation (Variables|Default|GetBox) (Math|Vector|MakeVector _door_2 0.0 0.0) false false))))
          (:B
            (Audio|PlaySoundatLocation "/Game/HorrorKit/Assets/Audio/Interactive/Plate/S_Close_Box_Plate_Cue.S_Close_Box_Plate_Cue" (Transformation|GetWorldLocation (Variables|Default|GetPlate)) "0, 0, 0" 1.0 1.0 0.0 "/Game/HorrorKit/Assets/Audio/Interactive/Plate/Info_Sound_Plate.Info_Sound_Plate")
            (Timeline|Animation%20Box Reverse))))
      (elif (== Component (Variables|Default|GetButton_01))
        (if (not (Audio|Components|Audio|IsPlaying (Variables|Default|GetAnimation_Button_01)))
          (bind _isa (Utilities|FlowControl|FlipFlop)
            (:A
              (Audio|PlaySoundatLocation "/Game/HorrorKit/Assets/Audio/Interactive/Plate/S_On_Plate_Cue.S_On_Plate_Cue" (Transformation|GetWorldLocation (Variables|Default|GetPlate)) "0, 0, 0" 1.0 1.0 0.0 "/Game/HorrorKit/Assets/Audio/Interactive/Plate/Info_Sound_Plate.Info_Sound_Plate")
              (bind _button (Timeline|Animation_Button_01 Play)
                (:Update
                  (Transformation|SetRelativeRotation (Variables|Default|GetButton_01) (Math|Rotator|MakeRotator _button 0.0 0.0) false false))
                (:Finished
                  (if _isa
                    (Audio|Components|Audio|Play _output 0.0)
                    (else
                      (Audio|Components|Audio|Stop _output))))))
            (:B
              (Audio|PlaySoundatLocation "/Game/HorrorKit/Assets/Audio/Interactive/Plate/S_Off_Plate_Cue.S_Off_Plate_Cue" (Transformation|GetWorldLocation (Variables|Default|GetPlate)) "0, 0, 0" 1.0 1.0 0.0 "/Game/HorrorKit/Assets/Audio/Interactive/Plate/Info_Sound_Plate.Info_Sound_Plate")
              (Timeline|Animation_Button_01 Reverse))))
        (elif (== Component (Variables|Default|GetButton_02))
          (if (not (Audio|Components|Audio|IsPlaying (Variables|Default|GetAnimation_Button_02)))
            (bind _isa_2 (Utilities|FlowControl|FlipFlop)
              (:A
                (Audio|PlaySoundatLocation "/Game/HorrorKit/Assets/Audio/Interactive/Plate/S_On_Plate_Cue.S_On_Plate_Cue" (Transformation|GetWorldLocation (Variables|Default|GetPlate)) "0, 0, 0" 1.0 1.0 0.0 "/Game/HorrorKit/Assets/Audio/Interactive/Plate/Info_Sound_Plate.Info_Sound_Plate")
                (bind _button_2 (Timeline|Animation_Button_02 Play)
                  (:Update
                    (Transformation|SetRelativeRotation (Variables|Default|GetButton_02) (Math|Rotator|MakeRotator _button_2 0.0 0.0) false false))
                  (:Finished
                    (Components|Activation|SetActive (Variables|Default|GetFire_02) _isa_2 false)
                    (if _isa_2
                      (Audio|Components|Audio|Play _output_2 0.0)
                      (bind _returnvalue (Utilities|Time|SetTimerbyEvent (delegate Custom|Event%20Light_02) 0.1 true))
                      (Variables|Default|SetTimer_02 _returnvalue)
                      (Rendering|SetVisibility (Variables|Default|GetPointLight_02) true false)
                      (else
                        (Audio|Components|Audio|Stop _output_2)
                        (Utilities|Time|ClearandInvalidateTimerbyHandle (Variables|Default|GetTimer_02))
                        (Rendering|SetVisibility (Variables|Default|GetPointLight_02) false false))))))
              (:B
                (Audio|PlaySoundatLocation "/Game/HorrorKit/Assets/Audio/Interactive/Plate/S_Off_Plate_Cue.S_Off_Plate_Cue" (Transformation|GetWorldLocation (Variables|Default|GetPlate)) "0, 0, 0" 1.0 1.0 0.0 "/Game/HorrorKit/Assets/Audio/Interactive/Plate/Info_Sound_Plate.Info_Sound_Plate")
                (Timeline|Animation_Button_02 Reverse))))
          (elif (== Component (Variables|Default|GetButton_03))
            (if (not (Audio|Components|Audio|IsPlaying (Variables|Default|GetAnimation_Button_03)))
              (bind _isa_3 (Utilities|FlowControl|FlipFlop)
                (:A
                  (Audio|PlaySoundatLocation "/Game/HorrorKit/Assets/Audio/Interactive/Plate/S_On_Plate_Cue.S_On_Plate_Cue" (Transformation|GetWorldLocation (Variables|Default|GetPlate)) "0, 0, 0" 1.0 1.0 0.0 "/Game/HorrorKit/Assets/Audio/Interactive/Plate/Info_Sound_Plate.Info_Sound_Plate")
                  (bind _button_3 (Timeline|Animation_Button_03 Play)
                    (:Update
                      (Transformation|SetRelativeRotation (Variables|Default|GetButton_03) (Math|Rotator|MakeRotator _button_3 0.0 0.0) false false))
                    (:Finished
                      (Components|Activation|SetActive (Variables|Default|GetFire_03) _isa_3 false)
                      (if _isa_3
                        (Audio|Components|Audio|Play _output_3 0.0)
                        (bind _returnvalue_2 (Utilities|Time|SetTimerbyEvent (delegate Custom|Event%20Light_03) 0.1 true))
                        (Variables|Default|SetTimer_03 _returnvalue_2)
                        (Rendering|SetVisibility (Variables|Default|GetPointLight_03) true false)
                        (else
                          (Audio|Components|Audio|Stop _output_3)
                          (Utilities|Time|ClearandInvalidateTimerbyHandle (Variables|Default|GetTimer_03))
                          (Rendering|SetVisibility (Variables|Default|GetPointLight_03) false false))))))
                (:B
                  (Audio|PlaySoundatLocation "/Game/HorrorKit/Assets/Audio/Interactive/Plate/S_Off_Plate_Cue.S_Off_Plate_Cue" (Transformation|GetWorldLocation (Variables|Default|GetPlate)) "0, 0, 0" 1.0 1.0 0.0 "/Game/HorrorKit/Assets/Audio/Interactive/Plate/Info_Sound_Plate.Info_Sound_Plate")
                  (Timeline|Animation_Button_03 Reverse))))
            (elif (== Component (Variables|Default|GetButton_04))
              (if (not (Audio|Components|Audio|IsPlaying (Variables|Default|GetAnimation_Button_04)))
                (bind _isa_4 (Utilities|FlowControl|FlipFlop)
                  (:A
                    (Audio|PlaySoundatLocation "/Game/HorrorKit/Assets/Audio/Interactive/Plate/S_On_Plate_Cue.S_On_Plate_Cue" (Transformation|GetWorldLocation (Variables|Default|GetPlate)) "0, 0, 0" 1.0 1.0 0.0 "/Game/HorrorKit/Assets/Audio/Interactive/Plate/Info_Sound_Plate.Info_Sound_Plate")
                    (bind _button_4 (Timeline|Animation_Button_04 Play)
                      (:Update
                        (Transformation|SetRelativeRotation (Variables|Default|GetButton_04) (Math|Rotator|MakeRotator _button_4 0.0 0.0) false false))
                      (:Finished
                        (Components|Activation|SetActive (Variables|Default|GetFire_04) _isa_4 false)
                        (if _isa_4
                          (Audio|Components|Audio|Play _output_4 0.0)
                          (bind _returnvalue_3 (Utilities|Time|SetTimerbyEvent (delegate Custom|Event%20Light_04) 0.1 true))
                          (Variables|Default|SetTimer_04 _returnvalue_3)
                          (Rendering|SetVisibility (Variables|Default|GetPointLight_04) true false)
                          (else
                            (Audio|Components|Audio|Stop _output_4)
                            (Utilities|Time|ClearandInvalidateTimerbyHandle (Variables|Default|GetTimer_04))
                            (Rendering|SetVisibility (Variables|Default|GetPointLight_04) false false))))))
                  (:B
                    (Audio|PlaySoundatLocation "/Game/HorrorKit/Assets/Audio/Interactive/Plate/S_Off_Plate_Cue.S_Off_Plate_Cue" (Transformation|GetWorldLocation (Variables|Default|GetPlate)) "0, 0, 0" 1.0 1.0 0.0 "/Game/HorrorKit/Assets/Audio/Interactive/Plate/Info_Sound_Plate.Info_Sound_Plate")
                    (Timeline|Animation_Button_04 Reverse))))
              (elif (== Component (Variables|Default|GetButton_05))
                (if (not (Audio|Components|Audio|IsPlaying (Variables|Default|GetAnimation_Button_05)))
                  (bind _isa_5 (Utilities|FlowControl|FlipFlop)
                    (:A
                      (Audio|PlaySoundatLocation "/Game/HorrorKit/Assets/Audio/Interactive/Plate/S_On_Plate_Cue.S_On_Plate_Cue" (Transformation|GetWorldLocation (Variables|Default|GetPlate)) "0, 0, 0" 1.0 1.0 0.0 "/Game/HorrorKit/Assets/Audio/Interactive/Plate/Info_Sound_Plate.Info_Sound_Plate")
                      (bind _button_5 (Timeline|Animation_Button_05 Play)
                        (:Update
                          (Transformation|SetRelativeRotation (Variables|Default|GetButton_05) (Math|Rotator|MakeRotator _button_5 0.0 0.0) false false))
                        (:Finished
                          (Components|Activation|SetActive (Variables|Default|GetFire_05) _isa_5 false)
                          (if _isa_5
                            (Audio|Components|Audio|Play _output_5 0.0)
                            (bind _returnvalue_4 (Utilities|Time|SetTimerbyEvent (delegate Custom|Event%20Light_05) 0.1 true))
                            (Variables|Default|SetTimer_05 _returnvalue_4)
                            (Rendering|SetVisibility (Variables|Default|GetPointLight_05) true false)
                            (else
                              (Audio|Components|Audio|Stop _output_5)
                              (Utilities|Time|ClearandInvalidateTimerbyHandle (Variables|Default|GetTimer_05))
                              (Rendering|SetVisibility (Variables|Default|GetPointLight_05) false false))))))
                    (:B
                      (Audio|PlaySoundatLocation "/Game/HorrorKit/Assets/Audio/Interactive/Plate/S_Off_Plate_Cue.S_Off_Plate_Cue" (Transformation|GetWorldLocation (Variables|Default|GetPlate)) "0, 0, 0" 1.0 1.0 0.0 "/Game/HorrorKit/Assets/Audio/Interactive/Plate/Info_Sound_Plate.Info_Sound_Plate")
                      (Timeline|Animation_Button_05 Reverse))))))))))))

(fn ConstructionScript)

(fn RandomLight
  (params (Light :type Point%20Light%20Component%20Object%20Reference))
  (Rendering|Components|Light|SetIntensity Light (Utilities|Select :Index (Math|Random|RandomIntegerinRange 0 4) :Option%200 1e+03 :Option%201 8e+02 :Option%202 6e+02 :Option%203 4e+02 :Option%204 2e+02)))

(event EventBeginPlay
  (for _index (range 0 4)
    (bind _returnvalue (Audio|SpawnSoundatLocation "/Game/HorrorKit/Assets/Audio/Interactive/Plate/S_Loop_Plate.S_Loop_Plate" (Transformation|GetWorldLocation (Variables|Default|GetPlate)) "0, 0, 0" 1.0 1.0 0.0 "/Game/HorrorKit/Assets/Audio/Interactive/Plate/Info_Sound_Plate.Info_Sound_Plate" 0 false))
    (Utilities|Array|Add (Variables|Default|GetSounds) _returnvalue)
    (Audio|Components|Audio|Stop _returnvalue)))