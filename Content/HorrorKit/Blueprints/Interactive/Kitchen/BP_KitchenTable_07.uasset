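; Interactive kitchen table prop in HorrorKit with two doors that open and close on player interaction.
; The Interactive event checks whether the right or left door component was used and ignores it while the checked door animation is playing.
; Each door's FlipFlop alternates playing and reversing a timeline that yaws its scene pivot, with wardrobe open and close sounds at the table.
; Timeline names are crossed: DoorRight uses the Left timeline and DoorLeft the Right.
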(event EventInteractive
  (params (Component :type Primitive%20Component%20Object%20Reference))
  (bind _table (Variables|Default|GetTable))
  (bind _table_2 (Variables|Default|GetTable))
  (bind _returnvalue (Transformation|GetWorldLocation _table))
  (bind _returnvalue_2 (Transformation|GetWorldLocation _table_2))
  (if (== Component (Variables|Default|GetDoor_Right))
    (if (not (Audio|Components|Audio|IsPlaying (Variables|Default|GetAnimation%20Door_Left)))
      (Utilities|FlowControl|FlipFlop
        (:A
          (Audio|PlaySoundatLocation "/Game/HorrorKit/Assets/Audio/Interactive/Wardrobe/S_Open_Wardrobe_Cue.S_Open_Wardrobe_Cue" _returnvalue "0, 0, 0" 1.0 1.0 0.0 "/Game/HorrorKit/Assets/Audio/Interactive/Wardrobe/Info_Sound_Box_WardRobe_Table.Info_Sound_Box_WardRobe_Table")
          (bind _door (Timeline|Animation%20Door_Left Play)
            (:Update
              (Transformation|SetRelativeRotation (Variables|Default|GetScene_Door_Right) (Math|Rotator|MakeRotator 0.0 0.0 _door) false false))))
        (:B
          (Audio|PlaySoundatLocation "/Game/HorrorKit/Assets/Audio/Interactive/Wardrobe/S_Close_Wardrobe_Cue.S_Close_Wardrobe_Cue" _returnvalue "0, 0, 0" 1.0 1.0 0.0 "/Game/HorrorKit/Assets/Audio/Interactive/Wardrobe/Info_Sound_Box_WardRobe_Table.Info_Sound_Box_WardRobe_Table")
          (Timeline|Animation%20Door_Left Reverse))))
    (elif (== Component (Variables|Default|GetDoor_Left))
      (if (not (Audio|Components|Audio|IsPlaying (Variables|Default|GetAnimation%20Door_Right)))
        (Utilities|FlowControl|FlipFlop
          (:A
            (Audio|PlaySoundatLocation "/Game/HorrorKit/Assets/Audio/Interactive/Wardrobe/S_Open_Wardrobe_Cue.S_Open_Wardrobe_Cue" _returnvalue_2 "0, 0, 0" 1.0 1.0 0.0 "/Game/HorrorKit/Assets/Audio/Interactive/Wardrobe/Info_Sound_Box_WardRobe_Table.Info_Sound_Box_WardRobe_Table")
            (bind _door_2 (Timeline|Animation%20Door_Right Play)
              (:Update
                (Transformation|SetRelativeRotation (Variables|Default|GetScene_Door_Left) (Math|Rotator|MakeRotator 0.0 0.0 _door_2) false false))))
          (:B
            (Audio|PlaySoundatLocation "/Game/HorrorKit/Assets/Audio/Interactive/Wardrobe/S_Close_Wardrobe_Cue.S_Close_Wardrobe_Cue" _returnvalue_2 "0, 0, 0" 1.0 1.0 0.0 "/Game/HorrorKit/Assets/Audio/Interactive/Wardrobe/Info_Sound_Box_WardRobe_Table.Info_Sound_Box_WardRobe_Table")
            (Timeline|Animation%20Door_Right Reverse)))))))

(fn ConstructionScript)