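; Interactive kitchen extractor hood with three speed buttons and a light button, each clicking and sliding between two positions via FlipFlop.
; The Interactive event routes by component, with per-button flags blocking re-presses during movement.
; Pressing a speed button releases the others through FDefault, though speeds drive no fan behavior here.
; The light button toggles the SpotLight and swaps the hood's light material.
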(event Custom|Event%20Button_01
  (if (stale _isa)
    (Audio|PlaySoundatLocation "/Game/HorrorKit/Assets/Audio/Interactive/Extractor_Hood/S_Button_Extractor_Hood_Cue.S_Button_Extractor_Hood_Cue" (Transformation|GetWorldLocation (Variables|Default|GetExtractor_Hood)) "0, 0, 0" 1.0 1.0 0.0 "/Game/HorrorKit/Assets/Audio/Interactive/Extractor_Hood/Info_Sound_Extractor_Hood.Info_Sound_Extractor_Hood")
    (bind _isa (Utilities|FlowControl|FlipFlop)
      (:A
        _)
      (:B
        _))
    (Components|MoveComponentTo (Variables|Default|GetButton_Speed_01) (Math|Vector|MakeVector (Math|Float|SelectFloat -0.8 0.0 _isa) 0.0 0.0) "0, 0, 0" false false 0.2 false)
    (Variables|Default|SetButton_01 false)))

(event Custom|Event%20Button_02
  (if (stale _isa)
    (Audio|PlaySoundatLocation "/Game/HorrorKit/Assets/Audio/Interactive/Extractor_Hood/S_Button_Extractor_Hood_Cue.S_Button_Extractor_Hood_Cue" (Transformation|GetWorldLocation (Variables|Default|GetExtractor_Hood)) "0, 0, 0" 1.0 1.0 0.0 "/Game/HorrorKit/Assets/Audio/Interactive/Extractor_Hood/Info_Sound_Extractor_Hood.Info_Sound_Extractor_Hood")
    (bind _isa (Utilities|FlowControl|FlipFlop)
      (:A
        _)
      (:B
        _))
    (Components|MoveComponentTo (Variables|Default|GetButton_Speed_02) (Math|Vector|MakeVector (Math|Float|SelectFloat -0.8 0.0 _isa) 0.0 0.0) "0, 0, 0" false false 0.2 false)
    (Variables|Default|SetButton_02 false)))

(event Custom|Event%20Button_03
  (if (stale _isa)
    (Audio|PlaySoundatLocation "/Game/HorrorKit/Assets/Audio/Interactive/Extractor_Hood/S_Button_Extractor_Hood_Cue.S_Button_Extractor_Hood_Cue" (Transformation|GetWorldLocation (Variables|Default|GetExtractor_Hood)) "0, 0, 0" 1.0 1.0 0.0 "/Game/HorrorKit/Assets/Audio/Interactive/Extractor_Hood/Info_Sound_Extractor_Hood.Info_Sound_Extractor_Hood")
    (bind _isa (Utilities|FlowControl|FlipFlop)
      (:A
        _)
      (:B
        _))
    (Components|MoveComponentTo (Variables|Default|GetButton_Speed_03) (Math|Vector|MakeVector (Math|Float|SelectFloat -0.8 0.0 _isa) 0.0 0.0) "0, 0, 0" false false 0.2 false)
    (Variables|Default|SetButton_03 false)))

(event EventInteractive
  (params (Component :type Primitive%20Component%20Object%20Reference))
  (if (== Component (Variables|Default|GetButton_Speed_01))
    (if (not (Variables|Default|GetButton_01))
      (Variables|Default|SetButton_01 true)
      (CallFunction|FDefault false true true)
      (Audio|PlaySoundatLocation "/Game/HorrorKit/Assets/Audio/Interactive/Extractor_Hood/S_Button_Extractor_Hood_Cue.S_Button_Extractor_Hood_Cue" (Transformation|GetWorldLocation (Variables|Default|GetExtractor_Hood)) "0, 0, 0" 1.0 1.0 0.0 "/Game/HorrorKit/Assets/Audio/Interactive/Extractor_Hood/Info_Sound_Extractor_Hood.Info_Sound_Extractor_Hood")
      (bind _isa (Utilities|FlowControl|FlipFlop)
        (:A
          _)
        (:B
          _))
      (Components|MoveComponentTo (Variables|Default|GetButton_Speed_01) (Math|Vector|MakeVector (Math|Float|SelectFloat -0.8 0.0 _isa) 0.0 0.0) "0, 0, 0" false false 0.2 false)
      (Variables|Default|SetButton_01 false))
    (elif (== Component (Variables|Default|GetButton_Speed_02))
      (if (not (Variables|Default|GetButton_02))
        (Variables|Default|SetButton_02 true)
        (CallFunction|FDefault true false true)
        (Audio|PlaySoundatLocation "/Game/HorrorKit/Assets/Audio/Interactive/Extractor_Hood/S_Button_Extractor_Hood_Cue.S_Button_Extractor_Hood_Cue" (Transformation|GetWorldLocation (Variables|Default|GetExtractor_Hood)) "0, 0, 0" 1.0 1.0 0.0 "/Game/HorrorKit/Assets/Audio/Interactive/Extractor_Hood/Info_Sound_Extractor_Hood.Info_Sound_Extractor_Hood")
        (bind _isa_2 (Utilities|FlowControl|FlipFlop)
          (:A
            _)
          (:B
            _))
        (Components|MoveComponentTo (Variables|Default|GetButton_Speed_02) (Math|Vector|MakeVector (Math|Float|SelectFloat -0.8 0.0 _isa_2) 0.0 0.0) "0, 0, 0" false false 0.2 false)
        (Variables|Default|SetButton_02 false))
      (elif (== Component (Variables|Default|GetButton_Speed_03))
        (if (not (Variables|Default|GetButton_03))
          (Variables|Default|SetButton_03 true)
          (CallFunction|FDefault true true false)
          (Audio|PlaySoundatLocation "/Game/HorrorKit/Assets/Audio/Interactive/Extractor_Hood/S_Button_Extractor_Hood_Cue.S_Button_Extractor_Hood_Cue" (Transformation|GetWorldLocation (Variables|Default|GetExtractor_Hood)) "0, 0, 0" 1.0 1.0 0.0 "/Game/HorrorKit/Assets/Audio/Interactive/Extractor_Hood/Info_Sound_Extractor_Hood.Info_Sound_Extractor_Hood")
          (bind _isa_3 (Utilities|FlowControl|FlipFlop)
            (:A
              _)
            (:B
              _))
          (Components|MoveComponentTo (Variables|Default|GetButton_Speed_03) (Math|Vector|MakeVector (Math|Float|SelectFloat -0.8 0.0 _isa_3) 0.0 0.0) "0, 0, 0" false false 0.2 false)
          (Variables|Default|SetButton_03 false))
        (elif (== Component (Variables|Default|GetButton_Light))
          (if (not (Variables|Default|GetButton_04))
            (Variables|Default|SetButton_04 true)
            (Audio|PlaySoundatLocation "/Game/HorrorKit/Assets/Audio/Interactive/Extractor_Hood/S_Button_Extractor_Hood_Cue.S_Button_Extractor_Hood_Cue" (Transformation|GetWorldLocation (Variables|Default|GetExtractor_Hood)) "0, 0, 0" 1.0 1.0 0.0 "/Game/HorrorKit/Assets/Audio/Interactive/Extractor_Hood/Info_Sound_Extractor_Hood.Info_Sound_Extractor_Hood")
            (bind _isa_4 (Utilities|FlowControl|FlipFlop)
              (:A
                _)
              (:B
                _))
            (Components|MoveComponentTo (Variables|Default|GetButton_Light) (Math|Vector|MakeVector (Math|Float|SelectFloat -0.8 0.0 _isa_4) 0.0 0.0) "0, 0, 0" false false 0.2 false)
            (Variables|Default|SetButton_04 false)
            (Rendering|SetVisibility (Variables|Default|GetSpotLight) _isa_4 false)
            (Rendering|Material|SetMaterial (Variables|Default|GetExtractor_Hood) 3 (select _isa_4 "/Game/HorrorKit/Assets/Models/Interactive/Kitchen/Extractor_Hood/M_Extractor_Hood_Light.M_Extractor_Hood_Light" "/Game/HorrorKit/Assets/Models/Interactive/Kitchen/Extractor_Hood/M_Extractor_Hood_Default.M_Extractor_Hood_Default"))))))))

(fn ConstructionScript)

(fn FDefault
  (params (Button%201 :type Boolean) (Button%202 :type Boolean) (Button%203 :type Boolean))
  (Utilities|FlowControl|Sequence
    (:then_0
      (if Button%201
        (CallFunction|EventButton01)))
    (:then_1
      (if Button%202
        (CallFunction|EventButton02)))
    (:then_2
      (if Button%203
        (CallFunction|EventButton03)))))