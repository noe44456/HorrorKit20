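; Interactive microwave oven prop with an openable door and a timer knob that starts or stops a cooking cycle.
; The Interactive event routes by component: the door flip-flops a timeline, while the knob rotates to the configured duration or back to zero.
; Looping timers turn the platter and tick the knob back alongside the light and hum, pausing timers and sound while the door is open.
; F_Timer ends the cycle, resetting everything with an end sound.
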(event Custom|Event%20Rotate
  (Transformation|AddRelativeRotation (Variables|Default|GetButton_01) "0.000000, 0,1.000000" false false))

(event Custom|Event%20Rotate%20platter
  (Transformation|AddRelativeRotation (Variables|Default|GetPlatter) "0.000000,0.500000,0.000000" false false))

(event EventInteractive
  (params (Component :type Primitive%20Component%20Object%20Reference))
  (bind _microwave_oven (Variables|Default|GetMicrowave_Oven))
  (bind _returnvalue (Transformation|GetWorldLocation _microwave_oven))
  (if (== Component (Variables|Default|GetDoor))
    (if (not (Audio|Components|Audio|IsPlaying (Variables|Default|GetAnimation%20Door)))
      (bind _isa (Utilities|FlowControl|FlipFlop)
        (:A
          (Audio|PlaySoundatLocation "/Game/HorrorKit/Assets/Audio/Interactive/Microwave_Oven/S_Microwave_Oven_Open_Cue.S_Microwave_Oven_Open_Cue" _returnvalue "0, 0, 0" 1.0 1.0 0.0 "/Game/HorrorKit/Assets/Audio/Interactive/Microwave_Oven/Info_Sound_Microwave_Oven.Info_Sound_Microwave_Oven")
          (bind _door (Timeline|Animation%20Door Play)
            (:Update
              (Transformation|SetRelativeRotation (Variables|Default|GetScene_Door) (Math|Rotator|MakeRotator 0.0 0.0 _door) false false))
            (:Finished
              (Utilities|FlowControl|Sequence
                (:then_0
                  (if (!= (.roll (Variables|/Script/Engine.SceneComponent|GetRelativeRotation (Variables|Default|GetButton_01))) 0.0)
                    (if _isa
                      (Class|KismetSystemLibrary|PauseTimer 0 "F_Timer")
                      (Utilities|Time|PauseTimerbyHandle (Variables|Default|GetTimer%20Rotate%20Button))
                      (Utilities|Time|PauseTimerbyHandle (Variables|Default|GetTimer%20Rotate%20Flatter))
                      (Audio|Components|Audio|Stop (Variables|Default|GetSound))
                      (else
                        (Class|KismetSystemLibrary|UnPauseTimer 0 "F_Timer")
                        (Utilities|Time|UnpauseTimerbyHandle (Variables|Default|GetTimer%20Rotate%20Button))
                        (Utilities|Time|UnpauseTimerbyHandle (Variables|Default|GetTimer%20Rotate%20Flatter))
                        (Audio|Components|Audio|Play (Variables|Default|GetSound) 0.0)))))
                (:then_1
                  (if (Variables|Default|GetPause)
                    (Audio|Components|Audio|Play (Variables|Default|GetSound) 0.0)
                    (Variables|Default|SetPause false)))))))
        (:B
          (Utilities|FlowControl|Sequence
            (:then_0
              (Timeline|Animation%20Door Reverse))
            (:then_1
              (Utilities|FlowControl|Delay 0.4)
              (Audio|PlaySoundatLocation "/Game/HorrorKit/Assets/Audio/Interactive/Microwave_Oven/S_Microwave_Oven_Close_Cue.S_Microwave_Oven_Close_Cue" _returnvalue "0, 0, 0" 1.0 1.0 0.0 "/Game/HorrorKit/Assets/Audio/Interactive/Microwave_Oven/Info_Sound_Microwave_Oven.Info_Sound_Microwave_Oven"))))))
    (elif (== Component (Variables|Default|GetButton_01))
      (if (not (Variables|Default|GetPlay))
        (Variables|Default|SetPlay true)
        (Audio|PlaySoundatLocation "/Game/HorrorKit/Assets/Audio/Interactive/Microwave_Oven/S_Microwave_Oven_Button_Cue.S_Microwave_Oven_Button_Cue" (Transformation|GetWorldLocation (Variables|Default|GetButton_01)) "0, 0, 0" 1.0 1.0 0.0 "/Game/HorrorKit/Assets/Audio/Interactive/Microwave_Oven/Info_Sound_Microwave_Oven.Info_Sound_Microwave_Oven")
        (Components|MoveComponentTo (Variables|Default|GetButton_01) (Variables|/Script/Engine.SceneComponent|GetRelativeLocation (Variables|Default|GetButton_01)) (Math|Rotator|MakeRotator (Math|Float|SelectFloat (* (Variables|Default|GetTimer) -1.0) 0.0 (== (.roll (Variables|/Script/Engine.SceneComponent|GetRelativeRotation (Variables|Default|GetButton_01))) 0.0)) 0.0 0.0) false false (/ (Variables|Default|GetTimer) 6e+01) false)
        (Variables|Default|SetPlay false)
        (if (!= (.roll (Variables|/Script/Engine.SceneComponent|GetRelativeRotation (Variables|Default|GetButton_01))) 0.0)
          (Utilities|Time|SetTimerbyFunctionName 0 "F_Timer" (Variables|Default|GetTimer) true)
          (bind _returnvalue_2 (Utilities|Time|SetTimerbyEvent (delegate Custom|Event%20Rotate%20platter) 0.05 true))
          (Variables|Default|SetTimer%20Rotate%20Flatter _returnvalue_2)
          (Rendering|SetVisibility (Variables|Default|GetPointLight) true false)
          (bind _returnvalue_3 (Utilities|Time|SetTimerbyEvent (delegate Custom|Event%20Rotate) 1.0 true))
          (Variables|Default|SetTimer%20Rotate%20Button _returnvalue_3)
          (Audio|Components|Audio|Play (Variables|Default|GetSound) 0.0)
          (Utilities|FlowControl|Sequence
            (:then_0
              (if _isa
                (Class|KismetSystemLibrary|PauseTimer 0 "F_Timer")
                (Utilities|Time|PauseTimerbyHandle (Variables|Default|GetTimer%20Rotate%20Button))
                (Utilities|Time|PauseTimerbyHandle (Variables|Default|GetTimer%20Rotate%20Flatter))))
            (:then_1
              (if _isa
                (Audio|Components|Audio|Stop (Variables|Default|GetSound))
                (Variables|Default|SetPause true))))
          (else
            (Utilities|Time|ClearTimerbyFunctionName 0 "F_Timer")
            (CallFunction|FTimer)))))))

(fn ConstructionScript
  (Variables|Default|SetTimer (Math|Float|Clamp(Float) (Variables|Default|GetTimer) 0.0 2e+02)))

(fn FTimer
  (Utilities|Time|ClearandInvalidateTimerbyHandle (Variables|Default|GetTimer%20Rotate%20Button))
  (Utilities|Time|ClearandInvalidateTimerbyHandle (Variables|Default|GetTimer%20Rotate%20Flatter))
  (Rendering|SetVisibility (Variables|Default|GetPointLight) false false)
  (Utilities|Time|ClearTimerbyFunctionName 0 "F_Timer")
  (Transformation|SetRelativeRotation (Variables|Default|GetButton_01) "0, 0, 0" false false)
  (Audio|Components|Audio|Stop (Variables|Default|GetSound))
  (Audio|PlaySoundatLocation "/Game/HorrorKit/Assets/Audio/Interactive/Microwave_Oven/S_Microwave_Oven_End_Cue.S_Microwave_Oven_End_Cue" (Transformation|GetWorldLocation (Variables|Default|GetMicrowave_Oven)) "0, 0, 0" 1.0 1.0 0.0 "/Game/HorrorKit/Assets/Audio/Interactive/Microwave_Oven/Info_Sound_Microwave_Oven.Info_Sound_Microwave_Oven"))

(event EventBeginPlay
  (bind _returnvalue (Audio|SpawnSoundatLocation "/Game/HorrorKit/Assets/Audio/Interactive/Microwave_Oven/S_Microwave_Oven_Loop.S_Microwave_Oven_Loop" (Transformation|GetWorldLocation (Variables|Default|GetMicrowave_Oven)) "0, 0, 0" 1.0 1.0 0.0 "/Game/HorrorKit/Assets/Audio/Interactive/Microwave_Oven/Info_Sound_Microwave_Oven.Info_Sound_Microwave_Oven" 0 false))
  (bind _output_get (Variables|Default|SetSound _returnvalue))
  (Audio|Components|Audio|Stop _output_get))