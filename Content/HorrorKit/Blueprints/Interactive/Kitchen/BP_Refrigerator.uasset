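; Interactive kitchen refrigerator whose freezer and fridge doors open and close independently with sound.
; The Interactive event matches the used component to a door, ignores it while that door animates, and uses a FlipFlop to play or reverse a timeline driving the pivot's yaw.
; The open sound plays immediately, while the close sound follows a short delay.
; The construction script optionally swaps the body to an alternate mesh via SwitchMesh.
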(event EventInteractive
  (params (Component :type Primitive%20Component%20Object%20Reference))
  (bind _door_freezer (Variables|Default|GetDoor_Freezer))
  (bind _door_refrigerator (Variables|Default|GetDoor_Refrigerator))
  (bind _returnvalue (Transformation|GetWorldLocation _door_refrigerator))
  (bind _returnvalue_2 (Transformation|GetWorldLocation _door_freezer))
  (if (== Component (Variables|Default|GetDoor_Freezer))
    (if (not (Audio|Components|Audio|IsPlaying (Variables|Default|GetAnimation_Door_Freezer)))
      (Utilities|FlowControl|FlipFlop
        (:A
          (Audio|PlaySoundatLocation "/Game/HorrorKit/Assets/Audio/Interactive/Refrigerator/S_Open_Refrigerator_Cue.S_Open_Refrigerator_Cue" _returnvalue_2 "0, 0, 0" 1.0 1.0 0.0 "/Game/HorrorKit/Assets/Audio/Interactive/Refrigerator/Info_Sound_Refrigerator.Info_Sound_Refrigerator")
          (bind _open_close (Timeline|Animation_Door_Freezer Play)
            (:Update
              (Transformation|SetRelativeRotation (Variables|Default|GetScene_Door_Freezer) (Math|Rotator|MakeRotator 0.0 0.0 _open_close) false false))))
        (:B
          (Utilities|FlowControl|Sequence
            (:then_0
              (Timeline|Animation_Door_Freezer Reverse))
            (:then_1
              (Utilities|FlowControl|Delay 0.5)
              (Audio|PlaySoundatLocation "/Game/HorrorKit/Assets/Audio/Interactive/Refrigerator/S_Close_Refrigerator_Cue.S_Close_Refrigerator_Cue" _returnvalue_2 "0, 0, 0" 1.0 1.0 0.0 "/Game/HorrorKit/Assets/Audio/Interactive/Refrigerator/Info_Sound_Refrigerator.Info_Sound_Refrigerator"))))))
    (elif (== Component (Variables|Default|GetDoor_Refrigerator))
      (if (not (Audio|Components|Audio|IsPlaying (Variables|Default|GetAnimation_Door_Refrigerator)))
        (Utilities|FlowControl|FlipFlop
          (:A
            (Audio|PlaySoundatLocation "/Game/HorrorKit/Assets/Audio/Interactive/Refrigerator/S_Open_Refrigerator_Cue.S_Open_Refrigerator_Cue" _returnvalue "0, 0, 0" 1.0 1.0 0.0 "/Game/HorrorKit/Assets/Audio/Interactive/Refrigerator/Info_Sound_Refrigerator.Info_Sound_Refrigerator")
            (bind _open_close_2 (Timeline|Animation_Door_Refrigerator Play)
              (:Update
                (Transformation|SetRelativeRotation (Variables|Default|GetScene_Door_Refrigerator) (Math|Rotator|MakeRotator 0.0 0.0 _open_close_2) false false))))
          (:B
            (Utilities|FlowControl|Sequence
              (:then_0
                (Timeline|Animation_Door_Refrigerator Reverse))
              (:then_1
                (Utilities|FlowControl|Delay 0.5)
                (Audio|PlaySoundatLocation "/Game/HorrorKit/Assets/Audio/Interactive/Refrigerator/S_Close_Refrigerator_Cue.S_Close_Refrigerator_Cue" _returnvalue "0, 0, 0" 1.0 1.0 0.0 "/Game/HorrorKit/Assets/Audio/Interactive/Refrigerator/Info_Sound_Refrigerator.Info_Sound_Refrigerator")))))))))

(fn ConstructionScript
  (if (Variables|Default|GetSwitch%20Mesh?)
    (Components|StaticMesh|SetStaticMesh (Variables|Default|GetRefrigerator) "/Game/HorrorKit/Assets/Models/Interactive/Kitchen/Refrigerator/SM_Refrigerator_02.SM_Refrigerator_02")))