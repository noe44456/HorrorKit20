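; Interactive kitchen table prop with four drawers (Box01–Box04) that the player can open and close individually.
; The Interactive event matches the passed component to a drawer and ignores it while that drawer's animation is still playing.
; A per-drawer FlipFlop alternates playing and reversing a timeline that slides the drawer along its local X, with open and close sounds at the table.
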(event EventInteractive
  (params (Component :type Primitive%20Component%20Object%20Reference))
  (bind _table (Variables|Default|GetTable))
  (bind _table_2 (Variables|Default|GetTable))
  (bind _table_3 (Variables|Default|GetTable))
  (bind _table_4 (Variables|Default|GetTable))
  (bind _returnvalue (Transformation|GetWorldLocation _table_4))
  (bind _returnvalue_2 (Transformation|GetWorldLocation _table))
  (bind _returnvalue_3 (Transformation|GetWorldLocation _table_2))
  (bind _returnvalue_4 (Transformation|GetWorldLocation _table_3))
  (if (== Component (Variables|Default|GetBox_01))
    (if (not (Audio|Components|Audio|IsPlaying (Variables|Default|GetAnimation_Box_01)))
      (Utilities|FlowControl|FlipFlop
        (:A
          (Audio|PlaySoundatLocation "/Game/HorrorKit/Assets/Audio/Interactive/Box_Table/Open_Box_Cue.Open_Box_Cue" _returnvalue_2 "0, 0, 0" 1.0 1.0 0.0 "/Game/HorrorKit/Assets/Audio/Interactive/Wardrobe/Info_Sound_Box_WardRobe_Table.Info_Sound_Box_WardRobe_Table")
          (bind _box (Timeline|Animation_Box_01 Play)
            (:Update
              (Transformation|SetRelativeLocation (Variables|Default|GetBox_01) (Math|Vector|MakeVector _box 0.0 0.0) false false))))
        (:B
          (Audio|PlaySoundatLocation "/Game/HorrorKit/Assets/Audio/Interactive/Box_Table/Close_Box_Cue.Close_Box_Cue" _returnvalue_2 "0, 0, 0" 1.0 1.0 0.0 "/Game/HorrorKit/Assets/Audio/Interactive/Wardrobe/Info_Sound_Box_WardRobe_Table.Info_Sound_Box_WardRobe_Table")
          (Timeline|Animation_Box_01 Reverse))))
    (elif (== Component (Variables|Default|GetBox_02))
      (if (not (Audio|Components|Audio|IsPlaying (Variables|Default|GetAnimation_Box_02)))
        (Utilities|FlowControl|FlipFlop
          (:A
            (Audio|PlaySoundatLocation "/Game/HorrorKit/Assets/Audio/Interactive/Box_Table/Open_Box_Cue.Open_Box_Cue" _returnvalue_3 "0, 0, 0" 1.0 1.0 0.0 "/Game/HorrorKit/Assets/Audio/Interactive/Wardrobe/Info_Sound_Box_WardRobe_Table.Info_Sound_Box_WardRobe_Table")
            (bind _box_2 (Timeline|Animation_Box_02 Play)
              (:Update
                (Transformation|SetRelativeLocation (Variables|Default|GetBox_02) (Math|Vector|MakeVector _box_2 0.0 0.0) false false))))
          (:B
            (Audio|PlaySoundatLocation "/Game/HorrorKit/Assets/Audio/Interactive/Box_Table/Close_Box_Cue.Close_Box_Cue" _returnvalue_3 "0, 0, 0" 1.0 1.0 0.0 "/Game/HorrorKit/Assets/Audio/Interactive/Wardrobe/Info_Sound_Box_WardRobe_Table.Info_Sound_Box_WardRobe_Table")
            (Timeline|Animation_Box_02 Reverse))))
      (elif (== Component (Variables|Default|GetBox_03))
        (if (not (Audio|Components|Audio|IsPlaying (Variables|Default|GetAnimation_Box_03)))
          (Utilities|FlowControl|FlipFlop
            (:A
              (Audio|PlaySoundatLocation "/Game/HorrorKit/Assets/Audio/Interactive/Box_Table/Open_Box_Cue.Open_Box_Cue" _returnvalue_4 "0, 0, 0" 1.0 1.0 0.0 "/Game/HorrorKit/Assets/Audio/Interactive/Wardrobe/Info_Sound_Box_WardRobe_Table.Info_Sound_Box_WardRobe_Table")
              (bind _box_3 (Timeline|Animation_Box_03 Play)
                (:Update
                  (Transformation|SetRelativeLocation (Variables|Default|GetBox_03) (Math|Vector|MakeVector _box_3 0.0 0.0) false false))))
            (:B
              (Audio|PlaySoundatLocation "/Game/HorrorKit/Assets/Audio/Interactive/Box_Table/Close_Box_Cue.Close_Box_Cue" _returnvalue_4 "0, 0, 0" 1.0 1.0 0.0 "/Game/HorrorKit/Assets/Audio/Interactive/Wardrobe/Info_Sound_Box_WardRobe_Table.Info_Sound_Box_WardRobe_Table")
              (Timeline|Animation_Box_03 Reverse))))
        (elif (== Component (Variables|Default|GetBox_04))
          (if (not (Audio|Components|Audio|IsPlaying (Variables|Default|GetAnimation_Box_04)))
            (Utilities|FlowControl|FlipFlop
              (:A
                (Audio|PlaySoundatLocation "/Game/HorrorKit/Assets/Audio/Interactive/Box_Table/Open_Box_Cue.Open_Box_Cue" _returnvalue "0, 0, 0" 1.0 1.0 0.0 "/Game/HorrorKit/Assets/Audio/Interactive/Wardrobe/Info_Sound_Box_WardRobe_Table.Info_Sound_Box_WardRobe_Table")
                (bind _box_4 (Timeline|Animation_Box_04 Play)
                  (:Update
                    (Transformation|SetRelativeLocation (Variables|Default|GetBox_04) (Math|Vector|MakeVector _box_4 0.0 0.0) false false))))
              (:B
                (Audio|PlaySoundatLocation "/Game/HorrorKit/Assets/Audio/Interactive/Box_Table/Close_Box_Cue.Close_Box_Cue" _returnvalue "0, 0, 0" 1.0 1.0 0.0 "/Game/HorrorKit/Assets/Audio/Interactive/Wardrobe/Info_Sound_Box_WardRobe_Table.Info_Sound_Box_WardRobe_Table")
                (Timeline|Animation_Box_04 Reverse)))))))))

(fn ConstructionScript)