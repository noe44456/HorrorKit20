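; BP_Bread_Bin is an interactive kitchen bread bin with a door that opens and closes.
; The Interactive event responds only to the DoorBreadBin component and ignores input while the AnimationDoor timeline is playing.
; A FlipFlop alternates between playing and reversing the timeline, which drives the door's relative pitch, with a matching open or close sound at the bin's location.
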(event EventInteractive
  (params (Component :type Primitive%20Component%20Object%20Reference))
  (bind _bread_bin (Variables|Default|GetBread%20Bin))
  (bind _returnvalue (Transformation|GetWorldLocation _bread_bin))
  (if (== Component (Variables|Default|GetDoor_Bread_Bin))
    (if (not (Audio|Components|Audio|IsPlaying (Variables|Default|GetAnimation%20Door)))
      (Utilities|FlowControl|FlipFlop
        (:A
          (Audio|PlaySoundatLocation "/Game/HorrorKit/Assets/Audio/Interactive/Bread_Bin/S_Bread_Bin_Open_Cue.S_Bread_Bin_Open_Cue" _returnvalue "0, 0, 0" 1.0 1.0 0.0 "/Game/HorrorKit/Assets/Audio/Interactive/Bread_Bin/Info_Sound_Bread_Bin.Info_Sound_Bread_Bin")
          (bind _door (Timeline|Animation%20Door Play)
            (:Update
              (Transformation|SetRelativeRotation (Variables|Default|GetDoor_Bread_Bin) (Math|Rotator|MakeRotator 0.0 _door 0.0) false false))))
        (:B
          (Audio|PlaySoundatLocation "/Game/HorrorKit/Assets/Audio/Interactive/Bread_Bin/S_Bread_Bin_Close_Cue.S_Bread_Bin_Close_Cue" _returnvalue "0, 0, 0" 1.0 1.0 0.0 "/Game/HorrorKit/Assets/Audio/Interactive/Bread_Bin/Info_Sound_Bread_Bin.Info_Sound_Bread_Bin")
          (Timeline|Animation%20Door Reverse))))))

(fn ConstructionScript)