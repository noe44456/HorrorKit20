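; Interactive kitchen sink with two cabinet doors and a working faucet.
; Interacting with a door toggles its Timeline swing with sound, while the faucet pauses the game and opens a blurred-background HUD widget linked to this sink.
; Hot, Cold and Off events share one path that rotates the handle and switches water particles and audio, with a Use flag briefly blocking interaction.
; Hot water starts steam after a timer, cancelled by Cold or Off.
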(event Custom|Event%20Open%20Widget
  (bind _character (Variables|Default|GetCharacter))
  (bind _character_2 (Variables|Default|GetCharacter))
  (bind _character_3 (Variables|Default|GetCharacter))
  (bind _hud (Variables|/Game/HorrorKit/Blueprints/Player/MyCharacter.MyCharacter_C|GetHud _character))
  (bind _hud_2 (Variables|/Game/HorrorKit/Blueprints/Player/MyCharacter.MyCharacter_C|GetHud _character_2))
  (bind _playercontroller (Variables|/Game/HorrorKit/Blueprints/Player/MyCharacter.MyCharacter_C|GetPlayerController _character_3))
  (bind _sink_kitchen_widget (Variables|/Game/HorrorKit/Blueprints/Player/Hud.Hud_C|GetSink_Kitchen_Widget _hud))
  (Game|SetGamePaused true)
  (Variables|/Game/HorrorKit/Blueprints/Interactive/Kitchen/Sink/Sink_Kitchen_Widget.Sink_Kitchen_Widget_C|SetSink_Kitchen _sink_kitchen_widget self)
  (Widget|SetVisibility _sink_kitchen_widget "Visible")
  (Default|FBlur _hud_2)
  (Default|FOpenWidget _playercontroller _hud_2)
  (Default|FSetCursorCenter _playercontroller))

(event Custom|Event%20Off
  (bind _crane (Variables|Default|GetCrane))
  (bind _relativerotation (Variables|/Script/Engine.SceneComponent|GetRelativeRotation _crane))
  (Utilities|Time|ClearandInvalidateTimerbyHandle (Variables|Default|GetTimerSmoke))
  (Variables|Default|SetOff true)
  (Audio|PlaySoundatLocation (select (Variables|Default|GetOff) "/Game/HorrorKit/Assets/Audio/Interactive/Sink/S_Close_Valve_Cue.S_Close_Valve_Cue" "/Game/HorrorKit/Assets/Audio/Interactive/Sink/S_Open_Valve_Cue.S_Open_Valve_Cue") (Transformation|GetWorldLocation (Variables|Default|GetCrane)) "0, 0, 0" 1.0 1.0 0.0 "/Game/HorrorKit/Assets/Audio/Interactive/Sink/Info_Sound_Sink.Info_Sound_Sink")
  (Variables|Default|SetUse true)
  (Components|MoveComponentTo (Variables|Default|GetCrane) (Variables|/Script/Engine.SceneComponent|GetRelativeLocation (Variables|Default|GetCrane)) (Math|Rotator|MakeRotator 0.0 (Math|Float|SelectFloat 0.0 12.0 (Variables|Default|GetOff)) (Math|Float|SelectFloat 0.0 (Math|Float|SelectFloat 35.0 -35.0 (Variables|Default|GetCold)) (Variables|Default|GetOff))) false false (Math|Float|SelectFloat 0.8 0.4 (or (> (.yaw _relativerotation) 0.0) (< (.yaw _relativerotation) 0.0))) false)
  (if (and (== (Variables|/Script/Engine.AudioComponent|GetSound (Variables|Default|GetAudio)) "/Game/HorrorKit/Assets/Audio/Interactive/Sink/S_Sink_Water_Loop.S_Sink_Water_Loop") (not (Variables|Default|GetOff)))
    (Utilities|FlowControl|Delay 0.1)
    (Variables|Default|SetUse false)
    (else
      (Audio|Components|Audio|SetSound (Variables|Default|GetAudio) (select (Variables|Default|GetOff) "/Game/HorrorKit/Assets/Audio/Interactive/Sink/S_Sink_Water_End_Cue.S_Sink_Water_End_Cue" "/Game/HorrorKit/Assets/Audio/Interactive/Sink/S_Sink_Water_Loop_Cue.S_Sink_Water_Loop_Cue"))
      (Audio|Components|Audio|Play (Variables|Default|GetAudio) 0.0)
      (Utilities|FlowControl|Delay 0.1)
      (if (Variables|Default|GetOff)
        (Components|Activation|SetActive (Variables|Default|GetWater_01) false false)
        (else
          (Components|Activation|SetActive (Variables|Default|GetWater_01) true false)))
      (Variables|Default|SetUse false))))

(event Custom|Event%20Hot
  (bind _crane (Variables|Default|GetCrane))
  (bind _relativerotation (Variables|/Script/Engine.SceneComponent|GetRelativeRotation _crane))
  (Utilities|FlowControl|Sequence
    (:then_0
      (Variables|Default|SetUse true)
      (Variables|Default|SetCold false)
      (Variables|Default|SetOff false)
      (Audio|PlaySoundatLocation (select (Variables|Default|GetOff) "/Game/HorrorKit/Assets/Audio/Interactive/Sink/S_Close_Valve_Cue.S_Close_Valve_Cue" "/Game/HorrorKit/Assets/Audio/Interactive/Sink/S_Open_Valve_Cue.S_Open_Valve_Cue") (Transformation|GetWorldLocation (Variables|Default|GetCrane)) "0, 0, 0" 1.0 1.0 0.0 "/Game/HorrorKit/Assets/Audio/Interactive/Sink/Info_Sound_Sink.Info_Sound_Sink")
      (Variables|Default|SetUse true)
      (Components|MoveComponentTo (Variables|Default|GetCrane) (Variables|/Script/Engine.SceneComponent|GetRelativeLocation (Variables|Default|GetCrane)) (Math|Rotator|MakeRotator 0.0 (Math|Float|SelectFloat 0.0 12.0 (Variables|Default|GetOff)) (Math|Float|SelectFloat 0.0 (Math|Float|SelectFloat 35.0 -35.0 (Variables|Default|GetCold)) (Variables|Default|GetOff))) false false (Math|Float|SelectFloat 0.8 0.4 (or (> (.yaw _relativerotation) 0.0) (< (.yaw _relativerotation) 0.0))) false)
      (if (and (== (Variables|/Script/Engine.AudioComponent|GetSound (Variables|Default|GetAudio)) "/Game/HorrorKit/Assets/Audio/Interactive/Sink/S_Sink_Water_Loop.S_Sink_Water_Loop") (not (Variables|Default|GetOff)))
        (Utilities|FlowControl|Delay 0.1)
        (Variables|Default|SetUse false)
        (else
          (Audio|Components|Audio|SetSound (Variables|Default|GetAudio) (select (Variables|Default|GetOff) "/Game/HorrorKit/Assets/Audio/Interactive/Sink/S_Sink_Water_End_Cue.S_Sink_Water_End_Cue" "/Game/HorrorKit/Assets/Audio/Interactive/Sink/S_Sink_Water_Loop_Cue.S_Sink_Water_Loop_Cue"))
          (Audio|Components|Audio|Play (Variables|Default|GetAudio) 0.0)
          (Utilities|FlowControl|Delay 0.1)
          (if (Variables|Default|GetOff)
            (Components|Activation|SetActive (Variables|Default|GetWater_01) false false)
            (else
              (Components|Activation|SetActive (Variables|Default|GetWater_01) true false)))
          (Variables|Default|SetUse false))))
    (:then_1
      (bind _returnvalue (Utilities|Time|SetTimerbyEvent (delegate Custom|Event%20Smoke) 3.0))
      (Variables|Default|SetTimerSmoke _returnvalue))))

(event Custom|Event%20Cold
  (bind _crane (Variables|Default|GetCrane))
  (bind _relativerotation (Variables|/Script/Engine.SceneComponent|GetRelativeRotation _crane))
  (Utilities|Time|ClearandInvalidateTimerbyHandle (Variables|Default|GetTimerSmoke))
  (Components|Activation|SetActive (Variables|Default|GetSmoke_01) false false)
  (Variables|Default|SetCold true)
  (Variables|Default|SetOff false)
  (Audio|PlaySoundatLocation (select (Variables|Default|GetOff) "/Game/HorrorKit/Assets/Audio/Interactive/Sink/S_Close_Valve_Cue.S_Close_Valve_Cue" "/Game/HorrorKit/Assets/Audio/Interactive/Sink/S_Open_Valve_Cue.S_Open_Valve_Cue") (Transformation|GetWorldLocation (Variables|Default|GetCrane)) "0, 0, 0" 1.0 1.0 0.0 "/Game/HorrorKit/Assets/Audio/Interactive/Sink/Info_Sound_Sink.Info_Sound_Sink")
  (Variables|Default|SetUse true)
  (Components|MoveComponentTo (Variables|Default|GetCrane) (Variables|/Script/Engine.SceneComponent|GetRelativeLocation (Variables|Default|GetCrane)) (Math|Rotator|MakeRotator 0.0 (Math|Float|SelectFloat 0.0 12.0 (Variables|Default|GetOff)) (Math|Float|SelectFloat 0.0 (Math|Float|SelectFloat 35.0 -35.0 (Variables|Default|GetCold)) (Variables|Default|GetOff))) false false (Math|Float|SelectFloat 0.8 0.4 (or (> (.yaw _relativerotation) 0.0) (< (.yaw _relativerotation) 0.0))) false)
  (if (and (== (Variables|/Script/Engine.AudioComponent|GetSound (Variables|Default|GetAudio)) "/Game/HorrorKit/Assets/Audio/Interactive/Sink/S_Sink_Water_Loop.S_Sink_Water_Loop") (not (Variables|Default|GetOff)))
    (Utilities|FlowControl|Delay 0.1)
    (Variables|Default|SetUse false)
    (else
      (Audio|Components|Audio|SetSound (Variables|Default|GetAudio) (select (Variables|Default|GetOff) "/Game/HorrorKit/Assets/Audio/Interactive/Sink/S_Sink_Water_End_Cue.S_Sink_Water_End_Cue" "/Game/HorrorKit/Assets/Audio/Interactive/Sink/S_Sink_Water_Loop_Cue.S_Sink_Water_Loop_Cue"))
      (Audio|Components|Audio|Play (Variables|Default|GetAudio) 0.0)
      (Utilities|FlowControl|Delay 0.1)
      (if (Variables|Default|GetOff)
        (Components|Activation|SetActive (Variables|Default|GetWater_01) false false)
        (else
          (Components|Activation|SetActive (Variables|Default|GetWater_01) true false)))
      (Variables|Default|SetUse false))))

(event Custom|Event%20Close%20Widget
  (bind _character (Variables|Default|GetCharacter))
  (bind _character_2 (Variables|Default|GetCharacter))
  (bind _hud (Variables|/Game/HorrorKit/Blueprints/Player/MyCharacter.MyCharacter_C|GetHud _character))
  (bind _playercontroller (Variables|/Game/HorrorKit/Blueprints/Player/MyCharacter.MyCharacter_C|GetPlayerController _character_2))
  (Game|SetGamePaused false)
  (Widget|SetVisibility (Variables|/Game/HorrorKit/Blueprints/Player/Hud.Hud_C|GetSink_Kitchen_Widget (Variables|/Game/HorrorKit/Blueprints/Player/MyCharacter.MyCharacter_C|GetHud (Variables|Default|GetCharacter))) "Hidden")
  (Default|FResetBlur _hud)
  (Default|FSetDefaultButtons _playercontroller)
  (Utilities|FlowControl|Delay 0.035)
  (Default|FCloseWidget _playercontroller)
  (Default|FFlipFlopVisCrosshair _hud true))

(event Custom|Event%20Smoke
  (if (and (not (Variables|Default|GetCold)) (not (Variables|Default|GetOff)))
    (Components|Activation|SetActive (Variables|Default|GetSmoke_01) true false)))

(event EventInteractive
  (params (Component :type Primitive%20Component%20Object%20Reference))
  (bind _table (Variables|Default|GetTable))
  (bind _table_2 (Variables|Default|GetTable))
  (bind _returnvalue (Transformation|GetWorldLocation _table))
  (bind _returnvalue_2 (Transformation|GetWorldLocation _table_2))
  (if (not (Variables|Default|GetUse))
    (if (== Component (Variables|Default|GetDoor_Right))
      (if (not (Audio|Components|Audio|IsPlaying (Variables|Default|GetAnimation%20Door_Right)))
        (Utilities|FlowControl|FlipFlop
          (:A
            (Audio|PlaySoundatLocation "/Game/HorrorKit/Assets/Audio/Interactive/Wardrobe/S_Open_Wardrobe_Cue.S_Open_Wardrobe_Cue" _returnvalue_2 "0, 0, 0" 1.0 1.0 0.0 "/Game/HorrorKit/Assets/Audio/Interactive/Wardrobe/Info_Sound_Box_WardRobe_Table.Info_Sound_Box_WardRobe_Table")
            (bind _door (Timeline|Animation%20Door_Right Play)
              (:Update
                (Transformation|SetRelativeRotation (Variables|Default|GetScene_Door_Right) (Math|Rotator|MakeRotator 0.0 0.0 _door) false false))))
          (:B
            (Audio|PlaySoundatLocation "/Game/HorrorKit/Assets/Audio/Interactive/Wardrobe/S_Close_Wardrobe_Cue.S_Close_Wardrobe_Cue" _returnvalue_2 "0, 0, 0" 1.0 1.0 0.0 "/Game/HorrorKit/Assets/Audio/Interactive/Wardrobe/Info_Sound_Box_WardRobe_Table.Info_Sound_Box_WardRobe_Table")
            (Timeline|Animation%20Door_Right Reverse))))
      (elif (== Component (Variables|Default|GetDoor_Left))
        (if (not (Audio|Components|Audio|IsPlaying (Variables|Default|GetAnimation%20Door_Left)))
          (Utilities|FlowControl|FlipFlop
            (:A
              (Audio|PlaySoundatLocation "/Game/HorrorKit/Assets/Audio/Interactive/Wardrobe/S_Open_Wardrobe_Cue.S_Open_Wardrobe_Cue" _returnvalue "0, 0, 0" 1.0 1.0 0.0 "/Game/HorrorKit/Assets/Audio/Interactive/Wardrobe/Info_Sound_Box_WardRobe_Table.Info_Sound_Box_WardRobe_Table")
              (bind _door_2 (Timeline|Animation%20Door_Left Play)
                (:Update
                  (Transformation|SetRelativeRotation (Variables|Default|GetScene_Door_Left) (Math|Rotator|MakeRotator 0.0 0.0 _door_2) false false))))
            (:B
              (Audio|PlaySoundatLocation "/Game/HorrorKit/Assets/Audio/Interactive/Wardrobe/S_Close_Wardrobe_Cue.S_Close_Wardrobe_Cue" _returnvalue "0, 0, 0" 1.0 1.0 0.0 "/Game/HorrorKit/Assets/Audio/Interactive/Wardrobe/Info_Sound_Box_WardRobe_Table.Info_Sound_Box_WardRobe_Table")
              (Timeline|Animation%20Door_Left Reverse))))
        (elif (== Component (Variables|Default|GetCrane))
          (CallFunction|EventOpenWidget))))))

(fn ConstructionScript)

(event EventBeginPlay
  (bind _asmy_character (Utilities|Casting|CastToMyCharacter (Game|GetPlayerCharacter 0)))
  (Variables|Default|SetCharacter _asmy_character)
  (bind _returnvalue (Audio|SpawnSoundatLocation "/Game/HorrorKit/Assets/Audio/Interactive/Sink/S_Sink_Water_End.S_Sink_Water_End" (Transformation|GetWorldLocation (Variables|Default|GetCrane)) "0, 0, 0" 1.0 1.0 0.0 "/Game/HorrorKit/Assets/Audio/Interactive/Sink/Info_Sound_Sink.Info_Sound_Sink" 0 false))
  (bind _output_get (Variables|Default|SetAudio _returnvalue))
  (Audio|Components|Audio|Stop _output_get))