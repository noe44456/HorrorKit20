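; Interactive kitchen table prop with a door and a sliding box drawer that the player can open and close.
; The Interactive event branches on the passed component and ignores it while that part's animation is playing.
; A FlipFlop per part alternates playing and reversing its timeline, with an open or close sound at the table.
; The timelines drive SceneDoor's relative yaw and the Box's relative X position.
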(event EventInteractive
  (params (Component :type Primitive%20Component%20Object%20Reference))
  (bind _table (Variables|Default|GetTable))
  (bind _table_2 (Variables|Default|GetTable))
  (bind _returnvalue (Transformation|GetWorldLocation _table))
  (bind _returnvalue_2 (Transformation|GetWorldLocation _table_2))
  (if (== Component (Variables|Default|GetDoor))
    (if (not (Audio|Components|Audio|IsPlaying (Variables|Default|GetAnimation_Door)))
      (Utilities|FlowControl|FlipFlop
        (:A
          (Audio|PlaySoundatLocation "/Game/HorrorKit/Assets/Audio/Interactive/Wardrobe/S_Open_Wardrobe_Cue.S_Open_Wardrobe_Cue" _returnvalue "0, 0, 0" 1.0 1.0 0.0 "/Game/HorrorKit/Assets/Audio/Interactive/Wardrobe/Info_Sound_Box_WardRobe_Table.Info_Sound_Box_WardRobe_Table")
          (bind _box (Timeline|Animation_Door Play)
            (:Update
              (Transformation|SetRelativeRotation (Variables|Default|GetScene_Door) (Math|Rotator|MakeRotator 0.0 0.0 _box) false false))))
        (:B
          (Audio|PlaySoundatLocation "/Game/HorrorKit/Assets/Audio/Interactive/Wardrobe/S_Close_Wardrobe_Cue.S_Close_Wardrobe_Cue" _returnvalue "0, 0, 0" 1.0 1.0 0.0 "/Game/HorrorKit/Assets/Audio/Interactive/Wardrobe/Info_Sound_Box_WardRobe_Table.Info_Sound_Box_WardRobe_Table")
          (Timeline|Animation_Door Reverse))))
    (elif (== Component (Variables|Default|GetBox))
      (if (not (Audio|Components|Audio|IsPlaying (Variables|Default|GetAnimation_Box)))
        (Utilities|FlowControl|FlipFlop
          (:A
            (Audio|PlaySoundatLocation "/Game/HorrorKit/Assets/Audio/Interactive/Box_Table/Open_Box_Cue.Open_Box_Cue" _returnvalue_2 "0, 0, 0" 1.0 1.0 0.0 "/Game/HorrorKit/Assets/Audio/Interactive/Wardrobe/Info_Sound_Box_WardRobe_Table.Info_Sound_Box_WardRobe_Table")
            (bind _box_2 (Timeline|Animation_Box Play)
              (:Update
                (Transformation|SetRelativeLocation (Variables|Default|GetBox) (Math|Vector|MakeVector _box_2 0.0 0.0) false false))))
          (:B
            (Audio|PlaySoundatLocation "/Game/HorrorKit/Assets/Audio/Interactive/Box_Table/Close_Box_Cue.Close_Box_Cue" _returnvalue_2 "0, 0, 0" 1.0 1.0 0.0 "/Game/HorrorKit/Assets/Audio/Interactive/Wardrobe/Info_Sound_Box_WardRobe_Table.Info_Sound_Box_WardRobe_Table")
            (Timeline|Animation_Box Reverse)))))))

(fn ConstructionScript)