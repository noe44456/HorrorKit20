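; Interactive kitchen table prop with two cabinet doors and two drawers that the player can open and close individually.
; The Interactive event checks which component was used and ignores it while that part's timeline is playing.
; Each part uses a FlipFlop to play or reverse its timeline, yawing door pivots or sliding drawers along X, with open and close sounds at the table.
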(event EventInteractive
  (params (Component :type Primitive%20Component%20Object%20Reference))
  (bind _table (Variables|Default|GetTable))
  (bind _table_2 (Variables|Default|GetTable))
  (bind _table_3 (Variables|Default|GetTable))
  (bind _table_4 (Variables|Default|GetTable))
  (bind _returnvalue (Transformation|GetWorldLocation _table_3))
  (bind _returnvalue_2 (Transformation|GetWorldLocation _table_4))
  (bind _returnvalue_3 (Transformation|GetWorldLocation _table))
  (bind _returnvalue_4 (Transformation|GetWorldLocation _table_2))
  (if (== Component (Variables|Default|GetDoor_Left))
    (if (not (Audio|Components|Audio|IsPlaying (Variables|Default|GetAnimation%20Door_Left)))
      (Utilities|FlowControl|FlipFlop
        (:A
          (Audio|PlaySoundatLocation "/Game/HorrorKit/Assets/Audio/Interactive/Wardrobe/S_Open_Wardrobe_Cue.S_Open_Wardrobe_Cue" _returnvalue_3 "0, 0, 0" 1.0 1.0 0.0 "/Game/HorrorKit/Assets/Audio/Interactive/Wardrobe/Info_Sound_Box_WardRobe_Table.Info_Sound_Box_WardRobe_Table")
          (bind _door (Timeline|Animation%20Door_Left Play)
            (:Update
              (Transformation|SetRelativeRotation (Variables|Default|GetScene_Door_Left) (Math|Rotator|MakeRotator 0.0 0.0 _door) false false))))
        (:B
          (Audio|PlaySoundatLocation "/Game/HorrorKit/Assets/Audio/Interactive/Wardrobe/S_Close_Wardrobe_Cue.S_Close_Wardrobe_Cue" _returnvalue_3 "0, 0, 0" 1.0 1.0 0.0 "/Game/HorrorKit/Assets/Audio/Interactive/Wardrobe/Info_Sound_Box_WardRobe_Table.Info_Sound_Box_WardRobe_Table")
          (Timeline|Animation%20Door_Left Reverse))))
    (elif (== Component (Variables|Default|GetDoor_Right))
      (if (not (Audio|Components|Audio|IsPlaying (Variables|Default|GetAnimation%20Door_Right)))
        (Utilities|FlowControl|FlipFlop
          (:A
            (Audio|PlaySoundatLocation "/Game/HorrorKit/Assets/Audio/Interactive/Wardrobe/S_Open_Wardrobe_Cue.S_Open_Wardrobe_Cue" _returnvalue_4 "0, 0, 0" 1.0 1.0 0.0 "/Game/HorrorKit/Assets/Audio/Interactive/Wardrobe/Info_Sound_Box_WardRobe_Table.Info_Sound_Box_WardRobe_Table")
            (bind _door_2 (Timeline|Animation%20Door_Right Play)
              (:Update
                (Transformation|SetRelativeRotation (Variables|Default|GetScene_Door_Right) (Math|Rotator|MakeRotator 0.0 0.0 _door_2) false false))))
          (:B
            (Audio|PlaySoundatLocation "/Game/HorrorKit/Assets/Audio/Interactive/Wardrobe/S_Close_Wardrobe_Cue.S_Close_Wardrobe_Cue" _returnvalue_4 "0, 0, 0" 1.0 1.0 0.0 "/Game/HorrorKit/Assets/Audio/Interactive/Wardrobe/Info_Sound_Box_WardRobe_Table.Info_Sound_Box_WardRobe_Table")
            (Timeline|Animation%20Door_Right Reverse))))
      (elif (== Component (Variables|Default|GetBox_Right))
        (if (not (Audio|Components|Audio|IsPlaying (Variables|Default|GetAnimation_Box_Right)))
          (Utilities|FlowControl|FlipFlop
            (:A
              (Audio|PlaySoundatLocation "/Game/HorrorKit/Assets/Audio/Interactive/Box_Table/Open_Box_Cue.Open_Box_Cue" _returnvalue "0, 0, 0" 1.0 1.0 0.0 "/Game/HorrorKit/Assets/Audio/Interactive/Wardrobe/Info_Sound_Box_WardRobe_Table.Info_Sound_Box_WardRobe_Table")
              (bind _box (Timeline|Animation_Box_Right Play)
                (:Update
                  (Transformation|SetRelativeLocation (Variables|Default|GetBox_Right) (Math|Vector|MakeVector _box 0.0 0.0) false false))))
            (:B
              (Audio|PlaySoundatLocation "/Game/HorrorKit/Assets/Audio/Interactive/Box_Table/Close_Box_Cue.Close_Box_Cue" _returnvalue "0, 0, 0" 1.0 1.0 0.0 "/Game/HorrorKit/Assets/Audio/Interactive/Wardrobe/Info_Sound_Box_WardRobe_Table.Info_Sound_Box_WardRobe_Table")
              (Timeline|Animation_Box_Right Reverse))))
        (elif (== Component (Variables|Default|GetBox_Left))
          (if (not (Audio|Components|Audio|IsPlaying (Variables|Default|GetAnimation_Box_Left)))
            (Utilities|FlowControl|FlipFlop
              (:A
                (Audio|PlaySoundatLocation "/Game/HorrorKit/Assets/Audio/Interactive/Box_Table/Open_Box_Cue.Open_Box_Cue" _returnvalue_2 "0, 0, 0" 1.0 1.0 0.0 "/Game/HorrorKit/Assets/Audio/Interactive/Wardrobe/Info_Sound_Box_WardRobe_Table.Info_Sound_Box_WardRobe_Table")
                (bind _box_2 (Timeline|Animation_Box_Left Play)
                  (:Update
                    (Transformation|SetRelativeLocation (Variables|Default|GetBox_Left) (Math|Vector|MakeVector _box_2 0.0 0.0) false false))))
              (:B
                (Audio|PlaySoundatLocation "/Game/HorrorKit/Assets/Audio/Interactive/Box_Table/Close_Box_Cue.Close_Box_Cue" _returnvalue_2 "0, 0, 0" 1.0 1.0 0.0 "/Game/HorrorKit/Assets/Audio/Interactive/Wardrobe/Info_Sound_Box_WardRobe_Table.Info_Sound_Box_WardRobe_Table")
                (Timeline|Animation_Box_Left Reverse)))))))))

(fn ConstructionScript)