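; BP_Rubbish_Heap is an interactive kitchen rubbish bin whose lid opens and closes.
; An Interactive event on the cover component alternates between opening and closing through a FlipFlop, ignoring input while the timeline is playing.
; The AnimationCover timeline drives the cover pivot's roll, playing forward to open and reversing to close.
; Each direction plays its own sound at the bin, with the closing sound slightly delayed.
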(event EventInteractive
  (params (Component :type Primitive%20Component%20Object%20Reference))
  (if (== (Variables|Default|GetCover_Rubbish_Heap) Component)
    (if (not (Audio|Components|Audio|IsPlaying (Variables|Default|GetAnimation%20Cover)))
      (Utilities|FlowControl|FlipFlop
        (:A
          (Audio|PlaySoundatLocation "/Game/HorrorKit/Assets/Audio/Interactive/Rubbish_Heap/S_Rubbish_Heap_Open_Cue.S_Rubbish_Heap_Open_Cue" (Transformation|GetWorldLocation (Variables|Default|GetRubbish_Heap)) "0, 0, 0" 1.0 1.0 0.0 "/Game/HorrorKit/Assets/Audio/Interactive/Rubbish_Heap/Info_Sound_Rubbish_Heap.Info_Sound_Rubbish_Heap")
          (bind _cover (Timeline|Animation%20Cover Play)
            (:Update
              (Transformation|SetRelativeRotation (Variables|Default|GetScene_Cover_Rubbish_Heap) (Math|Rotator|MakeRotator _cover 0.0 0.0) false false))))
        (:B
          (Utilities|FlowControl|Sequence
            (:then_0
              (Timeline|Animation%20Cover Reverse))
            (:then_1
              (Utilities|FlowControl|Delay 0.2)
              (Audio|PlaySoundatLocation "/Game/HorrorKit/Assets/Audio/Interactive/Rubbish_Heap/S_Rubbish_Heap_Close_Cue.S_Rubbish_Heap_Close_Cue" (Transformation|GetWorldLocation (Variables|Default|GetRubbish_Heap)) "0, 0, 0" 1.0 1.0 0.0 "/Game/HorrorKit/Assets/Audio/Interactive/Rubbish_Heap/Info_Sound_Rubbish_Heap.Info_Sound_Rubbish_Heap"))))))))

(fn ConstructionScript)