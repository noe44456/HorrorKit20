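; BP_Pistol is the player's pistol, handling firing, ammo and timed reload with animation flags, sounds, muzzle flash and smoke.
; Fire runs a line or sphere trace from the camera with random spread, looping on a timer in automatic mode until input or ammo ends.
; Traces consume a bullet and pass hits to an empty Hit event; line hits also spawn BP_Pistol_Impulse.
; Tick prints ammo counts for debugging.
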(event Custom|Event%20Hit
  (params (Hit :type Hit%20Result%20Structure)))

(fn ConstructionScript)

(fn MinusBullet
  (Utilities|Struct|SetmembersinPistol_S (Variables|Pistol|GetInfo_Pistol) (Math|Integer|Max(Integer) (- (Utilities|Struct|BreakPistol_S (Variables|Pistol|GetInfo_Pistol)) 1)))
  (return))

(fn SphereTrace
  (bind _info_pistol (Variables|Pistol|GetInfo_Pistol))
  (bind _character (Variables|Default|GetCharacter))
  (bind _spread (Utilities|Struct|BreakPistol_S _info_pistol))
  (bind _camera (Variables|/Game/HorrorKit/Blueprints/Player/MyCharacter.MyCharacter_C|GetCamera _character))
  (bind _returnvalue (Transformation|GetWorldLocation _camera))
  (bind _returnvalue_2 (* _spread 1e+01))
  (bind _returnvalue_3 (* _returnvalue_2 -1.0))
  (CallFunction|MinusBullet)
  (bind (_outhit _returnvalue_4) (Collision|SphereTraceByChannel _returnvalue (+ _returnvalue (* (Math|Vector|GetForwardVector _camera) (Utilities|Struct|BreakPistol_S (Variables|Pistol|GetInfo_Pistol))) (Math|Vector|MakeVector 0.0 (Math|Random|RandomFloatinRange _returnvalue_3 _returnvalue_2) (Math|Random|RandomFloatinRange _returnvalue_3 _returnvalue_2))) (Utilities|Struct|BreakHit_Box_S (Variables|Pistol|GetInfo_Hit_Box)) "TraceTypeQuery1" false 0 "ForDuration"))
  (if _returnvalue_4
    (CallFunction|EventHit _outhit))
  (if (not (and (Game|Player|IsInputKeyDown (Game|GetPlayerController 0) (Utilities|Struct|BreakInputActionKeyMapping (Utilities|Array|Get(acopy) (Class|InputSettings|GetActionMappingbyName (Class|InputSettings|GetInputSettings) "Fire")))) (> (Utilities|Struct|BreakPistol_S (Variables|Pistol|GetInfo_Pistol)) 0)))
    (CallFunction|EventRemoveAutomatic)))

(fn LineTrace
  (bind _info_pistol (Variables|Pistol|GetInfo_Pistol))
  (bind _character (Variables|Default|GetCharacter))
  (bind _spread (Utilities|Struct|BreakPistol_S _info_pistol))
  (bind _camera (Variables|/Game/HorrorKit/Blueprints/Player/MyCharacter.MyCharacter_C|GetCamera _character))
  (bind _returnvalue (Transformation|GetWorldLocation _camera))
  (bind _returnvalue_2 (* _spread 1e+01))
  (bind _returnvalue_3 (* _returnvalue_2 -1.0))
  (CallFunction|MinusBullet)
  (bind (_outhit _returnvalue_4) (Collision|LineTraceByChannel _returnvalue (+ _returnvalue (* (Math|Vector|GetForwardVector _camera) (Utilities|Struct|BreakPistol_S (Variables|Pistol|GetInfo_Pistol))) (Math|Vector|MakeVector 0.0 (Math|Random|RandomFloatinRange _returnvalue_3 _returnvalue_2) (Math|Random|RandomFloatinRange _returnvalue_3 _returnvalue_2))) "TraceTypeQuery1" true 0 "None"))
  (if _returnvalue_4
    (Utilities|FlowControl|Sequence
      (:then_0
        (CallFunction|EventHit _outhit)
        (if (not (and (Game|Player|IsInputKeyDown (Game|GetPlayerController 0) (Utilities|Struct|BreakInputActionKeyMapping (Utilities|Array|Get(acopy) (Class|InputSettings|GetActionMappingbyName (Class|InputSettings|GetInputSettings) "Fire")))) (> (Utilities|Struct|BreakPistol_S (Variables|Pistol|GetInfo_Pistol)) 0))) :!label _label
          (CallFunction|EventRemoveAutomatic)))
      (:then_1
        (Game|SpawnActorfromClass "/Game/HorrorKit/Blueprints/Weapons/Class/BP_Pistol_Impulse.BP_Pistol_Impulse_C" (Math|Transform|MakeTransform (.Location (Collision|BreakHitResult _outhit)) (Transformation|GetWorldRotation (.HitComponent (Collision|BreakHitResult _outhit))) "1,1,1") "Undefined" 0 0)))
    (else
      (goto _label))))

(event Custom|Event%20Reload
  (bind _character (Variables|Default|GetCharacter))
  (bind _character_2 (Variables|Default|GetCharacter))
  (bind _info_pistol (Variables|Pistol|GetInfo_Pistol))
  (bind _info_pistol_2 (Variables|Pistol|GetInfo_Pistol))
  (bind (_bullet _reloadbullet _maxbullet) (Utilities|Struct|BreakPistol_S _info_pistol))
  (bind (_bullet_2 _reloadbullet_2 _maxbullet_2) (Utilities|Struct|BreakPistol_S _info_pistol_2))
  (bind _guns_component (Variables|/Game/HorrorKit/Blueprints/Player/MyCharacter.MyCharacter_C|GetGuns_Component _character_2))
  (bind _anim_blueprint (Variables|/Game/HorrorKit/Blueprints/Player/MyCharacter.MyCharacter_C|GetAnim_Blueprint _character))
  (if (and (> _reloadbullet_2 0) (< _bullet_2 _maxbullet_2))
    (Audio|PlaySound2D "/Game/HorrorKit/Assets/Audio/Player/Weapon/S_Reload_Gun_Cue.S_Reload_Gun_Cue")
    (Rendering|SetVisibility (Variables|/Game/HorrorKit/Blueprints/Player/MyCharacter.MyCharacter_C|GetShop_Pistol _character_2) true false)
    (Variables|/Game/HorrorKit/Blueprints/Weapons/Guns_Component.Guns_Component_C|SetUse%20Animation _guns_component true)
    (Variables|/Game/HorrorKit/Blueprints/Player/Character/Animations/Anim_MyCharacter.Anim_MyCharacter_C|SetReload%20Pistol _anim_blueprint true)
    (Utilities|FlowControl|Delay 2.4)
    (Variables|/Game/HorrorKit/Blueprints/Player/Character/Animations/Anim_MyCharacter.Anim_MyCharacter_C|SetReload%20Pistol _anim_blueprint false)
    (Variables|/Game/HorrorKit/Blueprints/Weapons/Guns_Component.Guns_Component_C|SetUse%20Animation _guns_component false)
    (Rendering|SetVisibility (Variables|/Game/HorrorKit/Blueprints/Player/MyCharacter.MyCharacter_C|GetShop_Pistol (Variables|Default|GetCharacter)) false false)
    (Utilities|Struct|SetmembersinPistol_S (Variables|Pistol|GetInfo_Pistol) (Math|Integer|Min(Integer) (+ _bullet _reloadbullet) _maxbullet) (Math|Integer|Max(Integer) (- _reloadbullet (- _maxbullet _bullet))))))

(event Custom|Event%20Not%20Fire%20Pistol
  (Variables|/Game/HorrorKit/Blueprints/Player/Character/Animations/Anim_MyCharacter.Anim_MyCharacter_C|SetFire_Pistol (Variables|/Game/HorrorKit/Blueprints/Player/MyCharacter.MyCharacter_C|GetAnim_Blueprint (Variables|Default|GetCharacter)) false))

(event Custom|Event%20Fire
  (bind _pointlight (Variables|Default|GetPointLight))
  (bind _fire (Variables|Default|GetFire))
  (bind _character (Variables|Default|GetCharacter))
  (bind _anim_blueprint (Variables|/Game/HorrorKit/Blueprints/Player/MyCharacter.MyCharacter_C|GetAnim_Blueprint _character))
  (if (> (Utilities|Struct|BreakPistol_S (Variables|Pistol|GetInfo_Pistol)) 0)
    (if (not (Variables|/Game/HorrorKit/Blueprints/Weapons/Guns_Component.Guns_Component_C|GetUse%20Animation (Variables|/Game/HorrorKit/Blueprints/Player/MyCharacter.MyCharacter_C|GetGuns_Component (Variables|Default|GetCharacter))))
      (Utilities|FlowControl|Sequence
        (:then_0
          (Utilities|Time|ClearandInvalidateTimerbyHandle (Variables|Default|GetFire%20Timer))
          (Variables|/Game/HorrorKit/Blueprints/Weapons/Guns_Component.Guns_Component_C|SetUse%20Animation (Variables|/Game/HorrorKit/Blueprints/Player/MyCharacter.MyCharacter_C|GetGuns_Component (Variables|Default|GetCharacter)) true)
          (if (Variables|/Game/HorrorKit/Blueprints/Player/Character/Animations/Anim_MyCharacter.Anim_MyCharacter_C|GetFire_Pistol _anim_blueprint)
            _
            (else
              (Variables|/Game/HorrorKit/Blueprints/Player/Character/Animations/Anim_MyCharacter.Anim_MyCharacter_C|SetFire_Pistol _anim_blueprint true)
              (Utilities|FlowControl|Delay 0.2)))
          (Variables|/Game/HorrorKit/Blueprints/Player/Character/Animations/Anim_MyCharacter.Anim_MyCharacter_C|SetUse%20Fire%20Pistol _anim_blueprint true)
          (Utilities|FlowControl|Sequence
            (:then_0
              (Utilities|FlowControl|Delay 0.5)
              (Variables|/Game/HorrorKit/Blueprints/Player/Character/Animations/Anim_MyCharacter.Anim_MyCharacter_C|SetUse%20Fire%20Pistol _anim_blueprint false)
              (Utilities|FlowControl|Delay 0.01)
              (Variables|/Game/HorrorKit/Blueprints/Weapons/Guns_Component.Guns_Component_C|SetUse%20Animation (Variables|/Game/HorrorKit/Blueprints/Player/MyCharacter.MyCharacter_C|GetGuns_Component (Variables|Default|GetCharacter)) false))
            (:then_1
              (bind _returnvalue (Utilities|Time|SetTimerbyEvent (delegate Custom|Event%20Not%20Fire%20Pistol) 3.0))
              (Variables|Default|SetFire%20Timer _returnvalue))))
        (:then_1
          (Utilities|Time|ClearandInvalidateTimerbyHandle (Variables|Default|GetSmoke%20Timer))
          (Components|Activation|SetActive _fire true false)
          (Rendering|SetVisibility _pointlight true false)
          (Utilities|FlowControl|Sequence
            (:then_0
              (Utilities|FlowControl|Delay 0.17)
              (Rendering|SetVisibility _pointlight false false)
              (Components|Activation|SetActive _fire false false)
              (Audio|PlaySound2D "/Game/HorrorKit/Assets/Audio/Player/Weapon/S_Fire_Gun_Cue.S_Fire_Gun_Cue")
              (switch Utilities|FlowControl|Switch|SwitchonType_Fire (Utilities|Struct|BreakHit_Box_S (Variables|Pistol|GetInfo_Hit_Box))
                (:NewEnumerator0
                  (if (Utilities|Struct|BreakPistol_S (Variables|Pistol|GetInfo_Pistol))
                    (Utilities|Time|SetTimerbyFunctionName 0 "Line Trace" (Utilities|Struct|BreakPistol_S (Variables|Pistol|GetInfo_Pistol)) true)
                    (else
                      (CallFunction|LineTrace))))
                (:NewEnumerator1
                  (if (Utilities|Struct|BreakPistol_S (Variables|Pistol|GetInfo_Pistol))
                    (Utilities|Time|SetTimerbyFunctionName 0 "Sphere Trace" (Utilities|Struct|BreakPistol_S (Variables|Pistol|GetInfo_Pistol)) true)
                    (else
                      (CallFunction|SphereTrace))))))
            (:then_1
              (bind _returnvalue_2 (Utilities|Time|SetTimerbyEvent (delegate Custom|Event%20Smoke) 2.0))
              (Variables|Default|SetSmoke%20Timer _returnvalue_2))))))
    (else
      (Audio|PlaySound2D "/Game/HorrorKit/Assets/Audio/Player/Weapon/S_Pistol_Empty_Cue.S_Pistol_Empty_Cue"))))

(event Custom|Event%20Smoke
  (Components|Activation|SetActive (Variables|Default|GetSmoke) false false))

(event Custom|Event%20Remove%20Automatic
  (if (Utilities|Struct|BreakPistol_S (Variables|Pistol|GetInfo_Pistol))
    (switch Utilities|FlowControl|Switch|SwitchonType_Fire (Utilities|Struct|BreakHit_Box_S (Variables|Pistol|GetInfo_Hit_Box))
      (:NewEnumerator0
        (Utilities|Time|ClearTimerbyFunctionName 0 "Line Trace"))
      (:NewEnumerator1
        (Utilities|Time|ClearTimerbyFunctionName 0 "Sphere Trace")))))

(event EventTick
  (params (DeltaSeconds :type Float%20%28single-precision%29))
  (bind _info_pistol (Variables|Pistol|GetInfo_Pistol))
  (bind (_bullet _reloadbullet) (Utilities|Struct|BreakPistol_S _info_pistol))
  (Development|PrintString (Utilities|String|ToString(Text) (Utilities|Text|FormatText "Bullets - {Bullets} 
Reload Bullets - {Reload Bullets}" _bullet _reloadbullet)) true false "(R=0.000000,G=0.660000,B=1.000000,A=1.000000)" 0.0))

(event EventBeginPlay
  (bind _asmy_character (Utilities|Casting|CastToMyCharacter (Game|GetPlayerCharacter 0)))
  (Variables|Default|SetCharacter _asmy_character))