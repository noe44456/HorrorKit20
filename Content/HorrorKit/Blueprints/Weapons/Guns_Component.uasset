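; Player component that manages the pistol: equipping, holstering, reloading and firing through the character's Gun child actor.
; Selecting toggles the stored pistol class and the AnimBlueprint's TakePistol flag, with NotTakePistol clearing the child actor separately.
; Holstering caches InfoPistol, which is written onto the class-default struct before the next spawn to carry ammo over.
; UseAnimation blocks actions during animations and is only set here, never cleared.
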(event Custom|Event_Select_Pistol
  ;[0.03646 0 0.03531] Select Pistol
  (if (not (Variables|Default|GetUse%20Animation))
    (bind _pistol (Utilities|CasttoPistol)
      (:then
        (Variables|Info|SetInfo%20Pistol (Variables|/Game/HorrorKit/Blueprints/Weapons/Class/BP_Pistol.BP_Pistol_C|GetInfo_Pistol _pistol))
        (Variables|/Game/HorrorKit/Blueprints/Player/Character/Animations/Anim_MyCharacter.Anim_MyCharacter_C|SetTake_Pistol (Variables|/Game/HorrorKit/Blueprints/Player/MyCharacter.MyCharacter_C|GetAnim_Blueprint (Variables|Default|GetCharacter)) false)
        (Variables|Default|SetUse%20Animation true))
      (:Fail
        (if (Utilities|IsValidClass (Variables|Reference|GetBP_Pistol))
          (if (> (Utilities|Struct|BreakPistol_S (Variables|Info|GetInfo%20Pistol)) 0)
            (Utilities|Struct|SetmembersinPistol_S (.Info_Pistol (Utilities|GetClassDefaults (Variables|Reference|GetBP_Pistol))) (.Bullet (Utilities|Struct|BreakPistol_S (Variables|Info|GetInfo%20Pistol))) (.ReloadBullet (Utilities|Struct|BreakPistol_S (Variables|Info|GetInfo%20Pistol))) (.MaxBullet (Utilities|Struct|BreakPistol_S (Variables|Info|GetInfo%20Pistol))) (.Distance (Utilities|Struct|BreakPistol_S (Variables|Info|GetInfo%20Pistol))) (.AutoMatic (Utilities|Struct|BreakPistol_S (Variables|Info|GetInfo%20Pistol))) (.TimeAutoMatic (Utilities|Struct|BreakPistol_S (Variables|Info|GetInfo%20Pistol))) (.Spread (Utilities|Struct|BreakPistol_S (Variables|Info|GetInfo%20Pistol)))))
          (ChildActorComponent|SetChildActorClass (Variables|/Game/HorrorKit/Blueprints/Player/MyCharacter.MyCharacter_C|GetGun (Variables|Default|GetCharacter)) (Variables|Reference|GetBP_Pistol))
          (Variables|/Game/HorrorKit/Blueprints/Player/Character/Animations/Anim_MyCharacter.Anim_MyCharacter_C|SetTake_Pistol (Variables|/Game/HorrorKit/Blueprints/Player/MyCharacter.MyCharacter_C|GetAnim_Blueprint (Variables|Default|GetCharacter)) true)
          (Variables|Default|SetUse%20Animation true))))))

(event Custom|Event%20Not%20Take%20Pistol
  ;[0.03646 0 0.03531] Select Pistol
  (ChildActorComponent|SetChildActorClass (Variables|/Game/HorrorKit/Blueprints/Player/MyCharacter.MyCharacter_C|GetGun (Variables|Default|GetCharacter)) 0))

(event Custom|Event%20Fire%20Weapon
  ;[0.3802 0.1109 0.1109] Fire
  (if (not (Variables|Default|GetUse%20Animation))
    (bind _asbp_pistol (Utilities|Casting|CastToBP_Pistol (Variables|/Script/Engine.ChildActorComponent|GetChildActor (Variables|/Game/HorrorKit/Blueprints/Player/MyCharacter.MyCharacter_C|GetGun (Variables|Default|GetCharacter)))))
    (Default|EventFire _asbp_pistol)))

(event Custom|Reload_Weapon
  ;[0 0.3542 0.3263] Reload
  (if (not (Variables|Default|GetUse%20Animation))
    (bind _asbp_pistol (Utilities|Casting|CastToBP_Pistol (Variables|/Script/Engine.ChildActorComponent|GetChildActor (Variables|/Game/HorrorKit/Blueprints/Player/MyCharacter.MyCharacter_C|GetGun (Variables|Default|GetCharacter)))))
    (Default|EventReload _asbp_pistol)))

(fn AddPistol
  (params (BP :type BP%20Pistol%20Class%20Reference))
  (Variables|Reference|SetBP_Pistol BP))

(event EventBeginPlay
  (bind _asmy_character (Utilities|Casting|CastToMyCharacter (Game|GetPlayerCharacter 0)))
  (Variables|Default|SetCharacter _asmy_character))